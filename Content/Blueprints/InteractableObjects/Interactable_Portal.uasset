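; Clickable hex-grid portal that teleports the player character between paired In and Out hexagons, on either the world map or the arena.
; A FlipFlop boolean selects which end the character must be within one hex of.
; A custom flip-flop macro then toggles that state and picks the opposite end as destination.
; The character's "Everyone" calls apply the new transform and hex cell.
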(event EventBeginPlay
  (|CallParentFunction) ; This node is disabled and will not be called.\nDrag off pins to build functionality.
)

(event EventOnClicked
  (params (TouchedComponent :type Primitive%20Component%20Object%20Reference) (ButtonPressed :type Key%20Structure))
  (bind _game_inst_dg (Variables|Default|GetGame%20Inst%20DG))
  (bind _hexagonout_arena (Variables|InteractabelPortal|GetHexagonOut_Arena))
  (bind _game_inst_dg_2 (Variables|Default|GetGame%20Inst%20DG))
  (bind _hexagonin_world (Variables|InteractabelPortal|GetHexagonIn_World))
  (bind _hexagonout_world (Variables|InteractabelPortal|GetHexagonOut_World))
  (bind _game_inst_dg_3 (Variables|Default|GetGame%20Inst%20DG))
  (bind _hexagonin_arena (Variables|InteractabelPortal|GetHexagonIn_Arena))
  (bind _player_character_dg (Variables|/Game/Blueprints/GameSettings/GameInst_DG.GameInst_DG_C|GetPlayer%20Character%20DG _game_inst_dg))
  (bind _player_character_dg_2 (Variables|/Game/Blueprints/GameSettings/GameInst_DG.GameInst_DG_C|GetPlayer%20Character%20DG _game_inst_dg_2))
  (bind _player_character_dg_3 (Variables|/Game/Blueprints/GameSettings/GameInst_DG.GameInst_DG_C|GetPlayer%20Character%20DG _game_inst_dg_3))
  (bind _currentcharacterlocation (Variables|/Game/Blueprints/NPC/BaseCharacter_DG.BaseCharacter_DG_C|GetcurrentCharacterLocation _player_character_dg_2))
  (bind _currentcharacterlocationarena (Variables|/Game/Blueprints/NPC/BaseCharacter_DG.BaseCharacter_DG_C|GetcurrentCharacterLocationArena _player_character_dg_2))
  (if (Variables|Interactabel_Portal|GetInWorld)
    (if (Variables|InteractabelPortal|GetFlipFlop)
      (if (<= (CallFunction|HexagonDistance _currentcharacterlocation (Variables|InteractabelPortal|GetHexagonOut_World) true) 1)
        (Utilities|FlipFlopCustom :!label _label
          (:A
            (Default|EveryoneCallSetTranform _player_character_dg_3 (Transformation|GetActorLocation _hexagonin_world))
            (Default|EveryoneSetHexagonCell _player_character_dg_3 _hexagonin_world))
          (:B
            (Default|EveryoneCallSetTranform _player_character_dg_3 (Transformation|GetActorLocation _hexagonout_world))
            (Default|EveryoneSetHexagonCell _player_character_dg_3 _hexagonout_world))))
      (elif (<= (CallFunction|HexagonDistance _currentcharacterlocation (Variables|InteractabelPortal|GetHexagonIn_World) true) 1)
        (goto _label)))
    (elif (Variables|InteractabelPortal|GetFlipFlop)
      (if (<= (CallFunction|HexagonDistance _currentcharacterlocationarena (Variables|InteractabelPortal|GetHexagonOut_Arena) false) 1)
        (Utilities|FlipFlopCustom :!label _label_2
          (:A
            (Default|EveryoneCallSetTranform _player_character_dg (Transformation|GetWorldLocation (Variables|/Game/Blueprints/ProceduralGeneration/HexagonCellArena.HexagonCellArena_C|GetHexagonPointLocation _hexagonin_arena)))
            (Default|EveryoneSetHexagonCell _player_character_dg 0 _hexagonin_arena))
          (:B
            (Default|EveryoneCallSetTranform _player_character_dg (Transformation|GetWorldLocation (Variables|/Game/Blueprints/ProceduralGeneration/HexagonCellArena.HexagonCellArena_C|GetHexagonPointLocation _hexagonout_arena)))
            (Default|EveryoneSetHexagonCell _player_character_dg 0 _hexagonout_arena))))
      (elif (<= (CallFunction|HexagonDistance _currentcharacterlocationarena (Variables|InteractabelPortal|GetHexagonIn_Arena) false) 1)
        (goto _label_2)))))