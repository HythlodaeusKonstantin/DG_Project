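; Base Blueprint for clickable world objects that highlight when the cursor hovers over them.
; Cursor enter and exit events on the static mesh toggle custom depth rendering for an outline, and clicks call OnClick, all gated by the MeshCollision flag.
; OnClick is an empty hook, and BeginPlay caches the GameInst_DG game instance.
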(event OnBeginCursorOver(StaticMesh)
  (params (TouchedComponent :type Primitive%20Component%20Object%20Reference))
  (if (Variables|Default|GetMeshCollision)
    (CallFunction|OutlineActor true)))

(event OnEndCursorOver(StaticMesh)
  (params (TouchedComponent :type Primitive%20Component%20Object%20Reference))
  (if (Variables|Default|GetMeshCollision)
    (CallFunction|OutlineActor false)))

(event OnClicked(StaticMesh)
  (params (TouchedComponent :type Primitive%20Component%20Object%20Reference) (ButtonPressed :type Key%20Structure :default "None"))
  (if (Variables|Default|GetMeshCollision)
    (CallFunction|OnClick)))

(event EventBeginPlay
  (bind _asgame_inst_dg (Utilities|Casting|CastToGameInst_DG (Game|GetGameInstance)))
  (Variables|Default|SetGame%20Inst%20DG _asgame_inst_dg))

(fn ConstructionScript)

(fn OutlineActor
  (params (Active :type Boolean))
  (Rendering|SetRenderCustomDepth (Variables|Default|GetStaticMesh) Active))

(fn OnClick)