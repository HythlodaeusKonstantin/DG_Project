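; Movement component for PlayerCharacter_DG that moves its owner straight to a target location and tracks its speed.
; MoveToLocation opens a Tick gate that steps a fixed, frame-rate-dependent offset without sweep until within tolerance of the target.
; Each step faces the owner along its path with a -90 yaw correction and copies its transform into the character's variables.
; A looping timer samples position across a short delay, storing distance moved as Speed.
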(event Custom|MoveToLocation
  (params (TargetLocation :type Vector))
  (bind _player_character_dg (Variables|Default|GetPlayer%20Character%20DG))
  (bind _returnvalue (Transformation|GetActorTransform _player_character_dg))
  (bind (_location _rotation) (Math|Transform|BreakTransform _returnvalue))
  (Variables|Default|SetTargetLocation TargetLocation)
  (Utilities|FlowControl|Gate true) ; enters at Open
)

(event Custom|SpeedCounter
  (Variables|Default|SetLocationOld (Transformation|GetActorLocation (Components|GetOwner)))
  (Utilities|FlowControl|Delay 0.1)
  (Variables|Default|SetLocationNew (Transformation|GetActorLocation (Components|GetOwner)))
  (Variables|Default|SetSpeed (Math|Vector|Distance(Vector) (Variables|Default|GetLocationNew) (Variables|Default|GetLocationOld))))

(event EventBeginPlay
  (Utilities|Time|SetTimerbyFunctionName 0 "SpeedCounter" 0.1 true)
  (bind _asplayer_character_dg (Utilities|Casting|CastToPlayerCharacter_DG (Components|GetOwner)))
  (Variables|Default|SetPlayer%20Character%20DG _asplayer_character_dg))

(event EventTick
  (params (DeltaSeconds :type Float%20%28single-precision%29))
  (bind _returnvalue (Components|GetOwner))
  (bind _player_character_dg (Variables|Default|GetPlayer%20Character%20DG))
  (bind _targetlocation (Variables|Default|GetTargetLocation))
  (bind _returnvalue_2 (Transformation|GetActorLocation _returnvalue))
  (bind _returnvalue_3 (Transformation|GetActorTransform _player_character_dg))
  (bind _returnvalue_4 (Math|Rotator|FindLookatRotation _returnvalue_2 _targetlocation))
  (bind (_location _rotation) (Math|Transform|BreakTransform _returnvalue_3))
  (Utilities|FlowControl|Gate true :!label _label
    (:Exit
      (if (Math|Vector|Equal(Vector) (Transformation|GetActorLocation (Components|GetOwner)) (Variables|Default|GetTargetLocation) 15.0)
        (goto _label Close)
        (else
          (Transformation|AddActorWorldOffset (Components|GetOwner) (* (Math|Vector|GetForwardVector _returnvalue_4) 12.0))
          (Transformation|SetActorRotation (Components|GetOwner) (Math|Rotator|MakeRotator 0.0 0.0 (- (.Yaw (Math|Rotator|BreakRotator _returnvalue_4)) 9e+01)))
          (Variables|/Game/Blueprints/PlayerCharacter/PlayerCharacter_DG.PlayerCharacter_DG_C|SetCurrentActorRotation _player_character_dg _rotation)
          (Variables|/Game/Blueprints/PlayerCharacter/PlayerCharacter_DG.PlayerCharacter_DG_C|SetCurrentActorLocation _player_character_dg _location))))))