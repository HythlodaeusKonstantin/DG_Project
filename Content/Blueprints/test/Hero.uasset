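; Hero is a test Blueprint demonstrating how a child object accesses parameters inherited from its parent through Blueprint components.
; On BeginPlay it calls the parent implementation, sets the Name and Health fields on Stats, then prints both values with labels.
; Overlap and Tick events are disabled, and the construction script only calls its parent.
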(event EventBeginPlay
  (bind _stats (Variables|Default|Getstats))
  ;[1 1 1] Создание объекта-наследника и обращение к параметрам родителя через blueprint components
  (|CallParentFunction)
  (bind _output_get (Variables|/Game/Levels/stats.stats_C|Setname _stats "test"))
  (bind _output_get_2 (Variables|/Game/Levels/stats.stats_C|Sethealth _stats 150))
  (Development|PrintString "my name is ")
  (Development|PrintString _output_get)
  (Development|PrintString " and my health is ")
  (Development|PrintString (Utilities|String|ToString(Integer) _output_get_2)))

(event Collision|EventActorBeginOverlap
  (params (OtherActor :type Actor%20Object%20Reference))
  (|CallParentFunction OtherActor) ; This node is disabled and will not be called.\nDrag off pins to build functionality.
)

(event EventTick
  (params (DeltaSeconds :type Float%20%28single-precision%29))
  (|CallParentFunction DeltaSeconds) ; This node is disabled and will not be called.\nDrag off pins to build functionality.
)

(fn ConstructionScript
  (|CallParentFunction))