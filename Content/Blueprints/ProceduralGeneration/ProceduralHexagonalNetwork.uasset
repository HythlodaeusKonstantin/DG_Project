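; Procedural hex map actor that spawns rings of HexagonCell actors into a map keyed by vector index and links their neighbours.
; Generate turns the outer ring and random outward-spreading areas beyond a protected radius to water, and empties poorly connected cells.
; It then sorts cells into edge/empty lists, applies one random season material set and randomises rotations.
; FindPath runs an unfiltered breadth-first flood from a random edge cell, recording CameFrom without reconstructing a path.
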(event EventBeginPlay)

(fn ConstructionScript)

(fn Generate
  (bind _how_much_circle_you_want_ (Variables|GenerationDefault|GetHow%20Much%20Circle%20You%20Want?))
  (bind _hexallmap (Variables|HexagonCellsArrays|GetHexAllMap))
  ;[1 1 1] Очистка массива клеток гексов, установка начальных переменных
  (CallFunction|Clean)
  (Variables|GenerationProcess|SetCoordCurrent (Transformation|GetActorLocation self))
  (Variables|GenerationDefault|SetCircle 1)
  (Variables|GenerationProcess|SetIndexCurrent "0, 0, 0")
  ;[1 1 1] Расчет "защищенных" от создания пустоты кругов гексов и расчет кол-ва пустых областей
  (Variables|GenerationDefault|SetProtectedCircle (* (/ _how_much_circle_you_want_ 3) 2))
  (Variables|GenerationProcess|SetOrdinar%20Index 0)
  (Variables|GenerationDefault|SetAmountOfEmpty (* (/ _how_much_circle_you_want_ 3) 4))
  ;[1 1 1] Создание стартового гексагона
  (bind _returnvalue (Game|SpawnActorfromClass "/Game/Blueprints/ProceduralGeneration/HexagonCell.HexagonCell_C" (Math|Conversions|ToTransform(Vector) (Variables|GenerationProcess|GetCoordCurrent)) "Undefined" 0 (Variables|GenerationProcess|GetCoordCurrent) "0.000000,0.000000,0.000000" (Utilities|Array|MakeArray (Variables|CoubCoord|GetCoord_CoubeIndex_1) (Variables|CoubCoord|GetCoord_CoubeIndex_2) (Variables|CoubCoord|GetCoord_CoubeIndex_3) (Variables|CoubCoord|GetCoord_CoubeIndex_4) (Variables|CoubCoord|GetCoord_CoubeIndex_5) (Variables|CoubCoord|GetCoord_CoubeIndex_6)) false 0 0 true false 0 0 0))
  (Utilities|Map|Add (Variables|HexagonCellsArrays|GetHexAllMap) (Math|Vector|MakeVector 0.0 0.0 0.0) _returnvalue)
  ;[1 1 1] Создание цикла генерации по количеству заданных кругов
  (for _index (range 1 (Variables|GenerationDefault|GetHow%20Much%20Circle%20You%20Want?))
    ;;[1 1 1] Сдвиг шага генерации на сторону 3
    (Variables|GenerationProcess|SetCoordCurrent (- (Variables|GenerationProcess|GetCoordCurrent) (Variables|LocationCoord|GetCoord_1)))
    (Variables|GenerationProcess|SetIndexCurrent (+ (Variables|GenerationProcess|GetIndexCurrent) "0.000000,-1.000000,-1.000000"))
    ;[1 1 1] Инициализация цикла для создания гексов по кругу
    (for _index_2 (range 0 5)
      (switch int _index_2
        (:0
          ;;[1 1 1] Set up Temporal Location and Index
          (Variables|GenerationProcess|SetCoordTemporal (Variables|LocationCoord|GetCoord_3))
          (Variables|GenerationProcess|SetIndexTemporal (Variables|CoubCoord|GetCoord_CoubeIndex_1)))
        (:1
          (Variables|GenerationProcess|SetCoordTemporal (Variables|LocationCoord|GetCoord_4))
          (Variables|GenerationProcess|SetIndexTemporal (Variables|CoubCoord|GetCoord_CoubeIndex_6)))
        (:2
          (Variables|GenerationProcess|SetCoordTemporal (Variables|LocationCoord|GetCoord_5))
          (Variables|GenerationProcess|SetIndexTemporal (Variables|CoubCoord|GetCoord_CoubeIndex_5)))
        (:3
          (Variables|GenerationProcess|SetCoordTemporal (Variables|LocationCoord|GetCoord_6))
          (Variables|GenerationProcess|SetIndexTemporal (Variables|CoubCoord|GetCoord_CoubeIndex_4)))
        (:4
          (Variables|GenerationProcess|SetCoordTemporal (Variables|LocationCoord|GetCoord_1))
          (Variables|GenerationProcess|SetIndexTemporal (Variables|CoubCoord|GetCoord_CoubeIndex_3)))
        (:5
          (Variables|GenerationProcess|SetCoordTemporal (Variables|LocationCoord|GetCoord_2))
          (Variables|GenerationProcess|SetIndexTemporal (Variables|CoubCoord|GetCoord_CoubeIndex_2))))
      ;[1 1 1] Создание цикла по количеству гексов на данном круге
      (for _index_3 (range 1 (Variables|GenerationDefault|GetCircle))
        ;[1 1 1] Increment Circle and Ordinar Index
        (Math|Integer|IncrementInt (Variables|GenerationProcess|GetCircleIndex)
          (:%20%20
            (Math|Integer|IncrementInt (Variables|GenerationProcess|GetOrdinar%20Index)
              (:%20%20
                ;[1 1 1] Создание ячейки гекса
                (bind _returnvalue_2 (Game|SpawnActorfromClass "/Game/Blueprints/ProceduralGeneration/HexagonCell.HexagonCell_C" (Math|Conversions|ToTransform(Vector) (- (Variables|GenerationProcess|GetCoordCurrent) (Variables|GenerationProcess|GetCoordTemporal))) "Undefined" 0 (- (Variables|GenerationProcess|GetCoordCurrent) (Variables|GenerationProcess|GetCoordTemporal)) (+ (Variables|GenerationProcess|GetIndexCurrent) (Variables|GenerationProcess|GetIndexTemporal)) (Utilities|Array|MakeArray (+ (+ (Variables|GenerationProcess|GetIndexCurrent) (Variables|GenerationProcess|GetIndexTemporal)) "1.000000, 0,1.000000") (+ (+ (Variables|GenerationProcess|GetIndexCurrent) (Variables|GenerationProcess|GetIndexTemporal)) "0.000000,1.000000,1.000000") (+ (+ (Variables|GenerationProcess|GetIndexCurrent) (Variables|GenerationProcess|GetIndexTemporal)) "-1.000000,1.000000, 0") (+ (+ (Variables|GenerationProcess|GetIndexCurrent) (Variables|GenerationProcess|GetIndexTemporal)) "-1.000000, 0,-1.000000") (+ (+ (Variables|GenerationProcess|GetIndexCurrent) (Variables|GenerationProcess|GetIndexTemporal)) "0,-1.000000,-1.000000") (+ (+ (Variables|GenerationProcess|GetIndexCurrent) (Variables|GenerationProcess|GetIndexTemporal)) "1.000000,-1.000000, 0")) false (Variables|GenerationDefault|GetCircle) 0 true false (Variables|GenerationProcess|GetCircleIndex) (Variables|GenerationProcess|GetOrdinar%20Index) 0))
                (Utilities|Map|Add (Variables|HexagonCellsArrays|GetHexAllMap) (+ (Variables|GenerationProcess|GetIndexCurrent) (Variables|GenerationProcess|GetIndexTemporal)) _returnvalue_2)
                ;[1 1 1] Rewriting Coordinate and Index
                (Variables|GenerationProcess|SetCoordCurrent (- (Variables|GenerationProcess|GetCoordCurrent) (Variables|GenerationProcess|GetCoordTemporal)))
                (Variables|GenerationProcess|SetIndexCurrent (+ (Variables|GenerationProcess|GetIndexCurrent) (Variables|GenerationProcess|GetIndexTemporal)))
                ;[1 1 1] Set Hex From Last Circle To Empty
                (if (== (Variables|GenerationDefault|GetCircle) (Variables|GenerationDefault|GetHow%20Much%20Circle%20You%20Want?))
                  (Components|StaticMesh|SetStaticMesh (Variables|/Game/Blueprints/ProceduralGeneration/HexagonCell.HexagonCell_C|GetCell _returnvalue_2) "/Game/Meshes/HexagonMesh/HexWater.HexWater")
                  (Variables|/Game/Blueprints/ProceduralGeneration/HexagonCell.HexagonCell_C|SetEmpty? _returnvalue_2 true)
                  (Variables|/Game/Blueprints/ProceduralGeneration/HexagonCell.HexagonCell_C|SetCanPass? _returnvalue_2 false)
                  (Variables|/Game/Blueprints/ProceduralGeneration/HexagonCell.HexagonCell_C|SetWater? _returnvalue_2 true))))))))
    ;;[1 1 1] Increment Circle
    (Math|Integer|IncrementInt (Variables|GenerationDefault|GetCircle)
      (:%20%20
        ;;[1 1 1] Renew Circle Index
        (Variables|GenerationProcess|SetCircleIndex 0))))
  ;[1 1 1] Set Up Neigbors
  (bind _values (Utilities|Map|Values _hexallmap))
  (for _array_element _values
    (for _array_element_2 (Variables|/Game/Blueprints/ProceduralGeneration/HexagonCell.HexagonCell_C|GetNeigbors _array_element)
      (if (.ReturnValue (Utilities|Map|Find _hexallmap _array_element_2))
        (Utilities|Array|Add (Variables|/Game/Blueprints/ProceduralGeneration/HexagonCell.HexagonCell_C|GetNeigborsHex _array_element) (.Value (Utilities|Map|Find _hexallmap _array_element_2))))))
  ;[1 1 1] CreateHexagonCellsAll
  (bind _values_2 (Utilities|Map|Values (Variables|HexagonCellsArrays|GetHexAllMap)))
  (Variables|HexagonCellsArrays|SetHexagonCells-ALL _values_2)
  ;[1 1 1] Create Random Landscape Emtyness
  ;;[1 1 1] Cleaning
  (Utilities|Array|Clear (Variables|HexagonCellsArrays|GetHexagonCellsToEmpty))
  ;;[1 1 1] Calculate Random Hex To Empty
  (for _index_4 (range 1 (Variables|GenerationDefault|GetAmountOfEmpty))
    (Variables|CreateEmptySpaces|SetRandomCircleToEmpty (Math|Random|RandomIntegerinRange (Variables|GenerationDefault|GetProtectedCircle) (- (Variables|GenerationDefault|GetHow%20Much%20Circle%20You%20Want?) 1)))
    (Variables|CreateEmptySpaces|SetRandomCircleIndex (Math|Random|RandomIntegerinRange 1 (* (Variables|CreateEmptySpaces|GetRandomCircleToEmpty) 6)))
    ;;[1 1 1] Finding Out Random Hexes From All
    (bind _array_element_3 (Utilities|Array|ForEachLoopwithBreak (Variables|HexagonCellsArrays|GetHexagonCells-ALL) :!label _label)
      (:LoopBody
        (if (and (== (Variables|/Game/Blueprints/ProceduralGeneration/HexagonCell.HexagonCell_C|GetCircle _array_element_3) (Variables|CreateEmptySpaces|GetRandomCircleToEmpty)) (== (Variables|/Game/Blueprints/ProceduralGeneration/HexagonCell.HexagonCell_C|GetCircle%20Index _array_element_3) (Variables|CreateEmptySpaces|GetRandomCircleIndex)))
          (Utilities|Array|AddUnique (Variables|HexagonCellsArrays|GetHexagonCellsToEmpty) _array_element_3)
          (goto _label Break)))
      (:Completed
        ;;[1 1 1] Finding Array Of Hexes To Empty
        (for _array_element_4 (Variables|HexagonCellsArrays|GetHexagonCellsToEmpty)
          (for _array_element_5 (Variables|/Game/Blueprints/ProceduralGeneration/HexagonCell.HexagonCell_C|GetNeigborsHex _array_element_4)
            (if (> (Variables|/Game/Blueprints/ProceduralGeneration/HexagonCell.HexagonCell_C|GetCircle _array_element_5) (Variables|/Game/Blueprints/ProceduralGeneration/HexagonCell.HexagonCell_C|GetCircle _array_element_4))
              (Utilities|Array|AddUnique (Variables|HexagonCellsArrays|GetHexagonCellsToEmpty) _array_element_5))))
        ;;[1 1 1] Set Hexes Empty
        (for _array_element_6 (Variables|HexagonCellsArrays|GetHexagonCellsToEmpty)
          (Components|StaticMesh|SetStaticMesh (Variables|/Game/Blueprints/ProceduralGeneration/HexagonCell.HexagonCell_C|GetCell _array_element_6) "/Game/Meshes/HexagonMesh/HexWater.HexWater")
          (Variables|/Game/Blueprints/ProceduralGeneration/HexagonCell.HexagonCell_C|SetEmpty? _array_element_6 true)
          (Variables|/Game/Blueprints/ProceduralGeneration/HexagonCell.HexagonCell_C|SetCanPass? _array_element_6 false)
          (Variables|/Game/Blueprints/ProceduralGeneration/HexagonCell.HexagonCell_C|SetWater? _array_element_6 true)))))
  ;[1 1 1] Delete Hexagons With 0\1\2 Neihgbors
  ;;[1 1 1] Calculate Anount Of Visible Neihbours
  (for _array_element_7 (Variables|HexagonCellsArrays|GetHexagonCells-ALL)
    (Variables|GenerationEmpty|SetVisibleHexCount 0)
    (if (Utilities|Array|IsValidIndex (Variables|/Game/Blueprints/ProceduralGeneration/HexagonCell.HexagonCell_C|GetNeigborsHex _array_element_7))
      (for _array_element_8 (Variables|/Game/Blueprints/ProceduralGeneration/HexagonCell.HexagonCell_C|GetNeigborsHex _array_element_7)
        (if (not (Variables|/Game/Blueprints/ProceduralGeneration/HexagonCell.HexagonCell_C|GetEmpty? _array_element_8))
          (Math|Integer|IncrementInt (Variables|GenerationEmpty|GetVisibleHexCount))))
      ;;[1 1 1] Set Them Empty
      (if (Math|Boolean|ORBoolean (== (Variables|GenerationEmpty|GetVisibleHexCount) 0) (== (Variables|GenerationEmpty|GetVisibleHexCount) 1) (== (Variables|GenerationEmpty|GetVisibleHexCount) 2))
        (Components|StaticMesh|SetStaticMesh (Variables|/Game/Blueprints/ProceduralGeneration/HexagonCell.HexagonCell_C|GetCell _array_element_7) "/Game/Meshes/HexagonMesh/HexWater.HexWater")
        (Variables|/Game/Blueprints/ProceduralGeneration/HexagonCell.HexagonCell_C|SetEmpty? _array_element_7 true)
        (Variables|/Game/Blueprints/ProceduralGeneration/HexagonCell.HexagonCell_C|SetCanPass? _array_element_7 false)
        (Variables|/Game/Blueprints/ProceduralGeneration/HexagonCell.HexagonCell_C|SetWater? _array_element_7 false))))
  ;[1 1 1] Fulfill Hex Array Different Types
  ;;[1 1 1] Cleaning
  (Utilities|Array|Clear (Variables|HexagonCellsArrays|GetHexagonNotEdgeCells))
  (Utilities|Array|Clear (Variables|HexagonCellsArrays|GetHexagonEdgeCells))
  (Utilities|Array|Clear (Variables|HexagonCellsArrays|GetHexagonEmptyCells))
  (Utilities|Array|Clear (Variables|HexagonCellsArrays|GetHexagonNotEmptyCells))
  (Utilities|Array|Clear (Variables|HexagonCellsArrays|GetHexagonEmptyCellsNotEdge))
  (Utilities|Array|Clear (Variables|HexagonCellsArrays|GetHexagonEmptyCellsEdge))
  ;;[1 1 1] Find Out Not Empty Hex, Empty Hex, Empty Hex On Edge and Empty Hex Not On Edge
  (for _array_element_9 (Variables|HexagonCellsArrays|GetHexagonCells-ALL)
    (if (Variables|/Game/Blueprints/ProceduralGeneration/HexagonCell.HexagonCell_C|GetEmpty? _array_element_9)
      (Utilities|Array|AddUnique (Variables|HexagonCellsArrays|GetHexagonEmptyCells) _array_element_9)
      (else
        (Utilities|Array|AddUnique (Variables|HexagonCellsArrays|GetHexagonNotEmptyCells) _array_element_9))))
  (Utilities|FlowControl|Sequence
    (:then_0
      (for _array_element_10 (Variables|HexagonCellsArrays|GetHexagonEmptyCells)
        (bind _array_element_11 (Utilities|Array|ForEachLoopwithBreak (Variables|/Game/Blueprints/ProceduralGeneration/HexagonCell.HexagonCell_C|GetNeigborsHex _array_element_10) :!label _label_2)
          (:LoopBody
            (Variables|FulfillHexArrayDifferentTypes|SetTheIsNoEmptyCells true)
            (if (not (Variables|/Game/Blueprints/ProceduralGeneration/HexagonCell.HexagonCell_C|GetEmpty? _array_element_11))
              (Utilities|Array|AddUnique (Variables|HexagonCellsArrays|GetHexagonEmptyCellsEdge) _array_element_11)
              (Variables|FulfillHexArrayDifferentTypes|SetTheIsNoEmptyCells false)
              (goto _label_2 Break)))))
      (if (Variables|FulfillHexArrayDifferentTypes|GetTheIsNoEmptyCells)
        (Utilities|Array|AddUnique (Variables|HexagonCellsArrays|GetHexagonEmptyCellsNotEdge) _array_element_10)))
    (:then_1
      ;;[1 1 1] Find Out Hex On Edge and Out Of Edge
      (for _array_element_12 (Variables|HexagonCellsArrays|GetHexagonNotEmptyCells)
        (bind _array_element_13 (Utilities|Array|ForEachLoopwithBreak (Variables|/Game/Blueprints/ProceduralGeneration/HexagonCell.HexagonCell_C|GetNeigborsHex _array_element_12) :!label _label_3)
          (:LoopBody
            (Variables|FulfillHexArrayDifferentTypes|SetTheIsNoEmptyCells true)
            (if (Variables|/Game/Blueprints/ProceduralGeneration/HexagonCell.HexagonCell_C|GetEmpty? _array_element_13)
              (Utilities|Array|AddUnique (Variables|HexagonCellsArrays|GetHexagonEdgeCells) _array_element_12)
              (Variables|FulfillHexArrayDifferentTypes|SetTheIsNoEmptyCells false)
              (goto _label_3 Break)))
          (:Completed
            (if (Variables|FulfillHexArrayDifferentTypes|GetTheIsNoEmptyCells)
              (Utilities|Array|AddUnique (Variables|HexagonCellsArrays|GetHexagonNotEdgeCells) _array_element_12)))))
      ;[1 1 1] Set Up Materials And Rotate Hex
      (Variables|HexMaterials|SetRandomMaterial (Math|Random|RandomIntegerinRange 0 3))
      (for _array_element_14 (Variables|HexagonCellsArrays|GetHexagonNotEmptyCells)
        (switch int (Variables|HexMaterials|GetRandomMaterial)
          (:Default
            (Variables|HexMaterials|SetMaterial1 "/Game/Materials/Grass_Inst1.Grass_Inst1" :!label _label_4)
            (Variables|HexMaterials|SetMaterial2 "/Game/Materials/Grass_Inst2.Grass_Inst2"))
          (:0
            (goto _label_4))
          (:1
            (Variables|HexMaterials|SetMaterial1 "/Game/Materials/Autumn_Inst1.Autumn_Inst1")
            (Variables|HexMaterials|SetMaterial2 "/Game/Materials/Autumn_Inst2.Autumn_Inst2"))
          (:2
            (Variables|HexMaterials|SetMaterial1 "/Game/Materials/Winter_Inst1.Winter_Inst1")
            (Variables|HexMaterials|SetMaterial2 "/Game/Materials/Winter_Inst2.Winter_Inst2")))
        (Rendering|Material|SetMaterial (Variables|/Game/Blueprints/ProceduralGeneration/HexagonCell.HexagonCell_C|GetCell _array_element_14) 0 (Variables|HexMaterials|GetMaterial1))
        (Rendering|Material|SetMaterial (Variables|/Game/Blueprints/ProceduralGeneration/HexagonCell.HexagonCell_C|GetCell _array_element_14) 1 (Variables|HexMaterials|GetMaterial2))
        (switch int (Math|Random|RandomIntegerinRange 0 5)
          (:0
            (Variables|HexMaterials|SetUniversalRotator "0,60.000000, 0"))
          (:1
            (Variables|HexMaterials|SetUniversalRotator "0,120.000000, 0"))
          (:2
            (Variables|HexMaterials|SetUniversalRotator "0,180.000000, 0"))
          (:3
            (Variables|HexMaterials|SetUniversalRotator "0,240.000000, 0"))
          (:4
            (Variables|HexMaterials|SetUniversalRotator "0,300.000000, 0"))
          (:5
            (Variables|HexMaterials|SetUniversalRotator "0, 0, 0")))
        (Transformation|SetActorRotation _array_element_14 (Variables|HexMaterials|GetUniversalRotator))))))

(fn Clean
  (bind _hexallmap (Variables|HexagonCellsArrays|GetHexAllMap))
  ;[1 1 1] Cleaning
  (bind _values (Utilities|Map|Values _hexallmap))
  (if (Utilities|Array|IsValidIndex _values)
    (for _array_element _values
      (Actor|DestroyActor _array_element)))
  (Utilities|Map|Clear _hexallmap)
  (Utilities|Array|Clear (Variables|HexagonCellsArrays|GetHexagonCells-ALL)))

(fn FindPath
  (bind _tovisit (Variables|PathGeneration|GettoVisit))
  (bind _tovisit_2 (Variables|PathGeneration|GettoVisit))
  (bind _output (Utilities|Array|Get(acopy) _tovisit_2))
  ;[1 1 1] Задаем стартовый гекс посещенным и создаем массив посещенных вершин
  (bind _output_get (Variables|PathGeneration|SetpathfinderHexStart (.OutItem (Utilities|Array|Random (Variables|HexagonCellsArrays|GetHexagonEdgeCells)))))
  (Variables|PathGeneration|SetpathfinderHexGoal (.OutItem (Utilities|Array|Random (Variables|HexagonCellsArrays|GetHexagonNotEmptyCells))))
  (Variables|/Game/Blueprints/ProceduralGeneration/HexagonCell.HexagonCell_C|SetpathfinderVisited _output_get true)
  (Utilities|Array|Add _tovisit _output_get)
  ;[1 1 1] Пока в массиве посещенных вершин есть хотя бы один элемент, берем его, переписываем в переменную Current, затем удаляем и соседей Current в цикле добавляем в массив вершин к посещению
  (while (Utilities|Array|IsValidIndex _tovisit)
    (bind _output_get_2 (Variables|PathGeneration|SetpathfinderCurrentHex _output))
    (Utilities|Array|RemoveItem _tovisit_2 _output)
    (for _array_element (Variables|/Game/Blueprints/ProceduralGeneration/HexagonCell.HexagonCell_C|GetNeigborsHex _output_get_2)
      ;;[1 1 1] Если вершина не была посещена, добавляем и обновляем у гекса поле cameFrom
      (if (not (Variables|/Game/Blueprints/ProceduralGeneration/HexagonCell.HexagonCell_C|GetpathfinderVisited _array_element))
        (Utilities|Array|Add (Variables|PathGeneration|GettoVisit) _array_element)
        (Variables|/Game/Blueprints/ProceduralGeneration/HexagonCell.HexagonCell_C|SetpathfinderVisited _array_element true)
        (Variables|/Game/Blueprints/ProceduralGeneration/HexagonCell.HexagonCell_C|SetcameFrom _array_element _output_get_2)))))