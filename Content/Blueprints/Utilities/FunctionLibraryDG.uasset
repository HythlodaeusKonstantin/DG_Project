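; Blueprint function library of shared helpers for hex-grid maps, integer packing and HUD switching.
; Cube-coordinate functions measure distances between points or world/arena hex cells, and FindHex looks up cells by island and ordinal index in the GameInstance.
; Codec pairs pack two ints into three bytes or four digits into one int, whose decoder returns digits in reverse order.
; SwitchUI toggles world and combat widgets from the player's CurrentWorld.
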(fn MeasureDistanceCube
  (params (Start :type Vector) (Target :type Vector))
  (bind (_x _y _z) (Math|Vector|BreakVector Start))
  (bind (_x_2 _y_2 _z_2) (Math|Vector|BreakVector Target))
  (return (Math|Float|Truncate (Math|Float|Max(Float) (Math|Float|Absolute(Float) (- _x _x_2)) (Math|Float|Absolute(Float) (- _y _y_2)) (Math|Float|Absolute(Float) (- _z _z_2))))))

(fn EncodeTwoInttoThreeByte
  (params (a :type Integer) (b :type Integer))
  (return (Math|Conversions|ToByte(Integer) a) (Math|Conversions|ToByte(Integer) (/ b 100)) (Math|Conversions|ToByte(Integer) (Math|Integer|%(Integer) b 100))))

(fn DecodeThreeBytetoTwoInt
  (params (a1 :type Byte) (b1 :type Byte) (b2 :type Byte))
  (return (Math|Conversions|ToInteger(Byte) a1) (+ (* (Math|Conversions|ToInteger(Byte) b1) 100) (Math|Conversions|ToInteger(Byte) b2))))

(fn EncodeFourInttoOneInt
  (params (a :type Integer) (b :type Integer) (c :type Integer) (d :type Integer))
  (return (|((((((a*10)+b)*10)+c)*10)+d) a b c d)))

(fn DecodeOneInttoFourInt
  (params (a1 :type Integer))
  (return (Math|Float|Truncate (Math|Float|%(Float) (Math|Conversions|ToFloat(Integer) a1) 1e+01)) (Math|Float|Truncate (Math|Float|%(Float) (Math|Conversions|ToFloat(Integer) (/ a1 10)) 1e+01)) (Math|Float|Truncate (Math|Float|%(Float) (Math|Conversions|ToFloat(Integer) (/ a1 100)) 1e+01)) (Math|Float|Truncate (Math|Float|%(Float) (Math|Conversions|ToFloat(Integer) (/ a1 1000)) 1e+01))))

(fn FindHex
  (params (GameInstance :type Game%20Inst%20DG%20Object%20Reference) (IslandIndex :type Integer%20%28by%20ref%29) (OrdinarIndex :type Integer%20%28by%20ref%29))
  (bind _islandgenerationnetworks (Variables|/Game/Blueprints/GameSettings/GameInst_DG.GameInst_DG_C|GetIslandGenerationNetworks GameInstance))
  (bind _value (Utilities|Map|Find _islandgenerationnetworks IslandIndex))
  (bind _hexallmapint (Variables|/Game/Blueprints/ProceduralGeneration/ProceduralHexagonalNetwork.ProceduralHexagonalNetwork_C|GetHexAllMapInt _value))
  (bind (_value_2 _returnvalue) (Utilities|Map|Find _hexallmapint OrdinarIndex))
  (return _value_2 _returnvalue))

(fn SwitchUI
  (bind _asgame_inst_dg (Utilities|Casting|CastToGameInst_DG (Game|GetGameInstance)))
  (bind _asplayer_character_dg (Utilities|Casting|CastToPlayerCharacter_DG (Game|Player|GetPlayerPawn 0)))
  (Utilities|IsValid _asplayer_character_dg
    (:Is%20Valid
      (Utilities|FlowControl|Sequence
        (:then_0
          (switch Utilities|FlowControl|Switch|SwitchonCurrentWorld (Variables|/Game/Blueprints/NPC/BaseCharacter_DG.BaseCharacter_DG_C|GetCurrentWorld _asplayer_character_dg)
            (:NewEnumerator0
              (Widget|SetVisibility (Variables|/Game/Blueprints/UserInterface/InGameUI/InGameUI.InGameUI_C|GetActionBarCombat_UI (Variables|/Game/Blueprints/GameSettings/GameInst_DG.GameInst_DG_C|GetInGameUI _asgame_inst_dg)) "Hidden" :!label _label)
              (Widget|SetVisibility (Variables|/Game/Blueprints/UserInterface/InGameUI/InGameUI.InGameUI_C|GetExitArena (Variables|/Game/Blueprints/GameSettings/GameInst_DG.GameInst_DG_C|GetInGameUI _asgame_inst_dg)) "Hidden")
              (Widget|SetVisibility (Variables|/Game/Blueprints/UserInterface/InGameUI/InGameUI.InGameUI_C|GetActionBarWorldUI (Variables|/Game/Blueprints/GameSettings/GameInst_DG.GameInst_DG_C|GetInGameUI _asgame_inst_dg)) "Visible")
              (Widget|SetVisibility (Variables|/Game/Blueprints/UserInterface/InGameUI/InGameUI.InGameUI_C|GetCalendarUI (Variables|/Game/Blueprints/GameSettings/GameInst_DG.GameInst_DG_C|GetInGameUI _asgame_inst_dg)) "Visible")
              (Widget|SetVisibility (Variables|/Game/Blueprints/UserInterface/InGameUI/InGameUI.InGameUI_C|GetbtnEndTurn (Variables|/Game/Blueprints/GameSettings/GameInst_DG.GameInst_DG_C|GetInGameUI _asgame_inst_dg)) "Hidden")
              (Widget|SetVisibility (Variables|/Game/Blueprints/UserInterface/InGameUI/InGameUI.InGameUI_C|GetCombatTurnBasedUI (Variables|/Game/Blueprints/GameSettings/GameInst_DG.GameInst_DG_C|GetInGameUI _asgame_inst_dg)) "Hidden"))
            (:NewEnumerator1
              (goto _label))
            (:NewEnumerator2
              (Widget|SetVisibility (Variables|/Game/Blueprints/UserInterface/InGameUI/InGameUI.InGameUI_C|GetActionBarCombat_UI (Variables|/Game/Blueprints/GameSettings/GameInst_DG.GameInst_DG_C|GetInGameUI _asgame_inst_dg)) "Visible")
              (Widget|SetVisibility (Variables|/Game/Blueprints/UserInterface/InGameUI/InGameUI.InGameUI_C|GetExitArena (Variables|/Game/Blueprints/GameSettings/GameInst_DG.GameInst_DG_C|GetInGameUI _asgame_inst_dg)) "Visible")
              (Widget|SetVisibility (Variables|/Game/Blueprints/UserInterface/InGameUI/InGameUI.InGameUI_C|GetActionBarWorldUI (Variables|/Game/Blueprints/GameSettings/GameInst_DG.GameInst_DG_C|GetInGameUI _asgame_inst_dg)) "Hidden")
              (Widget|SetVisibility (Variables|/Game/Blueprints/UserInterface/InGameUI/InGameUI.InGameUI_C|GetCalendarUI (Variables|/Game/Blueprints/GameSettings/GameInst_DG.GameInst_DG_C|GetInGameUI _asgame_inst_dg)) "Hidden")
              (Widget|SetVisibility (Variables|/Game/Blueprints/UserInterface/InGameUI/InGameUI.InGameUI_C|GetbtnEndTurn (Variables|/Game/Blueprints/GameSettings/GameInst_DG.GameInst_DG_C|GetInGameUI _asgame_inst_dg)) "Visible")
              (Widget|SetVisibility (Variables|/Game/Blueprints/UserInterface/InGameUI/InGameUI.InGameUI_C|GetCombatTurnBasedUI (Variables|/Game/Blueprints/GameSettings/GameInst_DG.GameInst_DG_C|GetInGameUI _asgame_inst_dg)) "Visible"))))
        (:then_1
          (return))))))

(fn HexagonDistance
  (params (HexagonA :type Actor%20Object%20Reference) (HexagonB :type Actor%20Object%20Reference) (World :type Boolean))
  (if World
    (bind _ashexagon_cell_world (Utilities|Casting|CastToHexagonCellWorld HexagonA))
    (bind _ashexagon_cell_world_2 (Utilities|Casting|CastToHexagonCellWorld HexagonB))
    (LocalVariables|SetDistance (|((((abs((x1-x2)))+(abs((y1-y2))))+(abs((z1-z2))))/2) (.x (Variables|/Game/Blueprints/ProceduralGeneration/HexagonCellWorld.HexagonCellWorld_C|GetIndex _ashexagon_cell_world)) (.x (Variables|/Game/Blueprints/ProceduralGeneration/HexagonCellWorld.HexagonCellWorld_C|GetIndex _ashexagon_cell_world_2)) (.y (Variables|/Game/Blueprints/ProceduralGeneration/HexagonCellWorld.HexagonCellWorld_C|GetIndex _ashexagon_cell_world)) (.y (Variables|/Game/Blueprints/ProceduralGeneration/HexagonCellWorld.HexagonCellWorld_C|GetIndex _ashexagon_cell_world_2)) (.z (Variables|/Game/Blueprints/ProceduralGeneration/HexagonCellWorld.HexagonCellWorld_C|GetIndex _ashexagon_cell_world)) (.z (Variables|/Game/Blueprints/ProceduralGeneration/HexagonCellWorld.HexagonCellWorld_C|GetIndex _ashexagon_cell_world_2))))
    (else
      (bind _ashexagon_cell_arena (Utilities|Casting|CastToHexagonCellArena HexagonA))
      (bind _ashexagon_cell_arena_2 (Utilities|Casting|CastToHexagonCellArena HexagonB))
      (LocalVariables|SetDistance (|((((abs((x1-x2)))+(abs((y1-y2))))+(abs((z1-z2))))/2) (.x (Variables|/Game/Blueprints/ProceduralGeneration/HexagonCellArena.HexagonCellArena_C|GetIndex _ashexagon_cell_arena)) (.x (Variables|/Game/Blueprints/ProceduralGeneration/HexagonCellArena.HexagonCellArena_C|GetIndex _ashexagon_cell_arena_2)) (.y (Variables|/Game/Blueprints/ProceduralGeneration/HexagonCellArena.HexagonCellArena_C|GetIndex _ashexagon_cell_arena)) (.y (Variables|/Game/Blueprints/ProceduralGeneration/HexagonCellArena.HexagonCellArena_C|GetIndex _ashexagon_cell_arena_2)) (.z (Variables|/Game/Blueprints/ProceduralGeneration/HexagonCellArena.HexagonCellArena_C|GetIndex _ashexagon_cell_arena)) (.z (Variables|/Game/Blueprints/ProceduralGeneration/HexagonCellArena.HexagonCellArena_C|GetIndex _ashexagon_cell_arena_2))))))
  (return (Math|Float|Floor (LocalVariables|GetDistance))))