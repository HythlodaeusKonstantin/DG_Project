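; Turn-driven weather manager that runs the day/night cycle, ocean and rain changes, and ship foam effects.
; Each world turn advances an eight-step day, with timelines animating the sun, post-process and water parameter collection.
; A chance that grows until weather changes drives random shifts in wave height, post-process light and player rain particles.
; A 0.01-second self-rearming timer feeds player ship positions, headings and speeds into ocean and ship materials.
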(event Custom|WorldTurnEnded
  ;[1 0 0] Конец глобального хода
  (CallFunction|SunMovement)
  (CallFunction|ChangeWeather))

(event EventBeginPlay
  ;[1 1 1] Привязываем к диспатчеру конца глобального хода
  (EventDispatchers|BindEventtoGlobalTurnEnded (delegate Custom|WorldTurnEnded))
  ;[1 1 1] Инициализация
  (bind _asgame_inst_dg (Utilities|Casting|CastToGameInst_DG (Game|GetGameInstance)))
  (bind _output_get (Variables|Default|SetGame%20Inst%20DG _asgame_inst_dg))
  (Variables|/Game/Blueprints/GameSettings/GameInst_DG.GameInst_DG_C|SetWeatherManager _output_get self)
  (|Запускинастройкаосновныхвизуальныхэлементовпогоды))

(fn ConstructionScript)

(event Custom|SunMovement
  ;[1 1 1] Счетчик ходов
  (if (== (Variables|SunMovement|GetTurnCounter) 7)
    (Variables|SunMovement|SetTurnCounter -1)
    ;;[1 1 1] Счетчик дней
    (Math|Integer|IncrementInt (Variables|SunMovement|GetDaysCounter)
      (:%20%20
        _)))
  (Math|Integer|IncrementInt (Variables|SunMovement|GetTurnCounter)
    (:%20%20
      ;[1 1 1] Смена времени суток
      (switch int (Variables|SunMovement|GetTurnCounter)
        (:0
          (Variables|SunMovement|SetTimeOfTheDay "NewEnumerator0")
          (Development|PrintString "Наступило утро")
          (|Таймлайн-утро))
        (:1
          (Variables|SunMovement|SetTimeOfTheDay "NewEnumerator1")
          (Development|PrintString "Наступил день")
          (|Таймлайн-день1))
        (:2
          (|Таймлайн-день2))
        (:3
          (|Таймлайн-день3))
        (:4
          (Variables|SunMovement|SetTimeOfTheDay "NewEnumerator2")
          (Development|PrintString "Наступил вечер")
          (|Таймлайн-вечер))
        (:5
          (Variables|SunMovement|SetTimeOfTheDay "NewEnumerator3")
          (Development|PrintString "Наступила ночь")
          (|Таймлайн-ночь1))
        (:6
          (|Таймлайн-ночь2))
        (:7
          (|Таймлайн-ночь3))))))

(event Custom|WaitingGameLoading
  (bind _numnetplayers (Class|AdvancedSessionsLibrary|GetNumberOfNetworkPlayers))
  (bind _playercharacters (Variables|Default|GetPlayerCharacters))
  (bind _game_inst_dg (Variables|Default|GetGame%20Inst%20DG))
  (bind _player_character_dg (Variables|/Game/Blueprints/GameSettings/GameInst_DG.GameInst_DG_C|GetPlayer%20Character%20DG _game_inst_dg))
  (bind _generalnetworkmanager (Variables|/Game/Blueprints/NPC/BaseCharacter_DG.BaseCharacter_DG_C|GetGeneralNetworkManager _player_character_dg))
  ;[1 1 1] Comment
  ;;[1 1 1] Добавляем ссылки на игроков в текущей сессии для передачи данных по визуальным эффектам
  (Variables|Network|SetNum%20Net%20Players _numnetplayers)
  (for _index (range 0 (- _numnetplayers 1))
    (Utilities|IsValidWaiting _generalnetworkmanager
      (:Is%20Valid
        (Utilities|IsValid (.playercharacter (Utilities|Array|Get(acopy) (Variables|/Game/Blueprints/ReplicatedActors/ServerOnlyNetworkManager.ServerOnlyNetworkManager_C|GetPlayersInfo (Variables|/Game/Blueprints/ReplicatedActors/GeneralNetworkManager.GeneralNetworkManager_C|GetServerOnlyNetworkManager _generalnetworkmanager)) _index))
          (:Is%20Valid
            (Utilities|Array|Add _playercharacters (.playercharacter (Utilities|Array|Get(acopy) (Variables|/Game/Blueprints/ReplicatedActors/ServerOnlyNetworkManager.ServerOnlyNetworkManager_C|GetPlayersInfo (Variables|/Game/Blueprints/ReplicatedActors/GeneralNetworkManager.GeneralNetworkManager_C|GetServerOnlyNetworkManager _generalnetworkmanager)) _index))))
          (:Is%20Not%20Valid
            (Utilities|Array|Clear _playercharacters)
            (Utilities|Time|SetTimerbyEvent (delegate Custom|WaitingGameLoading) 0.01)))))))

(event Custom|WaitingGameInitialization
  (bind _numnetplayers (Class|AdvancedSessionsLibrary|GetNumberOfNetworkPlayers))
  (bind _playercharacters (Variables|Default|GetPlayerCharacters))
  (bind _game_inst_dg (Variables|Default|GetGame%20Inst%20DG))
  (bind _game_inst_dg_2 (Variables|Default|GetGame%20Inst%20DG))
  (bind _game_inst_dg_3 (Variables|Default|GetGame%20Inst%20DG))
  (bind _player_character_dg (Variables|/Game/Blueprints/GameSettings/GameInst_DG.GameInst_DG_C|GetPlayer%20Character%20DG _game_inst_dg))
  (bind _worldturnsystem (Variables|/Game/Blueprints/GameSettings/GameInst_DG.GameInst_DG_C|GetWorldTurnSystem _game_inst_dg_3))
  (bind _worldgenerationnetwork (Variables|/Game/Blueprints/GameSettings/GameInst_DG.GameInst_DG_C|GetWorldGenerationNetwork _game_inst_dg_2))
  (bind _generalnetworkmanager (Variables|/Game/Blueprints/NPC/BaseCharacter_DG.BaseCharacter_DG_C|GetGeneralNetworkManager _player_character_dg))
  ;[1 1 1] Проверяем валидность ключевых переменных
  (if (and (Utilities|IsValid _worldturnsystem) (Utilities|IsValid _worldgenerationnetwork))
    (Variables|Default|SetWorld%20Turn%20System _worldturnsystem)
    (Variables|Default|SetWorld%20Generation%20Network _worldgenerationnetwork)
    ;[1 1 1] Comment
    (Utilities|FlowControl|Sequence
      (:then_0
        (Utilities|FlowControl|Sequence
          (:then_0
            ;;[1 1 1] Добавляем ссылки на игроков в текущей сессии для передачи данных по визуальным эффектам
            (Variables|Network|SetNum%20Net%20Players _numnetplayers)
            (for _index (range 0 (- _numnetplayers 1))
              (Utilities|IsValidWaiting _generalnetworkmanager
                (:Is%20Valid
                  (Utilities|IsValid (.playercharacter (Utilities|Array|Get(acopy) (Variables|/Game/Blueprints/ReplicatedActors/ServerOnlyNetworkManager.ServerOnlyNetworkManager_C|GetPlayersInfo (Variables|/Game/Blueprints/ReplicatedActors/GeneralNetworkManager.GeneralNetworkManager_C|GetServerOnlyNetworkManager _generalnetworkmanager)) _index))
                    (:Is%20Valid
                      (Utilities|Array|Add _playercharacters (.playercharacter (Utilities|Array|Get(acopy) (Variables|/Game/Blueprints/ReplicatedActors/ServerOnlyNetworkManager.ServerOnlyNetworkManager_C|GetPlayersInfo (Variables|/Game/Blueprints/ReplicatedActors/GeneralNetworkManager.GeneralNetworkManager_C|GetServerOnlyNetworkManager _generalnetworkmanager)) _index))))
                    (:Is%20Not%20Valid
                      (Utilities|Array|Clear _playercharacters)
                      (Utilities|Time|SetTimerbyEvent (delegate Custom|WaitingGameLoading) 0.01)))))))
          (:then_1
            ;;[1 1 1] Запускаем систему ShipMovementFoam
            (CallFunction|ShipMovementFoam))))
      (:then_1
        (bind _returnvalue (Rendering|Material|CreateDynamicMaterialInstance "/Game/Materials/Postprosess/PP_Outline_Inst.PP_Outline_Inst" "None" "None" :!class /Script/Engine.KismetMaterialLibrary))
        (Variables|Default|SetPosprocessMaterial _returnvalue))
      (:then_2
        ;;[1 1 1] Создаем ссылку на солнце и постпроцесс, устанавливаем начальные настройки
        (bind _returnvalue_2 (Actor|GetActorOfClass "/Game/Blueprints/Weather/Sun.Sun_C"))
        (Variables|SunMovement|SetSun _returnvalue_2)
        (bind _returnvalue_3 (Actor|GetActorOfClass "/Script/Engine.PostProcessVolume"))
        (bind _output_get (Variables|Default|SetPostProcess _returnvalue_3))
        (Variables|/Script/Engine.PostProcessVolume|SetSettings _output_get (Utilities|Struct|MakePostProcessSettings "TEMP_ColorTemperature" 4e+03 (Math|Vector4|MakeVector4 1.0 1.0 1.0 0.6) (Utilities|Struct|MakeWeightedBlendables (Utilities|Array|MakeArray (Utilities|Struct|MakeWeightedBlendable 1.0 (Variables|Default|GetPosprocessMaterial))))))))
    (else
      (Utilities|Time|SetTimerbyEvent (delegate Custom|WaitingGameInitialization) 0.1))))

(event Custom|ChangeWeather
  ;[1 1 1] С некоторой вероятностью меняем погоду
  (if (>= (Variables|Default|GetWeatherChangeChance) (Math|Random|RandomFloatinRange 0.0 1.0))
    (Variables|Default|SetWeatherChangeChance 0.1)
    (Utilities|FlowControl|Sequence
      (:then_0
        ;[1 1 1] Изменение погоды в океане
        (Utilities|RandomCase 0.5
          (:true
            (Variables|Weather|SetOceanChanged true)
            (switch Utilities|FlowControl|Switch|SwitchonSizeEnum (Variables|Weather|GetWeatherMainType)
              (:NewEnumerator0
                (Variables|Weather|SetWeatherMainType "NewEnumerator1")
                (Variables|Weather|SetWindyOcean true))
              (:NewEnumerator1
                (Utilities|RandomCase 0.5
                  (:true
                    (Variables|Weather|SetWeatherMainType "NewEnumerator0"))
                  (:false
                    (Variables|Weather|SetWeatherMainType "NewEnumerator2"))))
              (:NewEnumerator2
                (Variables|Weather|SetWeatherMainType "NewEnumerator1")
                (Variables|Weather|SetWindyOcean true))))
          (:false
            (Variables|Weather|SetOceanChanged false)))
        ;[1 1 1] Изменение погоды в осадках
        (if (Variables|Weather|GetRainfall)
          (Utilities|RandomCase 0.25
            (:true
              (Variables|Weather|SetRainfall false))
            (:false
              (Utilities|RandomCase 0.25 :!label _label
                (:true
                  (switch Utilities|FlowControl|Switch|SwitchonSizeEnum (Variables|Weather|GetRainfallType)
                    (:NewEnumerator0
                      (Variables|Weather|SetRainfallType "NewEnumerator1"))
                    (:NewEnumerator1
                      (Utilities|RandomCase 0.5
                        (:true
                          (Variables|Weather|SetRainfallType "NewEnumerator0"))
                        (:false
                          (Variables|Weather|SetRainfallType "NewEnumerator2"))))
                    (:NewEnumerator2
                      (Variables|Weather|SetRainfallType "NewEnumerator1")))))))
          (else
            (Utilities|RandomCase 0.25
              (:true
                (Variables|Weather|SetRainfall true)
                (goto _label))))))
      (:then_1
        ;[1 1 1] Изменение океана
        (if (Variables|Weather|GetOceanChanged)
          (switch Utilities|FlowControl|Switch|SwitchonSizeEnum (Variables|Weather|GetWeatherMainType)
            (:NewEnumerator0
              ;;[1 1 1] Изменение погоды на хорошую
              (bind (_direction _wavehight _wavespeed _light) (Timeline|Calm PlayFromStart)
                (:Update
                  (Rendering|Material|SetScalarParameterValue (Variables|Default|GetMaterialParameterCollection) (Utilities|Name|MakeLiteralName "WaveHight") _wavehight :!class /Script/Engine.KismetMaterialLibrary)
                  (Rendering|Material|SetScalarParameterValue (Variables|Default|GetPosprocessMaterial) "Light" _light :!class /Script/Engine.MaterialInstanceDynamic))
                (:Finished
                  (Variables|Weather|SetRainfall false)
                  (Development|PrintString "Хорошая погода..."))))
            (:NewEnumerator1
              ;;[1 1 1] Изменение погоды на среднюю
              (if (Variables|Weather|GetWindyOcean)
                (bind (_direction_2 _wavehight_2 _wavespeed_2 _light_2) (Timeline|MiddleFromWindy PlayFromStart)
                  (:Update
                    (Rendering|Material|SetScalarParameterValue (Variables|Default|GetMaterialParameterCollection) (Utilities|Name|MakeLiteralName "WaveHight") _wavehight_2 :!class /Script/Engine.KismetMaterialLibrary)
                    (Rendering|Material|SetScalarParameterValue (Variables|Default|GetPosprocessMaterial) "Light" _light_2 :!class /Script/Engine.MaterialInstanceDynamic))
                  (:Finished
                    (Development|PrintString "Тучи на небе...")))
                (else
                  (bind (_direction_3 _wavehight_3 _wavespeed_3 _light_3) (Timeline|MiddleFromCalm PlayFromStart)
                    (:Update
                      (Rendering|Material|SetScalarParameterValue (Variables|Default|GetMaterialParameterCollection) (Utilities|Name|MakeLiteralName "WaveHight") _wavehight_3 :!class /Script/Engine.KismetMaterialLibrary)
                      (Rendering|Material|SetScalarParameterValue (Variables|Default|GetPosprocessMaterial) "Light" _light_3 :!class /Script/Engine.MaterialInstanceDynamic))
                    (:Finished
                      (Development|PrintString "Тучи на небе..."))))))
            (:NewEnumerator2
              ;;[1 1 1] Изменение погоды на плохую
              (bind (_direction_4 _wavehight_4 _wavespeed_4 _light_4) (Timeline|Windy PlayFromStart)
                (:Update
                  (Rendering|Material|SetScalarParameterValue (Variables|Default|GetMaterialParameterCollection) (Utilities|Name|MakeLiteralName "WaveHight") _wavehight_4 :!class /Script/Engine.KismetMaterialLibrary)
                  (Rendering|Material|SetScalarParameterValue (Variables|Default|GetPosprocessMaterial) "Light" _light_4 :!class /Script/Engine.MaterialInstanceDynamic))
                (:Finished
                  (Development|PrintString "Начинается буря...")))))))
      (:then_2
        ;[1 1 1] Изменение частоты осадков
        (if (Variables|Weather|GetRainfall)
          (switch Utilities|FlowControl|Switch|SwitchonSizeEnum (Variables|Weather|GetRainfallType)
            (:NewEnumerator0
              (Effects|Components|ParticleSystem|SetFloatParameter (Variables|/Game/Blueprints/Weather/Rainfall.Rainfall_C|GetParticleSystem (Variables|/Game/Blueprints/PlayerCharacter/PlayerCharacter_DG.PlayerCharacter_DG_C|GetRainfall (Variables|/Game/Blueprints/GameSettings/GameInst_DG.GameInst_DG_C|GetPlayer%20Character%20DG (Variables|Default|GetGame%20Inst%20DG)))) "Amount" 1e+03)
              (Development|PrintString "Осадки..."))
            (:NewEnumerator1
              (Effects|Components|ParticleSystem|SetFloatParameter (Variables|/Game/Blueprints/Weather/Rainfall.Rainfall_C|GetParticleSystem (Variables|/Game/Blueprints/PlayerCharacter/PlayerCharacter_DG.PlayerCharacter_DG_C|GetRainfall (Variables|/Game/Blueprints/GameSettings/GameInst_DG.GameInst_DG_C|GetPlayer%20Character%20DG (Variables|Default|GetGame%20Inst%20DG)))) "Amount" 5e+03)
              (Development|PrintString "Осадки..."))
            (:NewEnumerator2
              (Effects|Components|ParticleSystem|SetFloatParameter (Variables|/Game/Blueprints/Weather/Rainfall.Rainfall_C|GetParticleSystem (Variables|/Game/Blueprints/PlayerCharacter/PlayerCharacter_DG.PlayerCharacter_DG_C|GetRainfall (Variables|/Game/Blueprints/GameSettings/GameInst_DG.GameInst_DG_C|GetPlayer%20Character%20DG (Variables|Default|GetGame%20Inst%20DG)))) "Amount" 1e+04)
              (Development|PrintString "Осадки..."))))))
    (else
      ;[1 1 1] Каждый раз, если погода не поменялась, шанс увеличивается
      (Variables|Default|SetWeatherChangeChance (+ (Variables|Default|GetWeatherChangeChance) 0.1)))))

(event Custom|ShipMovementFoam
  (bind _numnetplayers (Class|AdvancedSessionsLibrary|GetNumberOfNetworkPlayers))
  ;[1 1 1] Система морской пены во время движения корабля
  ;;[1 1 1] Если кол-во игроков не совпадает с значением в переменной, обновляем ссылки на игроков
  (if (!= (Variables|Network|GetNum%20Net%20Players) 0)
    (if (== (Variables|Network|GetNum%20Net%20Players) (Class|AdvancedSessionsLibrary|GetNumberOfNetworkPlayers))
      ;;[1 1 1] Обновляем значение параметров в материале глобального океана
      (for (_array_element _array_index) (Variables|Default|GetPlayerCharacters)
        (Rendering|Material|SetVectorParameterValue (Variables|/Game/Blueprints/PlayerCharacter/PlayerCharacter_DG.PlayerCharacter_DG_C|GetShipMaterial _array_element) (Utilities|Array|Get(acopy) (Variables|WorldOcean|GetWorldOceanMaterial_PlayerCharacter_Location) _array_index) (Utilities|Struct|MakeLinearColor (.x (Transformation|GetActorLocation _array_element)) (.y (Transformation|GetActorLocation _array_element)) (.z (Transformation|GetActorLocation _array_element)) 1.0) :!class /Script/Engine.MaterialInstanceDynamic)
        (Rendering|Material|SetScalarParameterValue (Variables|/Game/Blueprints/ProceduralGeneration/ProceduralWorldGeneration.ProceduralWorldGeneration_C|GetWorldOceanMaterial (Variables|Default|GetWorld%20Generation%20Network)) (Utilities|Array|Get(acopy) (Variables|WorldOcean|GetWorldOceanMaterial_PlayerCharacter_Speed) _array_index) (Variables|/Game/Blueprints/CharacterComponents/Movement/MovementComponent.MovementComponent_C|GetSpeed (Variables|/Game/Blueprints/NPC/BaseCharacter_DG.BaseCharacter_DG_C|GetMovementComponent _array_element)) :!class /Script/Engine.MaterialInstanceDynamic)
        (if (> (Variables|/Game/Blueprints/CharacterComponents/Movement/MovementComponent.MovementComponent_C|GetSpeed (Variables|/Game/Blueprints/NPC/BaseCharacter_DG.BaseCharacter_DG_C|GetMovementComponent _array_element)) 0.0)
          (Rendering|Material|SetVectorParameterValue (Variables|/Game/Blueprints/ProceduralGeneration/ProceduralWorldGeneration.ProceduralWorldGeneration_C|GetWorldOceanMaterial (Variables|Default|GetWorld%20Generation%20Network)) (Utilities|Array|Get(acopy) (Variables|WorldOcean|GetWorldOceanMaterial_PlayerCharacter_Location) _array_index) (Utilities|Struct|MakeLinearColor (.x (Transformation|GetActorLocation _array_element)) (.y (Transformation|GetActorLocation _array_element)) (.x (Math|Vector|Normalize (* (Math|Vector|GetRightVector (Transformation|GetActorRotation _array_element)) -1.0))) (.y (Math|Vector|Normalize (* (Math|Vector|GetRightVector (Transformation|GetActorRotation _array_element)) -1.0)))) :!class /Script/Engine.MaterialInstanceDynamic)
          ;;[1 1 1] Вклюачем или отключаем тени - включает или отключает distancefield
          (Rendering|SetCastShadow (Variables|/Game/Blueprints/PlayerCharacter/PlayerCharacter_DG.PlayerCharacter_DG_C|GetShip _array_element) true)
          (else
            (Rendering|SetCastShadow (Variables|/Game/Blueprints/PlayerCharacter/PlayerCharacter_DG.PlayerCharacter_DG_C|GetShip _array_element) true))))
      (else
        ;;[1 1 1] Устанавливаем новые ссылки на игроков в текущей сессии
        (Variables|Network|SetNum%20Net%20Players _numnetplayers)
        (Utilities|Array|Clear (Variables|Default|GetPlayerCharacters))
        (for _index (range 0 (- _numnetplayers 1))
          (bind _asplayer_character_dg (Utilities|Casting|CastToPlayerCharacter_DG (Game|Player|GetPlayerPawn _index)))
          (Utilities|Array|Add (Variables|Default|GetPlayerCharacters) _asplayer_character_dg))))
    (Utilities|Time|SetTimerbyEvent (delegate Custom|ShipMovementFoam) 0.01)))