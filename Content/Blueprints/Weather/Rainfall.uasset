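; Weather effect that shows rain or snow for the owning player character while the game instance's WeatherManager reports rainfall.
; Each tick it reads the biome of the character's current location, taken from the cluster struct on the World Map.
; Winter maps to snow, Summer and Autumn to rain.
; The particle template is swapped only when temperature or rainfall state changes, and is cleared every tick without rainfall.
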(event EventBeginPlay
  (bind _asgame_inst_dg (Utilities|Casting|CastToGameInst_DG (Game|GetGameInstance)))
  (Variables|Default|SetGame%20Inst%20DG _asgame_inst_dg))

(event EventTick
  (params (DeltaSeconds :type Float%20%28single-precision%29))
  (bind _game_inst_dg (Variables|Default|GetGame%20Inst%20DG))
  (bind _playercharacterowner (Variables|Default|GetPlayerCharacterOwner))
  (bind _weathermanager (Variables|/Game/Blueprints/GameSettings/GameInst_DG.GameInst_DG_C|GetWeatherManager _game_inst_dg))
  (bind _currentcharacterlocation (Variables|/Game/Blueprints/NPC/BaseCharacter_DG.BaseCharacter_DG_C|GetcurrentCharacterLocation _playercharacterowner))
  (bind _biome (Variables|/Game/Blueprints/ProceduralGeneration/HexagonCellWorld.HexagonCellWorld_C|GetBiome _currentcharacterlocation))
  (Utilities|IsValid (Variables|Default|GetGame%20Inst%20DG)
    (:Is%20Valid
      (Utilities|IsValid _weathermanager
        (:Is%20Valid
          (if (Variables|/Game/Blueprints/Weather/WeatherManager.WeatherManager_C|GetRainfall _weathermanager)
            (Utilities|IsValid _currentcharacterlocation
              (:Is%20Valid
                (switch Utilities|FlowControl|Switch|SwitchonCurrentWorld (Variables|/Game/Blueprints/ProceduralGeneration/HexagonCellWorld.HexagonCellWorld_C|GetCurrentWorld _currentcharacterlocation)
                  (:NewEnumerator0
                    (Variables|Default|SetCurrentBiome (.biome (Variables|/Game/Blueprints/ProceduralGeneration/HexagonCellWorld.HexagonCellWorld_C|GetClusterStuct _currentcharacterlocation))))
                  (:NewEnumerator1
                    (Variables|Default|SetCurrentBiome _biome))
                  (:NewEnumerator2
                    (Variables|Default|SetCurrentBiome _biome)))
                (switch Utilities|FlowControl|Switch|SwitchonBiomes (Variables|Default|GetCurrentBiome)
                  (:NewEnumerator0
                    (Variables|Default|SetNewTemperature "NewEnumerator1"))
                  (:NewEnumerator1
                    (Variables|Default|SetNewTemperature "NewEnumerator0"))
                  (:NewEnumerator2
                    (Variables|Default|SetNewTemperature "NewEnumerator1")))
                (if (or (Utilities|Enum|NotEqual(Enum) (Variables|Default|GetNewTemperature) (Variables|Default|GetOldTemperature)) (Math|Boolean|NotEqual(Boolean) (Variables|/Game/Blueprints/Weather/WeatherManager.WeatherManager_C|GetRainfall (Variables|/Game/Blueprints/GameSettings/GameInst_DG.GameInst_DG_C|GetWeatherManager (Variables|Default|GetGame%20Inst%20DG))) (Variables|Default|GetRainfall)))
                  (switch Utilities|FlowControl|Switch|SwitchonTemperature (Variables|Default|GetNewTemperature)
                    (:NewEnumerator0
                      (Effects|Components|ParticleSystem|SetTemplate (Variables|Default|GetParticleSystem) "/Game/Blueprints/Weather/P_Snow.P_Snow")
                      (Variables|Default|SetOldTemperature (Variables|Default|GetNewTemperature))
                      (Variables|Default|SetRainfall true))
                    (:NewEnumerator1
                      (Effects|Components|ParticleSystem|SetTemplate (Variables|Default|GetParticleSystem) "/Game/Blueprints/Weather/P_Rain.P_Rain")
                      (Variables|Default|SetOldTemperature (Variables|Default|GetNewTemperature))
                      (Variables|Default|SetRainfall true))))))
            (else
              (Effects|Components|ParticleSystem|SetTemplate (Variables|Default|GetParticleSystem) 0)
              (Variables|Default|SetRainfall false))))))))

(fn ConstructionScript)