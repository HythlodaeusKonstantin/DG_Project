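; Construction-script tool that scatters instanced static meshes, presumably forest props for an arena, across a box area sized by XSize and YSize.
; It steps a GenerationGap grid through the box, line-tracing vertically against a single object type to find the surface.
; Hits passing a Dencity-driven random check become KeyPoints transforms with randomized rotation and height scale, which are then added as world-space instances.
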(event EventBeginPlay)

(event Collision|EventActorBeginOverlap
  (params (OtherActor :type Actor%20Object%20Reference)))

(event EventTick
  (params (DeltaSeconds :type Float%20%28single-precision%29)))

(fn ConstructionScript
  (bind _box (Variables|Default|GetBox))
  (bind _returnvalue (Components|Box|GetScaledBoxExtent _box))
  (bind _returnvalue_2 (Transformation|GetWorldLocation _box))
  (bind _returnvalue_3 (- (.y _returnvalue_2) (.y _returnvalue)))
  (Variables|Default|SetRefresh (Variables|Default|GetRefresh))
  (Utilities|Array|Clear (Variables|Default|GetKeyPoints))
  (Utilities|FlowControl|Sequence
    (:then_0
      (Components|Box|SetBoxExtent (Variables|Default|GetBox) (Math|Vector|MakeVector (Variables|Default|GetxSize) (Variables|Default|GetYSize) 5e+02) true))
    (:then_1
      (Variables|Default|SetCurrentPoint (Math|Vector|MakeVector (- (.x _returnvalue_2) (.x _returnvalue)) _returnvalue_3 (.z _returnvalue_2)))
      (for _index (range 0 (Math|Float|Truncate (/ (* 2 (Variables|Default|GetxSize)) (.x (Variables|Default|GetGenerationGap)))))
        (Variables|Default|SetCurrentPoint (Math|Vector|MakeVector (+ (.x (Variables|Default|GetCurrentPoint)) (.x (Variables|Default|GetGenerationGap))) _returnvalue_3 (.z (Variables|Default|GetCurrentPoint))))
        (for _index_2 (range 0 (Math|Float|Truncate (/ (* 2 (Variables|Default|GetYSize)) (.y (Variables|Default|GetGenerationGap)))))
          (Variables|Default|SetCurrentPoint (Math|Vector|MakeVector (.x (Variables|Default|GetCurrentPoint)) (+ (.y (Variables|Default|GetCurrentPoint)) (.y (Variables|Default|GetGenerationGap))) (.z (Variables|Default|GetCurrentPoint))))
          (bind _outhit (Collision|LineTraceForObjects (+ (Variables|Default|GetCurrentPoint) "0, 0,500.000000") (- (Variables|Default|GetCurrentPoint) "0, 0,500.000000") (Utilities|Array|MakeArray "ObjectTypeQuery7") true 0 "None"))
          (if (.bblockinghit _outhit)
            (Utilities|RandomCase (Variables|Default|GetDencity)
              (:true
                (Utilities|Array|Add (Variables|Default|GetKeyPoints) (Math|Transform|MakeTransform (Math|Vector|MakeVector (.x (.location _outhit)) (.y (.location _outhit)) (.z (.location _outhit))) (Math|Rotator|MakeRotator 0.0 0.0 (Math|Random|RandomFloatinRange 0.0 3.6e+02)) (Math|Vector|MakeVector 2.0 2.0 (Math|Random|RandomFloatinRange 1.75 2.25))))))))))
    (:then_2
      (for _array_element (Variables|Default|GetKeyPoints)
        (Class|InstancedStaticMeshComponent|AddInstanceWorldSpace (Variables|Default|GetInstancedStaticMesh) _array_element)))))