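; Clickable hex cell actor for the world map that handles mouse hover and click for player movement.
; Hover shows the hex highlight and has the player character mark a path, which is cleared when the cursor leaves.
; For impassable interactable cells, hover targets a neighbour via FindClosestNeighbour, seeded randomly then replaced by closer passable ones.
; Clicking passable or interactable cells clears any found path and calls the character's OnClick.
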(event OnBeginCursorOver(Cell)
  (params (TouchedComponent :type Primitive%20Component%20Object%20Reference))
  (bind _gameinst (Variables|Default|GetGameInst))
  (bind _player_character_dg (Variables|/Game/Blueprints/GameSettings/GameInst_DG.GameInst_DG_C|GetPlayer%20Character%20DG _gameinst))
  (bind _currentcharacterlocationworld (Variables|/Game/Blueprints/NPC/BaseCharacter_DG.BaseCharacter_DG_C|GetcurrentCharacterLocationWorld _player_character_dg))
  ;[1 1 1] Включает и отключает отображение подсветки над гексом при наведении мышкой
  (Rendering|SetVisibility (Variables|Components|GetHexArea) true false)
  (Utilities|IsValid _player_character_dg
    (:Is%20Valid
      (if (not (or (== _currentcharacterlocationworld 0) (== _currentcharacterlocationworld self)))
        (if (Variables|Initialization|GetCanPass?)
          (Variables|Interactions|SetTargetHexCell self)
          (if (== (Variables|HexagonCellWorld_C|GetCurrentWorld self) (Variables|HexagonCellWorld_C|GetCurrentWorld (Variables|/Game/Blueprints/NPC/BaseCharacter_DG.BaseCharacter_DG_C|GetcurrentCharacterLocationWorld (Variables|/Game/Blueprints/GameSettings/GameInst_DG.GameInst_DG_C|GetPlayer%20Character%20DG (Variables|Default|GetGameInst))))) :!label _label
            (Default|ClientMarkWayEvent (Variables|/Game/Blueprints/GameSettings/GameInst_DG.GameInst_DG_C|GetPlayer%20Character%20DG (Variables|Default|GetGameInst)) (Variables|Interactions|GetTargetHexCell)))
          (elif (Variables|Initialization|GetInteractabe?)
            (bind _hextargetneighbour (CallFunction|FindClosestNeighbour (Variables|Initialization|GetNeigborsHex)))
            (Variables|Interactions|SetTargetHexCell _hextargetneighbour)
            (goto _label)))))))

(event OnEndCursorOver(Cell)
  (params (TouchedComponent :type Primitive%20Component%20Object%20Reference))
  (bind _gameinst (Variables|Default|GetGameInst))
  (bind _player_character_dg (Variables|/Game/Blueprints/GameSettings/GameInst_DG.GameInst_DG_C|GetPlayer%20Character%20DG _gameinst))
  (bind _currentcharacterlocationworld (Variables|/Game/Blueprints/NPC/BaseCharacter_DG.BaseCharacter_DG_C|GetcurrentCharacterLocationWorld _player_character_dg))
  ;[1 1 1] Включает и отключает отображение подсветки над гексом при наведении мышкой
  (Rendering|SetVisibility (Variables|Components|GetHexArea) false false)
  (Utilities|IsValid _player_character_dg
    (:Is%20Valid
      (if (not (or (== _currentcharacterlocationworld 0) (== _currentcharacterlocationworld self)))
        (Default|ClientUnmarkWayEvent (Variables|/Game/Blueprints/GameSettings/GameInst_DG.GameInst_DG_C|GetPlayer%20Character%20DG (Variables|Default|GetGameInst)))))))

(event OnClicked(Cell)
  (params (TouchedComponent :type Primitive%20Component%20Object%20Reference) (ButtonPressed :type Key%20Structure))
  (bind _gameinst (Variables|Default|GetGameInst))
  (bind _player_character_dg (Variables|/Game/Blueprints/GameSettings/GameInst_DG.GameInst_DG_C|GetPlayer%20Character%20DG _gameinst))
  ;[1 1 1] Запуск логики перемещения по клику на гекс
  (if (not (== (Variables|/Game/Blueprints/NPC/BaseCharacter_DG.BaseCharacter_DG_C|GetcurrentCharacterLocationWorld (Variables|/Game/Blueprints/GameSettings/GameInst_DG.GameInst_DG_C|GetPlayer%20Character%20DG (Variables|Default|GetGameInst))) self))
    (if (Variables|Initialization|GetCanPass?)
      (Variables|Interactions|SetTargetHexCell self :!label _label)
      (if (Utilities|Array|IsValidIndex (Variables|/Game/Blueprints/NPC/BaseCharacter_DG.BaseCharacter_DG_C|GetFound%20Path (Variables|/Game/Blueprints/GameSettings/GameInst_DG.GameInst_DG_C|GetPlayer%20Character%20DG (Variables|Default|GetGameInst))))
        (Default|ClientUnmarkWayEvent _player_character_dg))
      (Default|OnClick _player_character_dg self (Variables|Initialization|GetInteractabe?))
      (elif (Variables|Initialization|GetInteractabe?)
        (goto _label)))))

(event EventBeginPlay
  ;[0 0 0] Инициализация
  (|CallParentFunction))

(fn ConstructionScript)

(fn FindClosestNeighbour
  (params (Neigbours :type Array%20of%20Hexagon%20Cell%20World%20Object%20References))
  (bind _output_get (LocalVariables|SetHexTarget (.OutItem (Utilities|Array|Random Neigbours))))
  (LocalVariables|SetMinDist (Transformation|GetDistanceTo _output_get (Variables|/Game/Blueprints/GameSettings/GameInst_DG.GameInst_DG_C|GetPlayer%20Character%20DG (Variables|Default|GetGameInst))))
  (for _array_element Neigbours
    (if (< (Transformation|GetDistanceTo _array_element (Variables|/Game/Blueprints/GameSettings/GameInst_DG.GameInst_DG_C|GetPlayer%20Character%20DG (Variables|Default|GetGameInst))) (LocalVariables|GetMinDist))
      (if (Variables|HexagonCellWorld_C|GetCanPass? _array_element)
        (LocalVariables|SetMinDist (Transformation|GetDistanceTo _array_element (Variables|/Game/Blueprints/GameSettings/GameInst_DG.GameInst_DG_C|GetPlayer%20Character%20DG (Variables|Default|GetGameInst))))
        (LocalVariables|SetHexTarget _array_element))))
  (return (LocalVariables|GetHexTarget)))