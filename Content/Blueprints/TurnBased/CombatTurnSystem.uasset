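; Turn-based combat manager that registers itself with the game instance and alternates rounds between player and enemy sides.
; StartCombat sorts each side by ascending Initiation, always gives players the first turn despite the computed initiative comparison, and starts the battle through CombatManager.
; On the server, each turn end refills the active character's action points, rotates it to the queue's back and activates the next, flipping sides after a full cycle.
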(event Custom|Start%20Combat
  (params (PlayerCharacters :type Array%20of%20Base%20Character%20DG%20Object%20References) (EnemyCharacters :type Array%20of%20Base%20Character%20DG%20Object%20References))
  (Utilities|FlowControl|Sequence
    (:then_0
      (bind (_playersinitiative _playersincombat _enemyincombat) (CallFunction|FulfillTurnBasedQueue PlayerCharacters EnemyCharacters))
      (Variables|Default|SetPlayers%20in%20Combat _playersincombat)
      (Variables|Default|SetEnemy%20in%20Combat _enemyincombat)
      (bind _output_get (Variables|Default|SetPlayers%20Initiative true))
      (if _output_get
        (Variables|/Game/Blueprints/NPC/BaseCharacter_DG.BaseCharacter_DG_C|SetCharacterMove (Utilities|Array|Get(acopy) (Variables|Default|GetPlayers%20in%20Combat)) true)
        (else
          (Variables|/Game/Blueprints/NPC/BaseCharacter_DG.BaseCharacter_DG_C|SetCharacterMove (Utilities|Array|Get(acopy) (Variables|Default|GetEnemy%20in%20Combat)) true))))
    (:then_1
      (Default|StartBattle-Server (Variables|/Game/Blueprints/NPC/BaseCharacter_DG.BaseCharacter_DG_C|GetCombatManager (Utilities|Array|Get(acopy) PlayerCharacters))))))

(event Custom|OnTurnEnded
  (if (Networking|IsServer)
    (if (== (Variables|Default|GetLargeMoveCounter) 0)
      (if (Variables|Default|GetPlayers%20Initiative)
        (Variables|Default|SetCurrentCharactersQueue (Variables|Default|GetPlayers%20in%20Combat))
        (else
          (Variables|Default|SetCurrentCharactersQueue (Variables|Default|GetEnemy%20in%20Combat)))))
    (Variables|/Game/Blueprints/NPC/BaseCharacter_DG.BaseCharacter_DG_C|SetCharacterMove (Utilities|Array|Get(acopy) (Variables|Default|GetCurrentCharactersQueue)) false)
    (Variables|/Game/Blueprints/CharacterComponents/CharacterStats/StatsComponent.StatsComponent_C|SetActionPoints (Variables|/Game/Blueprints/NPC/BaseCharacter_DG.BaseCharacter_DG_C|GetStatsComponent (Utilities|Array|Get(acopy) (Variables|Default|GetCurrentCharactersQueue))) 10)
    (bind _newqueue (CallFunction|MoveQueue (Variables|Default|GetCurrentCharactersQueue) (Utilities|Array|Get(acopy) (Variables|Default|GetCurrentCharactersQueue))))
    (Variables|Default|SetCurrentCharactersQueue _newqueue)
    (bind _result (Math|Integer|IncrementInt (Variables|Default|GetLargeMoveCounter))
      (:%20%20
        (if (>= _result (Utilities|Array|Length (Variables|Default|GetCurrentCharactersQueue)))
          (Utilities|FlowControl|Sequence
            (:then_0
              (Variables|Default|SetPlayers%20Initiative (not (Variables|Default|GetPlayers%20Initiative)))
              (Variables|Default|SetLargeMoveCounter 0)
              (Development|PrintString "Конец большого хода"))
            (:then_1
              (if (Variables|Default|GetPlayers%20Initiative)
                (Variables|/Game/Blueprints/NPC/BaseCharacter_DG.BaseCharacter_DG_C|SetCharacterMove (Utilities|Array|Get(acopy) (Variables|Default|GetPlayers%20in%20Combat)) true)
                (else
                  (Variables|/Game/Blueprints/NPC/BaseCharacter_DG.BaseCharacter_DG_C|SetCharacterMove (Utilities|Array|Get(acopy) (Variables|Default|GetEnemy%20in%20Combat)) true)))))
          (else
            (Variables|/Game/Blueprints/NPC/BaseCharacter_DG.BaseCharacter_DG_C|SetCharacterMove (Utilities|Array|Get(acopy) (Variables|Default|GetCurrentCharactersQueue)) true)
            (Development|PrintString "Конец малого хода")))))))

(event EventBeginPlay
  (|Инициализация)
  (EventDispatchers|BindEventtoTurnEnded (delegate Custom|OnTurnEnded)))

(fn ConstructionScript)

(fn SortArray
  (params (Array :type Array%20of%20Base%20Character%20DG%20Object%20References))
  (bind _initiationtosort (LocalVariables|GetInitiationToSort))
  (bind _indexofminvalue (Math|Integer|MinOfIntArray _initiationtosort))
  (for _array_element Array
    (Utilities|Array|Add (LocalVariables|GetInitiationToSort) (Variables|/Game/Blueprints/CharacterComponents/CharacterStats/StatsComponent.StatsComponent_C|GetInitiation (Variables|/Game/Blueprints/NPC/BaseCharacter_DG.BaseCharacter_DG_C|GetStatsComponent _array_element))))
  (bind _output_get (LocalVariables|SetArrayLenght (- (Utilities|Array|Length _initiationtosort) 1)))
  (for _index (range 0 _output_get)
    (Utilities|Array|SetArrayElem (LocalVariables|GetArrayToSort) _index (Utilities|Array|Get(acopy) Array _indexofminvalue) true)
    (Utilities|Array|SetArrayElem _initiationtosort _indexofminvalue 9999))
  (return (LocalVariables|GetArrayToSort)))

(fn ComparePlayerEnemyInitiation
  (params (Players :type Array%20of%20Base%20Character%20DG%20Object%20References) (Enemy :type Array%20of%20Base%20Character%20DG%20Object%20References))
  (for _array_element Players
    (LocalVariables|SetPlayersInitiation (+ (Variables|/Game/Blueprints/CharacterComponents/CharacterStats/StatsComponent.StatsComponent_C|GetInitiation (Variables|/Game/Blueprints/NPC/BaseCharacter_DG.BaseCharacter_DG_C|GetStatsComponent _array_element)) (LocalVariables|GetPlayersInitiation))))
  (for _array_element_2 Enemy
    (LocalVariables|SetEnemyInitiation (+ (Variables|/Game/Blueprints/CharacterComponents/CharacterStats/StatsComponent.StatsComponent_C|GetInitiation (Variables|/Game/Blueprints/NPC/BaseCharacter_DG.BaseCharacter_DG_C|GetStatsComponent _array_element_2)) (LocalVariables|GetEnemyInitiation))))
  (return (>= (LocalVariables|GetPlayersInitiation) (LocalVariables|GetEnemyInitiation))))

(fn FulfillTurnBasedQueue
  (params (PlayerCharacters :type Array%20of%20Base%20Character%20DG%20Object%20References) (EnemyCharacters :type Array%20of%20Base%20Character%20DG%20Object%20References))
  (bind _sortedarray (CallFunction|SortArray PlayerCharacters))
  (LocalVariables|SetPlayerCharactersInCombat _sortedarray)
  (bind _sortedarray_2 (CallFunction|SortArray EnemyCharacters))
  (LocalVariables|SetEnemyCharactersInCombat _sortedarray_2)
  (bind _playershaveinitiative (CallFunction|ComparePlayerEnemyInitiation (LocalVariables|GetPlayerCharactersInCombat) (LocalVariables|GetEnemyCharactersInCombat)))
  (bind _output_get (LocalVariables|SetPlayersHaveInitiative _playershaveinitiative))
  (return _output_get (LocalVariables|GetPlayerCharactersInCombat) (LocalVariables|GetEnemyCharactersInCombat)))

(fn MoveQueue
  (params (Queue :type Array%20of%20Base%20Character%20DG%20Object%20References) (CurrentElement :type Base%20Character%20DG%20Object%20Reference%20%28by%20ref%29))
  (LocalVariables|SetCurrentQueue Queue)
  (LocalVariables|SetCurrentCharacterElement CurrentElement)
  (Utilities|Array|RemoveItem (LocalVariables|GetCurrentQueue) (LocalVariables|GetCurrentCharacterElement))
  (Utilities|Array|Add (LocalVariables|GetCurrentQueue) (LocalVariables|GetCurrentCharacterElement))
  (return (LocalVariables|GetCurrentQueue)))