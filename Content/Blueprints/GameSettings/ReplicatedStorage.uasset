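; ReplicatedStorage shares the active world save between server and clients and registers itself on GameInst_DG.
; On BeginPlay the authority copies island, world-generation and save fields from the active WorldStorage save into its variables, while remotes write those variables into their save.
; Both then call LoadWorld and set InGame.
; SaveGameMulticast overwrites the active save from the passed data and calls GenerateWorld; an older sync graph is left unconnected.
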(event Custom|SaveGameMulticast
  (params (WorldStorageSaveData :type World%20Storage%20Save%20Data%20Structure%20%28by%20ref%29))
  (bind (_worldgenerationhexagondata _worldgenerationnetworkdata _worlddatasaved_ _islandsonworldmap _indexofcurrentislandinarray _savename) (Utilities|Struct|BreakWorldStorageSaveData WorldStorageSaveData))
  (bind _game_inst_dg (Variables|Default|GetGame%20Inst%20DG))
  (bind _activesavegame_worldstorage (Variables|/Game/Blueprints/GameSettings/GameInst_DG.GameInst_DG_C|GetActiveSaveGame_WorldStorage _game_inst_dg))
  (Utilities|FlowControl|Sequence
    (:then_0
      (Variables|/Game/Blueprints/GameSettings/WorldStorage.WorldStorage_C|SetIndexOfCurrentIslandInArray _activesavegame_worldstorage _indexofcurrentislandinarray)
      (Variables|/Game/Blueprints/GameSettings/WorldStorage.WorldStorage_C|SetIslandsOnWorldMap _activesavegame_worldstorage _islandsonworldmap)
      (Variables|/Game/Blueprints/GameSettings/WorldStorage.WorldStorage_C|SetSaveName _activesavegame_worldstorage _savename)
      (Variables|/Game/Blueprints/GameSettings/WorldStorage.WorldStorage_C|SetWorldDataSaved? _activesavegame_worldstorage _worlddatasaved_)
      (Variables|/Game/Blueprints/GameSettings/WorldStorage.WorldStorage_C|SetWorldGenerationHexagonData _activesavegame_worldstorage _worldgenerationhexagondata)
      (Variables|/Game/Blueprints/GameSettings/WorldStorage.WorldStorage_C|SetWorldGenerationNetworkData _activesavegame_worldstorage _worldgenerationnetworkdata))
    (:then_1
      (Default|GenerateWorld (Variables|Default|GetGame%20Inst%20DG)))))

(event EventBeginPlay
  (bind _asgame_inst_dg (Utilities|Casting|CastToGameInst_DG (Game|GetGameInstance)))
  (bind _output_get (Variables|Default|SetGame%20Inst%20DG _asgame_inst_dg))
  (Variables|/Game/Blueprints/GameSettings/GameInst_DG.GameInst_DG_C|SetReplicatedStorage _output_get self)
  (Networking|SwitchHasAuthority
    (:Authority
      (Variables|ActiveSaveGameWorldStorage|SetIndex%20Of%20Current%20Island%20in%20Array (Variables|/Game/Blueprints/GameSettings/WorldStorage.WorldStorage_C|GetIndexOfCurrentIslandInArray (Variables|/Game/Blueprints/GameSettings/GameInst_DG.GameInst_DG_C|GetActiveSaveGame_WorldStorage (Variables|Default|GetGame%20Inst%20DG))))
      (Variables|ActiveSaveGameWorldStorage|SetIslands%20on%20World%20Map (Variables|/Game/Blueprints/GameSettings/WorldStorage.WorldStorage_C|GetIslandsOnWorldMap (Variables|/Game/Blueprints/GameSettings/GameInst_DG.GameInst_DG_C|GetActiveSaveGame_WorldStorage (Variables|Default|GetGame%20Inst%20DG))))
      (Variables|ActiveSaveGameWorldStorage|SetSave%20Name (Variables|/Game/Blueprints/GameSettings/WorldStorage.WorldStorage_C|GetSaveName (Variables|/Game/Blueprints/GameSettings/GameInst_DG.GameInst_DG_C|GetActiveSaveGame_WorldStorage (Variables|Default|GetGame%20Inst%20DG))))
      (Variables|ActiveSaveGameWorldStorage|SetWorld%20Data%20Saved? (Variables|/Game/Blueprints/GameSettings/WorldStorage.WorldStorage_C|GetWorldDataSaved? (Variables|/Game/Blueprints/GameSettings/GameInst_DG.GameInst_DG_C|GetActiveSaveGame_WorldStorage (Variables|Default|GetGame%20Inst%20DG))))
      (Variables|ActiveSaveGameWorldStorage|SetWorld%20Generation%20Hexagon%20Data (Variables|/Game/Blueprints/GameSettings/WorldStorage.WorldStorage_C|GetWorldGenerationHexagonData (Variables|/Game/Blueprints/GameSettings/GameInst_DG.GameInst_DG_C|GetActiveSaveGame_WorldStorage (Variables|Default|GetGame%20Inst%20DG))))
      (Variables|ActiveSaveGameWorldStorage|SetWorld%20Generation%20Network%20Data (Variables|/Game/Blueprints/GameSettings/WorldStorage.WorldStorage_C|GetWorldGenerationNetworkData (Variables|/Game/Blueprints/GameSettings/GameInst_DG.GameInst_DG_C|GetActiveSaveGame_WorldStorage (Variables|Default|GetGame%20Inst%20DG))))
      (Default|LoadWorld (Variables|Default|GetGame%20Inst%20DG) :!label _label)
      (Variables|/Game/Blueprints/GameSettings/GameInst_DG.GameInst_DG_C|SetInGame? (Variables|Default|GetGame%20Inst%20DG) true))
    (:Remote
      (Utilities|FlowControl|Sequence
        (:then_0
          (Variables|/Game/Blueprints/GameSettings/WorldStorage.WorldStorage_C|SetIndexOfCurrentIslandInArray (Variables|/Game/Blueprints/GameSettings/GameInst_DG.GameInst_DG_C|GetActiveSaveGame_WorldStorage (Variables|Default|GetGame%20Inst%20DG)) (Variables|ActiveSaveGameWorldStorage|GetIndex%20Of%20Current%20Island%20in%20Array))
          (Variables|/Game/Blueprints/GameSettings/WorldStorage.WorldStorage_C|SetIslandsOnWorldMap (Variables|/Game/Blueprints/GameSettings/GameInst_DG.GameInst_DG_C|GetActiveSaveGame_WorldStorage (Variables|Default|GetGame%20Inst%20DG)) (Variables|ActiveSaveGameWorldStorage|GetIslands%20on%20World%20Map))
          (Variables|/Game/Blueprints/GameSettings/WorldStorage.WorldStorage_C|SetSaveName (Variables|/Game/Blueprints/GameSettings/GameInst_DG.GameInst_DG_C|GetActiveSaveGame_WorldStorage (Variables|Default|GetGame%20Inst%20DG)) (Variables|ActiveSaveGameWorldStorage|GetSave%20Name))
          (Variables|/Game/Blueprints/GameSettings/WorldStorage.WorldStorage_C|SetWorldDataSaved? (Variables|/Game/Blueprints/GameSettings/GameInst_DG.GameInst_DG_C|GetActiveSaveGame_WorldStorage (Variables|Default|GetGame%20Inst%20DG)) (Variables|ActiveSaveGameWorldStorage|GetWorld%20Data%20Saved?))
          (Variables|/Game/Blueprints/GameSettings/WorldStorage.WorldStorage_C|SetWorldGenerationHexagonData (Variables|/Game/Blueprints/GameSettings/GameInst_DG.GameInst_DG_C|GetActiveSaveGame_WorldStorage (Variables|Default|GetGame%20Inst%20DG)) (Variables|ActiveSaveGameWorldStorage|GetWorld%20Generation%20Hexagon%20Data))
          (Variables|/Game/Blueprints/GameSettings/WorldStorage.WorldStorage_C|SetWorldGenerationNetworkData (Variables|/Game/Blueprints/GameSettings/GameInst_DG.GameInst_DG_C|GetActiveSaveGame_WorldStorage (Variables|Default|GetGame%20Inst%20DG)) (Variables|ActiveSaveGameWorldStorage|GetWorld%20Generation%20Network%20Data)))
        (:then_1
          (goto _label))))))

(fn ConstructionScript)