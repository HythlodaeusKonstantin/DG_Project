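; ArenaNetwork is an actor that builds and manages the hexagon cell grid of a procedurally generated battle arena.
; Generate spawns HexagonCellArena actors in zigzag columns with three-axis indices and links neighbours, while other functions snap cells to the landscape and bucket their heights into eleven relative levels.
; On BeginPlay it registers itself in the game instance through its creating LocationManager and applies landscape and forest materials matching the island's biome.
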(event EventBeginPlay
  (|Инициализация)
  (Utilities|FlowControl|Sequence
    (:then_0
      (bind _outactors (Actor|GetAllActorsOfClass "/Game/Blueprints/ReplicatedActors/LocationManager.LocationManager_C"))
      ;[1 1 1] Добавление данного нетворка в мапу - это делает только Location Manager, создавший данный нетворк
      (for _array_element _outactors
        (if (Variables|/Game/Blueprints/ReplicatedActors/LocationManager.LocationManager_C|GetArenaCreator _array_element)
          (Variables|/Game/Blueprints/ReplicatedActors/LocationManager.LocationManager_C|SetArenaCreator _array_element false)
          (Utilities|Map|Add (Variables|/Game/Blueprints/GameSettings/GameInst_DG.GameInst_DG_C|GetArenaNetworks (Variables|Default|GetGame%20Inst%20DG)) (Variables|/Game/Blueprints/ReplicatedActors/LocationManager.LocationManager_C|GetArenaKeys _array_element) self))))
    (:then_1
      (Utilities|FlowControl|Sequence
        (:then_0
          (bind _output_get (Variables|Default|SetBiome (Variables|/Game/Blueprints/ProceduralGeneration/ProceduralHexagonalNetwork.ProceduralHexagonalNetwork_C|GetBiom (.Value (Utilities|Map|Find (Variables|/Game/Blueprints/GameSettings/GameInst_DG.GameInst_DG_C|GetIslandGenerationNetworks (Variables|Default|GetGame%20Inst%20DG)) (.IslandIndex (Utilities|Struct|BreakArenaKey (Variables|/Game/Blueprints/ReplicatedActors/LocationManager.LocationManager_C|GetArenaKeys _array_element))))))))
          (switch Utilities|FlowControl|Switch|SwitchonBiomes _output_get
            (:NewEnumerator0
              (Variables|Materials|SetLandscapeMaterial "/Game/Materials/Landscape/LandscapeSummerArena_Inst.LandscapeSummerArena_Inst")
              (Variables|Materials|SetForestMaterial "/Game/Materials/Environment/Forest/ForestSummer_Inst.ForestSummer_Inst"))
            (:NewEnumerator1
              (Variables|Materials|SetLandscapeMaterial "/Game/Materials/Landscape/LandscapeWinterArena_Inst.LandscapeWinterArena_Inst")
              (Variables|Materials|SetForestMaterial "/Game/Materials/Environment/Forest/ForestWinter_Inst.ForestWinter_Inst"))
            (:NewEnumerator2
              (Variables|Materials|SetLandscapeMaterial "/Game/Materials/Landscape/LandscapeAutumnArena_Inst.LandscapeAutumnArena_Inst")
              (Variables|Materials|SetForestMaterial "/Game/Materials/Environment/Forest/ForestAutumn_Inst.ForestAutumn_Inst"))))
        (:then_1
          (Rendering|Material|SetMaterial (Variables|Default|GetArenaLandscape) 0 (Variables|Materials|GetLandscapeMaterial))
          (for _array_element_2 (Variables|Default|GetForestDistibutionArenaTools)
            (Rendering|Material|SetMaterial (Variables|/Game/Blueprints/Props/ForestDistibutionArenaTool.ForestDistibutionArenaTool_C|GetInstancedStaticMesh _array_element_2) 0 (Variables|Materials|GetForestMaterial))))))))

(fn ConstructionScript
  (Utilities|FlowControl|Sequence
    (:then_0
      (Variables|Default|SetCoordinatStart "0, 0, 0")
      (for _index (range 1 (Variables|Default|GetMoveRight))
        (Variables|Default|SetCoordinatStart (+ (Variables|Default|GetCoordinatStart) (Variables|Default|GetCoord_2))))
      (for _index_2 (range 1 (Variables|Default|GetMoveUp))
        (Variables|Default|SetCoordinatStart (+ (Variables|Default|GetCoordinatStart) "0,150.000000, 0"))))
    (:then_1
      ;[1 1 1] Находим центральную точку арены - для тумана войны
      (Variables|Default|SetArenaOrigin (.Origin (Collision|GetComponentBounds (Variables|Default|GetArenaLandscape)))))))

(fn Generate
  (Variables|Default|SetCoordinatStart "0, 0, 0")
  (for _index (range 1 (Variables|Default|GetMoveRight))
    (Variables|Default|SetCoordinatStart (+ (Variables|Default|GetCoordinatStart) (Variables|Default|GetCoord_2))))
  (for _index_2 (range 1 (Variables|Default|GetMoveUp))
    (Variables|Default|SetCoordinatStart (+ (Variables|Default|GetCoordinatStart) "0,150.000000, 0")))
  (CallFunction|Clean)
  (Utilities|FlowControl|Sequence
    (:then_0
      (Variables|Default|SetCurrent%20Ordinar%20Index 0)
      (Variables|Default|SetCoordCurrent (Variables|Default|GetCoordinatStart))
      (Variables|Default|SetIndexCurrent "0, 0, 0")
      (for _index_3 (range 0 (Variables|Default|GetWidth))
        (LocalVariables|SetflipFlopBool true)
        (bind _returnvalue (Game|SpawnActorfromClass "/Game/Blueprints/ProceduralGeneration/HexagonCellArena.HexagonCellArena_C" (Math|Conversions|ToTransform(Vector) (Variables|Default|GetCoordCurrent)) "Undefined" 0 (Variables|Default|GetCoordCurrent) (Utilities|CalculateNeighbours) 0 true "NewEnumerator2" (Variables|Default|GetIndexCurrent) (Variables|Default|GetCurrent%20Ordinar%20Index) 0))
        (Utilities|Map|Add (Variables|Default|GetHexAllMap) (Variables|Default|GetIndexCurrent) _returnvalue)
        (Utilities|Map|Add (Variables|Default|GetHexAllMapOrdinarIndex) (Variables|Default|GetCurrent%20Ordinar%20Index) _returnvalue)
        (Math|Integer|IncrementInt (Variables|Default|GetCurrent%20Ordinar%20Index)
          (:%20%20
            (LocalVariables|SetlastIndexWidth (Variables|Default|GetIndexCurrent))
            (LocalVariables|SetlastCoordWidth (Variables|Default|GetCoordCurrent))
            (for _index_4 (range 0 (Variables|Default|GetHeight))
              (if (LocalVariables|GetflipFlopBool)
                (Variables|Default|SetCoordCurrent (+ (Variables|Default|GetCoordCurrent) (Variables|Default|GetCoord_3)))
                (Variables|Default|SetIndexCurrent (+ (Variables|Default|GetIndexCurrent) "1.000000,0.000000,1.000000"))
                (LocalVariables|SetflipFlopBool false)
                (else
                  (Variables|Default|SetCoordCurrent (+ (Variables|Default|GetCoordCurrent) (Variables|Default|GetCoord_4)))
                  (Variables|Default|SetIndexCurrent (+ (Variables|Default|GetIndexCurrent) "0.000000,1.000000,1.000000"))
                  (LocalVariables|SetflipFlopBool true)))
              (bind _returnvalue_2 (Game|SpawnActorfromClass "/Game/Blueprints/ProceduralGeneration/HexagonCellArena.HexagonCellArena_C" (Math|Conversions|ToTransform(Vector) (Variables|Default|GetCoordCurrent)) "Undefined" 0 (Variables|Default|GetCoordCurrent) (Utilities|CalculateNeighbours) 0 true "NewEnumerator2" (Variables|Default|GetIndexCurrent) (Variables|Default|GetCurrent%20Ordinar%20Index) 0))
              (Utilities|Map|Add (Variables|Default|GetHexAllMap) (Variables|Default|GetIndexCurrent) _returnvalue_2)
              (Utilities|Map|Add (Variables|Default|GetHexAllMapOrdinarIndex) (Variables|Default|GetCurrent%20Ordinar%20Index) _returnvalue_2)
              (Math|Integer|IncrementInt (Variables|Default|GetCurrent%20Ordinar%20Index)))
            ;[1 1 1] Сдвигаемся вправо
            (Variables|Default|SetCoordCurrent (+ (LocalVariables|GetlastCoordWidth) (Variables|Default|GetCoord_2)))
            (Variables|Default|SetIndexCurrent (+ (LocalVariables|GetlastIndexWidth) "1.000000,-1.000000,0.000000"))))))
    (:then_1
      ;[1 1 1] Set Up Neigbors
      (bind _values (Utilities|Map|Values (Variables|Default|GetHexAllMap)))
      (for _array_element _values
        (for _array_element_2 (Variables|/Game/Blueprints/ProceduralGeneration/HexagonCellArena.HexagonCellArena_C|GetNeigbors _array_element)
          (if (.ReturnValue (Utilities|Map|Find (Variables|Default|GetHexAllMap) _array_element_2))
            (Utilities|Array|Add (Variables|/Game/Blueprints/ProceduralGeneration/HexagonCellArena.HexagonCellArena_C|GetNeigborsHex _array_element) (.Value (Utilities|Map|Find (Variables|Default|GetHexAllMap) _array_element_2))))))
      ;[1 1 1] CreateHexagonCellsAll
      (bind _values_2 (Utilities|Map|Values (Variables|Default|GetHexAllMap)))
      (Variables|Default|SetHexagonCells-ALL _values_2))))

(fn Clean
  (for _array_element (Variables|Default|GetHexagonCells-ALL)
    (Actor|DestroyActor _array_element))
  (Utilities|Map|Clear (Variables|Default|GetHexAllMap))
  (Utilities|Array|Clear (Variables|Default|GetHexagonCells-ALL))
  (Utilities|Map|Clear (Variables|Default|GetHexAllMapOrdinarIndex)))

(fn SnapHextoLandscape
  (for _array_element (Variables|Default|GetHexagonCells-ALL)
    (Default|SnaptoLandscape _array_element)))

(fn CalculateHexagonHightLevel
  (bind _hexagoncells_all (Variables|Default|GetHexagonCells-ALL))
  (bind _hexarenalocationz (Variables|Default|GetHexArenaLocationZ))
  (bind _hexarenalocation (Variables|Default|GetHexArenaLocation))
  (bind _indexofminvalue (Math|Float|MinOfFloatArray _hexarenalocationz))
  (bind _output (Utilities|Array|Get(acopy) _hexarenalocation _indexofminvalue))
  (Utilities|Array|Clear (Variables|Default|GetHexArenaLocationZ))
  (Utilities|Array|Clear (Variables|Default|GetHexArenaLocation))
  (for _array_element _hexagoncells_all
    (Utilities|Array|Add (Variables|Default|GetHexArenaLocationZ) (.z (Transformation|GetWorldLocation (Variables|/Game/Blueprints/ProceduralGeneration/HexagonCellArena.HexagonCellArena_C|GetHexagonPointLocation _array_element))))
    (Utilities|Array|Add (Variables|Default|GetHexArenaLocation) (Math|Vector|MakeVector 0.0 0.0 (.z (Transformation|GetWorldLocation (Variables|/Game/Blueprints/ProceduralGeneration/HexagonCellArena.HexagonCellArena_C|GetHexagonPointLocation _array_element))))))
  (for _array_element_2 _hexagoncells_all
    (switch int (Math|Float|Round (* 10 (/ (Math|Vector|Distance(Vector) (Math|Vector|MakeVector 0.0 0.0 (.z (Transformation|GetWorldLocation (Variables|/Game/Blueprints/ProceduralGeneration/HexagonCellArena.HexagonCellArena_C|GetHexagonPointLocation _array_element_2)))) _output) (Math|Vector|Distance(Vector) (Utilities|Array|Get(acopy) _hexarenalocation (.IndexOfMaxValue (Math|Float|MaxOfFloatArray _hexarenalocationz))) _output))))
      (:Default
        (Development|PrintString "Что-то пошло не так..."))
      (:0
        (Variables|/Game/Blueprints/ProceduralGeneration/HexagonCellArena.HexagonCellArena_C|SetHexHeight _array_element_2 "NewEnumerator0"))
      (:1
        (Variables|/Game/Blueprints/ProceduralGeneration/HexagonCellArena.HexagonCellArena_C|SetHexHeight _array_element_2 "NewEnumerator1"))
      (:2
        (Variables|/Game/Blueprints/ProceduralGeneration/HexagonCellArena.HexagonCellArena_C|SetHexHeight _array_element_2 "NewEnumerator2"))
      (:3
        (Variables|/Game/Blueprints/ProceduralGeneration/HexagonCellArena.HexagonCellArena_C|SetHexHeight _array_element_2 "NewEnumerator3"))
      (:4
        (Variables|/Game/Blueprints/ProceduralGeneration/HexagonCellArena.HexagonCellArena_C|SetHexHeight _array_element_2 "NewEnumerator4"))
      (:5
        (Variables|/Game/Blueprints/ProceduralGeneration/HexagonCellArena.HexagonCellArena_C|SetHexHeight _array_element_2 "NewEnumerator11"))
      (:6
        (Variables|/Game/Blueprints/ProceduralGeneration/HexagonCellArena.HexagonCellArena_C|SetHexHeight _array_element_2 "NewEnumerator6"))
      (:7
        (Variables|/Game/Blueprints/ProceduralGeneration/HexagonCellArena.HexagonCellArena_C|SetHexHeight _array_element_2 "NewEnumerator7"))
      (:8
        (Variables|/Game/Blueprints/ProceduralGeneration/HexagonCellArena.HexagonCellArena_C|SetHexHeight _array_element_2 "NewEnumerator8"))
      (:9
        (Variables|/Game/Blueprints/ProceduralGeneration/HexagonCellArena.HexagonCellArena_C|SetHexHeight _array_element_2 "NewEnumerator9"))
      (:10
        (Variables|/Game/Blueprints/ProceduralGeneration/HexagonCellArena.HexagonCellArena_C|SetHexHeight _array_element_2 "NewEnumerator10")))))