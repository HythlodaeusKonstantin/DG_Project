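; BaseEnemy_DG is a base enemy NPC Blueprint that toggles an outline when the mouse cursor hovers over it.
; BaseSkeletalMesh's begin and end cursor-over events call OutlineActor with true or false.
; OutlineActor loops over the direct children of CharacterCollection and sets Render Custom Depth on each skeletal mesh, covering multi-part characters.
; BeginPlay is a disabled stub and the construction script only calls its parent.
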(event OnBeginCursorOver(BaseSkeletalMesh)
  (params (TouchedComponent :type Primitive%20Component%20Object%20Reference))
  ;[0 1 0] Включает\выключает outline
  (CallFunction|OutlineActor true))

(event OnEndCursorOver(BaseSkeletalMesh)
  (params (TouchedComponent :type Primitive%20Component%20Object%20Reference))
  ;[0 1 0] Включает\выключает outline
  (CallFunction|OutlineActor false))

(event EventBeginPlay
  (|CallParentFunction) ; This node is disabled and will not be called.\nDrag off pins to build functionality.
)

(fn ConstructionScript
  (|CallParentFunction))

(fn OutlineActor
  (params (Active :type Boolean))
  (for _array_element (Components|GetChildrenComponents (Variables|Default|GetCharacterCollection) false)
    (if (.bSuccess (Utilities|Casting|CastToSkeletalMeshComponent _array_element))
      (Rendering|SetRenderCustomDepth (.AsSkeletal%20Mesh%20Component (Utilities|Casting|CastToSkeletalMeshComponent _array_element)) Active))))