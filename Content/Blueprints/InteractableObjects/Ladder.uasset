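; Ladder is an interactable object Blueprint that responds to cursor hover and clicks on its Box component.
; Box cursor-over events toggle OutlineActor on and off, and a Box click calls OnClick.
; Both functions only call their parent implementations, so the outline and click behavior come from the parent class, with no ladder-specific logic here.
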(event OnBeginCursorOver(Box)
  (params (TouchedComponent :type Primitive%20Component%20Object%20Reference))
  (CallFunction|OutlineActor true))

(event OnEndCursorOver(Box)
  (params (TouchedComponent :type Primitive%20Component%20Object%20Reference))
  (CallFunction|OutlineActor false))

(event OnClicked(Box)
  (params (TouchedComponent :type Primitive%20Component%20Object%20Reference) (ButtonPressed :type Key%20Structure :default "None"))
  (CallFunction|OnClick))

(event EventBeginPlay
  (|CallParentFunction) ; This node is disabled and will not be called.\nDrag off pins to build functionality.
)

(event Collision|EventActorBeginOverlap
  (params (OtherActor :type Actor%20Object%20Reference))
  (|CallParentFunction OtherActor) ; This node is disabled and will not be called.\nDrag off pins to build functionality.
)

(event EventTick
  (params (DeltaSeconds :type Float%20%28single-precision%29))
  (|CallParentFunction DeltaSeconds) ; This node is disabled and will not be called.\nDrag off pins to build functionality.
)

(fn ConstructionScript
  (|CallParentFunction))

(fn OutlineActor
  (params (Active :type Boolean))
  (|CallParentFunction Active))

(fn OnClick
  (|CallParentFunction))