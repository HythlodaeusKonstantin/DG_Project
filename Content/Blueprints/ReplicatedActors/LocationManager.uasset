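; LocationManager is a player-owned actor that moves its player character between the world map, procedural hex islands and battle arenas.
; Islands spawn as ProceduralHexagonalNetwork actors and arenas load as uniquely named level instances at fixed slot offsets, both registered in GameInstance maps.
; Arena entry polls on a timer until the arena network registers.
; Camera and UI switches run only for the GameInstance's player character, with server and multicast events updating player lists.
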(event EventBeginPlay
  (|Инициализация))

(fn ConstructionScript)

(fn SwitchonSlotIsland
  (params (Selection :type Integer))
  (switch int Selection
    (:0
      (LocalVariables|SetLocationToLoadIslandTemp "20000.000000, 0, 0"))
    (:1
      (LocalVariables|SetLocationToLoadIslandTemp "-20000.000000, 0, 0"))
    (:2
      (LocalVariables|SetLocationToLoadIslandTemp "0.000000,20000.000000,0.000000"))
    (:3
      (LocalVariables|SetLocationToLoadIslandTemp "0,-20000.000000, 0")))
  (return (LocalVariables|GetLocationToLoadIslandTemp)))

(fn SwitchonSlotArena
  (params (ArenaSlotIndex :type Integer))
  (switch int ArenaSlotIndex
    (:0
      (LocalVariables|SetLocationToLoadIslandTemp "40000.000000, 0, 0"))
    (:1
      (LocalVariables|SetLocationToLoadIslandTemp "-40000.000000, 0, 0"))
    (:2
      (LocalVariables|SetLocationToLoadIslandTemp "0.000000,40000.000000,0.000000"))
    (:3
      (LocalVariables|SetLocationToLoadIslandTemp "0,-40000.000000, 0")))
  (return (LocalVariables|GetLocationToLoadIslandTemp)))

(fn CreateUniqueLevelName
  (params (levelName :type String) (ArenaKey :type Arena%20Key%20Structure))
  (return (Utilities|String|Append (Utilities|String|ToString(Integer) (.islandindex ArenaKey)) (Utilities|String|ToString(Integer) (.ordinarindex ArenaKey)) levelName)))

(event Custom|SetLocationManagetToPlayerCharacter
  (bind _returnvalue (Components|GetOwner))
  (Utilities|IsValid _returnvalue
    (:Is%20Valid
      (bind _asplayer_character_dg (Utilities|Casting|CastToPlayerCharacter_DG _returnvalue))
      (bind _output_get (Variables|General|SetConnected%20Player%20Character%20DG _asplayer_character_dg))
      (Variables|/Game/Blueprints/PlayerCharacter/PlayerCharacter_DG.PlayerCharacter_DG_C|SetLocationManager _output_get self)
      (bind _asgame_inst_dg (Utilities|Casting|CastToGameInst_DG (Game|GetGameInstance)))
      (Variables|General|SetGame%20Inst%20DG _asgame_inst_dg))
    (:Is%20Not%20Valid
      (Utilities|Time|SetTimerbyFunctionName 0 "SetLocationManagetToPlayerCharacter" 0.5))))

(event Custom|EnterIsland
  (params (Index%20Of%20This%20Island%20in%20Array :type Integer%20%28by%20ref%29))
  (bind _connected_player_character_dg (Variables|General|GetConnected%20Player%20Character%20DG))
  (bind _connected_player_character_dg_2 (Variables|General|GetConnected%20Player%20Character%20DG))
  (bind _game_inst_dg (Variables|General|GetGame%20Inst%20DG))
  (bind _islandgenerationnetworks (Variables|/Game/Blueprints/GameSettings/GameInst_DG.GameInst_DG_C|GetIslandGenerationNetworks _game_inst_dg))
  (bind _value (Utilities|Map|Find _islandgenerationnetworks Index%20Of%20This%20Island%20in%20Array))
  ;[0 1 0] Вход на остров
  (Variables|Islands|SetCurrentIslandNetwork _value)
  (Variables|/Game/Blueprints/PlayerCharacter/PlayerCharacter_DG.PlayerCharacter_DG_C|SetLastWorldLocationHex _connected_player_character_dg_2 (Variables|/Game/Blueprints/NPC/BaseCharacter_DG.BaseCharacter_DG_C|GetcurrentCharacterLocation _connected_player_character_dg_2))
  (Default|TransfertoIsland _value _connected_player_character_dg)
  (Variables|/Game/Blueprints/NPC/BaseCharacter_DG.BaseCharacter_DG_C|SetHexagon%20Cells%20ALL%20-%20FindPath _connected_player_character_dg (Variables|/Game/Blueprints/ProceduralGeneration/ProceduralHexagonalNetwork.ProceduralHexagonalNetwork_C|GetHexagonCells-ALL (Variables|Islands|GetCurrentIslandNetwork)))
  (Variables|/Game/Blueprints/PlayerCharacter/PlayerCharacter_DG.PlayerCharacter_DG_C|SetCurrentWorld _connected_player_character_dg "NewEnumerator1")
  (if (== (Variables|General|GetConnected%20Player%20Character%20DG) (Variables|/Game/Blueprints/GameSettings/GameInst_DG.GameInst_DG_C|GetPlayer%20Character%20DG (Variables|General|GetGame%20Inst%20DG)))
    (|Активациякамеры_Входнаостров)
    (CallFunction|AddPlayerInfotoIslandNetwork-Server Index%20Of%20This%20Island%20in%20Array)))

(event Custom|AddPlayerInfoToIslandNetwork%20-%20Server
  (params (Key :type Integer%20%28by%20ref%29))
  ;[1 0 0] Добавляем игрока в массив игроков в нетворке острова - Сервер
  (Utilities|Array|Add (Variables|/Game/Blueprints/ProceduralGeneration/ProceduralHexagonalNetwork.ProceduralHexagonalNetwork_C|GetPlayersOnIsland (.Value (Utilities|Map|Find (Variables|/Game/Blueprints/GameSettings/GameInst_DG.GameInst_DG_C|GetIslandGenerationNetworks (Variables|General|GetGame%20Inst%20DG)) Key))) (Variables|/Game/Blueprints/PlayerCharacter/PlayerCharacter_DG.PlayerCharacter_DG_C|GetPlayerInfo (Variables|General|GetConnected%20Player%20Character%20DG))))

(event Custom|Enter%20Island%20-%20Location%20Manager
  (params (Index%20Of%20This%20Island%20in%20Array :type Integer) (IslandSlotIndex :type Integer) (IslandExist :type Boolean))
  ;[0 1 0] Вход на остров
  (if IslandExist
    (CallFunction|EnterIsland Index%20Of%20This%20Island%20in%20Array)
    (else
      (CallFunction|CreateIsland IslandSlotIndex Index%20Of%20This%20Island%20in%20Array)
      (CallFunction|EnterIsland Index%20Of%20This%20Island%20in%20Array))))

(event Custom|Exit%20Island
  (bind _connected_player_character_dg (Variables|General|GetConnected%20Player%20Character%20DG))
  ;[0 1 0] Выход из острова
  (Variables|/Game/Blueprints/NPC/BaseCharacter_DG.BaseCharacter_DG_C|SetHexagon%20Cells%20ALL%20-%20FindPath _connected_player_character_dg (Variables|/Game/Blueprints/ProceduralGeneration/ProceduralWorldGeneration.ProceduralWorldGeneration_C|GetHexagonCells-ALL (Variables|/Game/Blueprints/GameSettings/GameInst_DG.GameInst_DG_C|GetWorldGenerationNetwork (Variables|General|GetGame%20Inst%20DG))))
  (Variables|/Game/Blueprints/PlayerCharacter/PlayerCharacter_DG.PlayerCharacter_DG_C|SetCurrentWorld _connected_player_character_dg "NewEnumerator0")
  (if (== (Variables|General|GetConnected%20Player%20Character%20DG) (Variables|/Game/Blueprints/GameSettings/GameInst_DG.GameInst_DG_C|GetPlayer%20Character%20DG (Variables|General|GetGame%20Inst%20DG)))
    ;;[0 1 0] Активация камеры
    (|Активациякамеры_Выходсострова)))

(event Custom|CreateIsland
  (params (IslandSlotIndex :type Integer) (IndexOfThisIslandInArray :type Integer%20%28by%20ref%29))
  ;[0 1 0] Вход на остров
  (bind _locationtoloadisland (CallFunction|SwitchonSlotIsland IslandSlotIndex))
  (bind _returnvalue (Game|SpawnActorfromClass "/Game/Blueprints/ProceduralGeneration/ProceduralHexagonalNetwork.ProceduralHexagonalNetwork_C" (Math|Transform|MakeTransform _locationtoloadisland) "Undefined" 0 0))
  (Utilities|Map|Add (Variables|/Game/Blueprints/GameSettings/GameInst_DG.GameInst_DG_C|GetIslandGenerationNetworks (Variables|General|GetGame%20Inst%20DG)) IndexOfThisIslandInArray _returnvalue)
  (Default|LoadIsland _returnvalue IndexOfThisIslandInArray))

(event Custom|Destroy%20Island
  (params (Key :type Integer%20%28by%20ref%29))
  ;[0 1 0] Уничтожение острова
  (Variables|Islands|SetCurrentIslandNetwork (.Value (Utilities|Map|Find (Variables|/Game/Blueprints/GameSettings/GameInst_DG.GameInst_DG_C|GetIslandGenerationNetworks (Variables|General|GetGame%20Inst%20DG)) Key)))
  (Utilities|Map|Remove (Variables|/Game/Blueprints/GameSettings/GameInst_DG.GameInst_DG_C|GetIslandGenerationNetworks (Variables|General|GetGame%20Inst%20DG)) Key)
  (for _array_element (Variables|/Game/Blueprints/ProceduralGeneration/ProceduralHexagonalNetwork.ProceduralHexagonalNetwork_C|GetHexagonCells-ALL (Variables|Islands|GetCurrentIslandNetwork))
    (Actor|DestroyActor _array_element))
  (Actor|DestroyActor (Variables|Islands|GetCurrentIslandNetwork)))

(event Custom|EnterBattleArena%20LocationManager
  (params (ArenaSlotIndex :type Integer) (IslandIndex :type Integer) (OrdinarIndex :type Integer) (ArenaExist :type Boolean))
  ;[1 1 1] Выбор создавать арену или только заходить
  (if (and ArenaExist (.ReturnValue (Utilities|Map|Find (Variables|/Game/Blueprints/GameSettings/GameInst_DG.GameInst_DG_C|GetArenaLevels (Variables|General|GetGame%20Inst%20DG)) (Utilities|Struct|MakeArenaKey IslandIndex OrdinarIndex))))
    (CallFunction|EnterArena-LocationManage IslandIndex OrdinarIndex)
    (else
      (CallFunction|CreateArena-LocationManage ArenaSlotIndex IslandIndex OrdinarIndex)
      (CallFunction|EnterArena-LocationManage IslandIndex OrdinarIndex))))

(event Custom|RemovePlayerFromAssignToBattle%20-%20Multicast
  (params (IslandIndex :type Integer%20%28by%20ref%29) (OrdinarIndex :type Integer%20%28by%20ref%29))
  ;[0 0 1] Удаление игрока из списка готовых к бою - в PreBattle виджете - Мультикаст
  (Utilities|Array|RemoveItem (Variables|/Game/Blueprints/ProceduralGeneration/HexagonCellWorld.HexagonCellWorld_C|GetPlayersAssignToBattle (.Value (Utilities|Map|Find (Variables|/Game/Blueprints/ProceduralGeneration/ProceduralHexagonalNetwork.ProceduralHexagonalNetwork_C|GetHexAllMapInt (.Value (Utilities|Map|Find (Variables|/Game/Blueprints/GameSettings/GameInst_DG.GameInst_DG_C|GetIslandGenerationNetworks (Variables|General|GetGame%20Inst%20DG)) IslandIndex))) OrdinarIndex))) (.PlayerName (Utilities|Struct|BreakPlayersNetInfo (Variables|/Game/Blueprints/PlayerCharacter/PlayerCharacter_DG.PlayerCharacter_DG_C|GetPlayerInfo (Variables|General|GetConnected%20Player%20Character%20DG))))))

(event Custom|Create%20Arena%20-%20LocationManage
  (params (ArenaSlotIndex :type Integer) (IslandIndex :type Integer) (OrdinarIndex :type Integer))
  (bind _arenakey (Utilities|Struct|MakeArenaKey IslandIndex OrdinarIndex))
  (bind _game_inst_dg (Variables|General|GetGame%20Inst%20DG))
  (bind _game_inst_dg_2 (Variables|General|GetGame%20Inst%20DG))
  (bind _islandgenerationnetworks (Variables|/Game/Blueprints/GameSettings/GameInst_DG.GameInst_DG_C|GetIslandGenerationNetworks _game_inst_dg_2))
  (bind _arenalevels (Variables|/Game/Blueprints/GameSettings/GameInst_DG.GameInst_DG_C|GetArenaLevels _game_inst_dg))
  (bind _value (Utilities|Map|Find _islandgenerationnetworks IslandIndex))
  (bind (_value_2 _returnvalue) (Utilities|Map|Find _arenalevels _arenakey))
  (bind _hexallmapint (Variables|/Game/Blueprints/ProceduralGeneration/ProceduralHexagonalNetwork.ProceduralHexagonalNetwork_C|GetHexAllMapInt _value))
  (bind _value_3 (Utilities|Map|Find _hexallmapint OrdinarIndex))
  (bind _enemycamp (Variables|/Game/Blueprints/ProceduralGeneration/HexagonCellWorld.HexagonCellWorld_C|GetEnemyCamp _value_3))
  ;[1 1 1] Создание арены - если до этого она уже была создана, просто загружаем арену
  (Variables|Arena|SetArenaCreator true)
  (Variables|Arena|SetArenaKeys _arenakey)
  (if _returnvalue
    (Variables|/Script/Engine.LevelStreaming|SetbShouldBeLoaded _value_2 true)
    (Variables|Arena|SetcurrentStreamingLevel _value_2)
    (else
      (bind _locationtoloadisland (CallFunction|SwitchonSlotArena ArenaSlotIndex))
      (bind _uniquelevelname (CallFunction|CreateUniqueLevelName (.levelname _enemycamp) _arenakey))
      (bind _returnvalue_2 (Class|LevelStreamingDynamic|LoadLevelInstance (.levelname _enemycamp) _locationtoloadisland "0, 0, 0" _uniquelevelname))
      (bind _output_get (Variables|Arena|SetcurrentStreamingLevel _returnvalue_2))
      (Utilities|Map|Add (Variables|/Game/Blueprints/GameSettings/GameInst_DG.GameInst_DG_C|GetArenaLevels (Variables|General|GetGame%20Inst%20DG)) (Utilities|Struct|MakeArenaKey IslandIndex OrdinarIndex) _output_get))))

(event Custom|Enter%20Arena%20-%20LocationManage
  (params (IslandIndex :type Integer) (OrdinarIndex :type Integer))
  (bind _arenakey (Utilities|Struct|MakeArenaKey IslandIndex OrdinarIndex))
  (bind _game_inst_dg (Variables|General|GetGame%20Inst%20DG))
  (bind _connected_player_character_dg (Variables|General|GetConnected%20Player%20Character%20DG))
  (bind _arenanetworks (Variables|/Game/Blueprints/GameSettings/GameInst_DG.GameInst_DG_C|GetArenaNetworks _game_inst_dg))
  (bind (_value _returnvalue) (Utilities|Map|Find _arenanetworks _arenakey))
  ;[1 1 1] Вход на арену
  (if _returnvalue
    (|Перемещениеигроканаарену _value)
    (Variables|Default|SetCurrentArenaNetwork _value)
    (Variables|/Game/Blueprints/PlayerCharacter/PlayerCharacter_DG.PlayerCharacter_DG_C|SetCurrentArenaHex _connected_player_character_dg OrdinarIndex)
    (Variables|/Game/Blueprints/PlayerCharacter/PlayerCharacter_DG.PlayerCharacter_DG_C|SetCurrentWorld _connected_player_character_dg "NewEnumerator2")
    (if (== (Variables|General|GetConnected%20Player%20Character%20DG) (Variables|/Game/Blueprints/GameSettings/GameInst_DG.GameInst_DG_C|GetPlayer%20Character%20DG (Variables|General|GetGame%20Inst%20DG)))
      (Default|AddPlayerInfotoArenaNetwork-Client (Variables|General|GetConnected%20Player%20Character%20DG) IslandIndex OrdinarIndex)
      (CallFunction|SwitchUIArena)
      (CallFunction|RemovePlayerfromAssigntoBattle-Server IslandIndex OrdinarIndex))
    (else
      (Utilities|Time|SetTimerbyFunctionName 0 "Waiting for filling Arena Networks Event" 0.5))))

(event Custom|Exit%20Arena
  (bind _connected_player_character_dg (Variables|General|GetConnected%20Player%20Character%20DG))
  ;[1 1 1] Выход игрока из арены - смена UI
  (Variables|/Game/Blueprints/PlayerCharacter/PlayerCharacter_DG.PlayerCharacter_DG_C|SetCurrentArenaHex _connected_player_character_dg 9999)
  (Variables|/Game/Blueprints/PlayerCharacter/PlayerCharacter_DG.PlayerCharacter_DG_C|SetCurrentWorld _connected_player_character_dg "NewEnumerator1")
  (if (== _connected_player_character_dg (Variables|/Game/Blueprints/GameSettings/GameInst_DG.GameInst_DG_C|GetPlayer%20Character%20DG (Variables|General|GetGame%20Inst%20DG)))
    ;;[1 1 1] Смена камеры у вышедшего с арены игрока
    (CallFunction|SwitchUIWorldMap)))

(event Custom|Destroy%20Arena
  (params (IslandIndex :type Integer) (OrdinarIndex :type Integer))
  (bind _arenakey (Utilities|Struct|MakeArenaKey IslandIndex OrdinarIndex))
  (bind _game_inst_dg (Variables|General|GetGame%20Inst%20DG))
  ;[1 1 1] Уничтожение (выгрузка из памяти) арены
  (Utilities|Map|Remove (Variables|/Game/Blueprints/GameSettings/GameInst_DG.GameInst_DG_C|GetArenaNetworks _game_inst_dg) _arenakey)
  (Variables|/Script/Engine.LevelStreaming|SetbShouldBeLoaded (.Value (Utilities|Map|Find (Variables|/Game/Blueprints/GameSettings/GameInst_DG.GameInst_DG_C|GetArenaLevels _game_inst_dg) _arenakey)) false))

(event Custom|RemovePlayerFromAssignToBattle%20-%20Server
  (params (IslandIndex :type Integer%20%28by%20ref%29) (OrdinarIndex :type Integer%20%28by%20ref%29))
  ;[1 0 0] Удаление игрока из списка готовых к бою - в PreBattle виджете - Сервер
  (CallFunction|RemovePlayerfromAssigntoBattle-Multicast IslandIndex OrdinarIndex))

(event Custom|Waiting%20for%20filling%20Arena%20Networks%20Event
  (bind _connected_player_character_dg (Variables|General|GetConnected%20Player%20Character%20DG))
  ;[1 1 1] Вход на арену
  (if (.ReturnValue (Utilities|Map|Find (Variables|/Game/Blueprints/GameSettings/GameInst_DG.GameInst_DG_C|GetArenaNetworks (Variables|General|GetGame%20Inst%20DG)) (Utilities|Struct|MakeArenaKey (stale Custom|Enter%20Arena%20-%20LocationManage IslandIndex) (stale Custom|Enter%20Arena%20-%20LocationManage OrdinarIndex))))
    (|Перемещениеигроканаарену (.Value (Utilities|Map|Find (Variables|/Game/Blueprints/GameSettings/GameInst_DG.GameInst_DG_C|GetArenaNetworks (Variables|General|GetGame%20Inst%20DG)) (Utilities|Struct|MakeArenaKey (stale Custom|Enter%20Arena%20-%20LocationManage IslandIndex) (stale Custom|Enter%20Arena%20-%20LocationManage OrdinarIndex)))))
    (Variables|Default|SetCurrentArenaNetwork (.Value (Utilities|Map|Find (Variables|/Game/Blueprints/GameSettings/GameInst_DG.GameInst_DG_C|GetArenaNetworks (Variables|General|GetGame%20Inst%20DG)) (Utilities|Struct|MakeArenaKey (stale Custom|Enter%20Arena%20-%20LocationManage IslandIndex) (stale Custom|Enter%20Arena%20-%20LocationManage OrdinarIndex)))))
    (Variables|/Game/Blueprints/PlayerCharacter/PlayerCharacter_DG.PlayerCharacter_DG_C|SetCurrentArenaHex _connected_player_character_dg (stale Custom|Enter%20Arena%20-%20LocationManage OrdinarIndex))
    (Variables|/Game/Blueprints/PlayerCharacter/PlayerCharacter_DG.PlayerCharacter_DG_C|SetCurrentWorld _connected_player_character_dg "NewEnumerator2")
    (if (== (Variables|General|GetConnected%20Player%20Character%20DG) (Variables|/Game/Blueprints/GameSettings/GameInst_DG.GameInst_DG_C|GetPlayer%20Character%20DG (Variables|General|GetGame%20Inst%20DG)))
      (Default|AddPlayerInfotoArenaNetwork-Client (Variables|General|GetConnected%20Player%20Character%20DG) (stale Custom|Enter%20Arena%20-%20LocationManage IslandIndex) (stale Custom|Enter%20Arena%20-%20LocationManage OrdinarIndex))
      (CallFunction|SwitchUIArena)
      (CallFunction|RemovePlayerfromAssigntoBattle-Server (stale Custom|Enter%20Arena%20-%20LocationManage IslandIndex) (stale Custom|Enter%20Arena%20-%20LocationManage OrdinarIndex)))
    (else
      (Utilities|Time|SetTimerbyFunctionName 0 "Waiting for filling Arena Networks Event" 0.5))))