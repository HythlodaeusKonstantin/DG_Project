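; LevelStreamer actor that streams battle arena levels in and out at runtime and registers itself on the DG player controller at BeginPlay.
; EnterBattleArena loads the named arena as a level instance at a given location and keeps the streaming level reference so ExitBattleArena can unload it.
; Instance names are built from the player's current island and location indices plus the arena name, keeping them distinct per location.
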(event Custom|EnterBattleArena
  (params (ArenaName :type String) (ArenaLocation :type Vector))
  (bind _uniquelevelname (CallFunction|CreateUniqueLevelName ArenaName))
  (bind _returnvalue (Class|LevelStreamingDynamic|LoadLevelInstance ArenaName ArenaLocation "0, 0, 0" _uniquelevelname))
  (Variables|Default|SetcurrentStreamingLevel _returnvalue))

(event Custom|ExitBattleArena
  (Variables|/Script/Engine.LevelStreaming|SetbShouldBeLoaded (Variables|Default|GetcurrentStreamingLevel) false))

(event EventBeginPlay
  (bind _asplayer_character_dg (Utilities|Casting|CastToPlayerCharacter_DG (Game|Player|GetPlayerPawn 0)))
  (Variables|Default|SetPlayer%20Character%20DG _asplayer_character_dg)
  (bind _asplayer_controller_dg (Utilities|Casting|CastToPlayerController_DG (Game|GetPlayerController 0)))
  (bind _output_get (Variables|Default|SetPlayer%20Controller%20DG _asplayer_controller_dg))
  (Variables|/Game/Blueprints/GameSettings/PlayerController_DG.PlayerController_DG_C|SetLevelStreamer _output_get self))

(fn ConstructionScript)

(fn CreateUniqueLevelName
  (params (levelName :type String))
  (bind _player_character_dg (Variables|Default|GetPlayer%20Character%20DG))
  (bind _currentplayerlocation (Variables|/Game/Blueprints/PlayerCharacter/PlayerCharacter_DG.PlayerCharacter_DG_C|GetcurrentPlayerLocation _player_character_dg))
  (return (Utilities|String|Append (Utilities|String|ToString(Integer) (Variables|/Game/Blueprints/ProceduralGeneration/HexagonCellWorld.HexagonCellWorld_C|GetIndexOfThisIslandInArray _currentplayerlocation)) (Utilities|String|ToString(Vector) (Variables|/Game/Blueprints/ProceduralGeneration/HexagonCellWorld.HexagonCellWorld_C|GetIndex _currentplayerlocation)) levelName)))