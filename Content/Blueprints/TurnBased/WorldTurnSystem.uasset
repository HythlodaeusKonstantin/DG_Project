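; World turn manager for a multiplayer turn-based game, driving shared turns, a day counter and the time of day.
; It registers with the game instance, then records connecting players' info with Steam or random nicknames and a ready flag.
; When all flags are set, the server refills action points and advances an eight-turn day cycle.
; A multicast event updates morning-to-night phases and rotates the sun through per-turn timelines; combat entry is an empty stub.
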(event Custom|NewPlayerConnection
  (params (PlayerController :type Player%20Controller%20DG%20Object%20Reference))
  (bind _numnetplayers (Class|AdvancedSessionsLibrary|GetNumberOfNetworkPlayers))
  (bind _randomplayernickname (Variables|Default|GetRandomPlayerNickname))
  ;[1 0 0] Устанавливаем базовую информацию о игроках на сервере
  (if (!= _numnetplayers (Variables|Default|GetNum%20Net%20Players))
    (Variables|Default|SetNum%20Net%20Players _numnetplayers)
    (if (Class|AdvancedSessionsLibrary|HasOnlineSubsystem "STEAM")
      (Variables|Default|SetPlayer%20Nickname (Class|AdvancedIdentityLibrary|GetPlayerNickname (Class|AdvancedSessionsLibrary|GetUniqueNetID PlayerController)))
      (else
        (bind _output_get (Variables|Default|SetPlayer%20Nickname (.OutItem (Utilities|Array|Random _randomplayernickname))))
        (Utilities|Array|RemoveItem _randomplayernickname _output_get)))
    (bind _asplayer_character_dg (Utilities|Casting|CastToPlayerCharacter_DG (Pawn|GetControlledPawn PlayerController)))
    (Variables|/Game/Blueprints/PlayerCharacter/PlayerCharacter_DG.PlayerCharacter_DG_C|SetPlayerInfo _asplayer_character_dg (Utilities|Struct|MakePlayersNetInfo (Variables|Default|GetPlayer%20Nickname) PlayerController _asplayer_character_dg (- (Variables|Default|GetNum%20Net%20Players) 1)))
    (Utilities|Array|AddUnique (Variables|Default|GetPlayersInfo) (Utilities|Struct|MakePlayersNetInfo (Variables|Default|GetPlayer%20Nickname) PlayerController _asplayer_character_dg (- (Variables|Default|GetNum%20Net%20Players) 1)))
    (Utilities|Array|Add (Variables|Default|GetPlayersRadyForNextTurn) false)))

(event Custom|EndTurn%20-%20Renew%20-%20Server
  (bind _playersradyfornextturn (Variables|Default|GetPlayersRadyForNextTurn))
  ;[1 0 0] Проверка у всех ли игроков закончился ход
  (Variables|Default|SetEveryoneReadyForNextTurn true)
  (bind _array_element (Utilities|Array|ForEachLoopwithBreak (Variables|Default|GetPlayersRadyForNextTurn) :!label _label)
    (:LoopBody
      (if (not _array_element)
        (Variables|Default|SetEveryoneReadyForNextTurn false)
        (goto _label Break)))
    (:Completed
      (if (Variables|Default|GetEveryoneReadyForNextTurn)
        (Utilities|FlowControl|Sequence
          (:then_0
            ;[1 0 0] Обновляем очки действия, если ход закончен
            (for _array_element_2 (Variables|Default|GetPlayersInfo)
              (Variables|/Game/Blueprints/TurnBased/WorldTurnComponent.WorldTurnComponent_C|SetActionPoints (Variables|/Game/Blueprints/NPC/BaseCharacter_DG.BaseCharacter_DG_C|GetWorldTurnComponent (.PlayerCharacter (Utilities|Struct|BreakPlayersNetInfo _array_element_2))) 10)
              (for (_ _array_index) _playersradyfornextturn
                (Utilities|Array|SetArrayElem _playersradyfornextturn _array_index false))))
          (:then_1
            ;[1 0 0] Счетчик ходов
            (if (== (Variables|Default|GetTurnCounter) 8)
              (Variables|Default|SetTurnCounter 0)
              ;;[1 0 0] Счетчик дней
              (Math|Integer|IncrementInt (Variables|Default|GetDaysCounter)
                (:%20%20
                  _)))
            (Math|Integer|IncrementInt (Variables|Default|GetTurnCounter)
              (:%20%20
                (CallFunction|SunChanging-Multicast)))))))))

(event Custom|SunChanging%20-%20Multicast
  ;[1 0 0] Счетчик ходов
  (switch int (Variables|Default|GetTurnCounter)
    (:1
      (Variables|Default|SetTimeOfTheDay "NewEnumerator0")
      (Development|PrintString "Наступило утро")
      (bind _track (Timeline|Timeline_4 PlayFromStart)
        (:Update
          (Transformation|SetActorRotation (Variables|/Game/Blueprints/GameSettings/GameInst_DG.GameInst_DG_C|GetSun (Variables|Default|GetGame%20Inst%20DG)) (Math|Rotator|MakeRotator 0.0 _track 0.0)))))
    (:2
      (Variables|Default|SetTimeOfTheDay "NewEnumerator1")
      (Development|PrintString "Наступил день")
      (bind _track_2 (Timeline|Morning PlayFromStart)
        (:Update
          (Transformation|SetActorRotation (Variables|/Game/Blueprints/GameSettings/GameInst_DG.GameInst_DG_C|GetSun (Variables|Default|GetGame%20Inst%20DG)) (Math|Rotator|MakeRotator 0.0 _track_2 0.0)))))
    (:3
      (bind _track_3 (Timeline|Timeline_0 PlayFromStart)
        (:Update
          (Transformation|SetActorRotation (Variables|/Game/Blueprints/GameSettings/GameInst_DG.GameInst_DG_C|GetSun (Variables|Default|GetGame%20Inst%20DG)) (Math|Rotator|MakeRotator 0.0 _track_3 0.0)))))
    (:4
      (bind _track_4 (Timeline|Timeline_1 PlayFromStart)
        (:Update
          (Transformation|SetActorRotation (Variables|/Game/Blueprints/GameSettings/GameInst_DG.GameInst_DG_C|GetSun (Variables|Default|GetGame%20Inst%20DG)) (Math|Rotator|MakeRotator 0.0 _track_4 0.0)))))
    (:5
      (Variables|Default|SetTimeOfTheDay "NewEnumerator2")
      (Development|PrintString "Наступил вечер")
      (bind _track_5 (Timeline|Timeline_2 PlayFromStart)
        (:Update
          (Transformation|SetActorRotation (Variables|/Game/Blueprints/GameSettings/GameInst_DG.GameInst_DG_C|GetSun (Variables|Default|GetGame%20Inst%20DG)) (Math|Rotator|MakeRotator 0.0 _track_5 0.0)))))
    (:6
      (Variables|Default|SetTimeOfTheDay "NewEnumerator3")
      (Development|PrintString "Наступила ночь")
      (bind _track_6 (Timeline|Timeline_3 PlayFromStart)
        (:Update
          (Transformation|SetActorRotation (Variables|/Game/Blueprints/GameSettings/GameInst_DG.GameInst_DG_C|GetSun (Variables|Default|GetGame%20Inst%20DG)) (Math|Rotator|MakeRotator 0.0 _track_6 0.0)))
        (:Finished
          (Transformation|SetActorRotation (Variables|/Game/Blueprints/GameSettings/GameInst_DG.GameInst_DG_C|GetSun (Variables|Default|GetGame%20Inst%20DG)) (Math|Rotator|MakeRotator 0.0 9e+01 0.0)))))))

(event Custom|EnterCombat)

(event EventBeginPlay
  (Utilities|FlowControl|Sequence
    (:then_0
      ;[0 0 0] Инициализация
      (bind _asgame_inst_dg (Utilities|Casting|CastToGameInst_DG (Game|GetGameInstance)))
      (bind _output_get (Variables|Default|SetGame%20Inst%20DG _asgame_inst_dg))
      (Variables|/Game/Blueprints/GameSettings/GameInst_DG.GameInst_DG_C|SetWorldTurnSystem _output_get self)
      (bind _asplayer_controller_dg (Utilities|Casting|CastToPlayerController_DG (Game|GetPlayerController 0)))
      (Variables|Default|SetPlayer%20Controller%20DG _asplayer_controller_dg))
    (:then_1
      (Default|WorldTurnSystemInitialization (Variables|Default|GetPlayer%20Controller%20DG)))))

(fn ConstructionScript)