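; Network manager component on PlayerCharacter_DG that registers joining players and syncs the saved world from server to clients.
; On begin play, the server records each player's index and Steam or random nickname in ServerOnlyNetworkManager.
; Loading chains server-client calls, sending save arrays element by element and slot maps as four flattened pairs, then rebuilds world, islands and arenas.
; Finally it sends changed hexes' battle assignments as packed integers and re-enables input.
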(event EventBeginPlay
  (|Инициализация)
  (CallFunction|WorldTurnSystemInitialization))

(fn ConstructionScript)

(fn TransferIslandSlotMaptoValues
  (bind _gameinstance (Variables|Default|GetGameInstance))
  (bind _island_index_slots (Variables|/Game/Blueprints/GameSettings/GameInst_DG.GameInst_DG_C|GetIsland%20Index%20Slots _gameinstance))
  (bind _keys (Utilities|Map|Keys _island_index_slots))
  (for (_array_element _array_index) _keys
    (switch int _array_index
      (:0
        (LocalVariables|SetKey1 _array_element)
        (LocalVariables|SetValue1 (.Value (Utilities|Map|Find _island_index_slots _array_element))))
      (:1
        (LocalVariables|SetKey2 _array_element)
        (LocalVariables|SetValue2 (.Value (Utilities|Map|Find _island_index_slots _array_element))))
      (:2
        (LocalVariables|SetKey3 _array_element)
        (LocalVariables|SetValue3 (.Value (Utilities|Map|Find _island_index_slots _array_element))))
      (:3
        (LocalVariables|SetKey4 _array_element)
        (LocalVariables|SetValue4 (.Value (Utilities|Map|Find _island_index_slots _array_element))))))
  (return (LocalVariables|GetKey1) (LocalVariables|GetValue1) (LocalVariables|GetKey2) (LocalVariables|GetValue2) (LocalVariables|GetKey3) (LocalVariables|GetValue3) (LocalVariables|GetKey4) (LocalVariables|GetValue4)))

(fn TransferArenaSlotMaptoValues
  (bind _gameinstance (Variables|Default|GetGameInstance))
  (bind _arena_index_slots (Variables|/Game/Blueprints/GameSettings/GameInst_DG.GameInst_DG_C|GetArena%20Index%20Slots _gameinstance))
  (bind _keys (Utilities|Map|Keys _arena_index_slots))
  (for (_array_element _array_index) _keys
    (switch int _array_index
      (:0
        (LocalVariables|SetKey1 _array_element)
        (LocalVariables|SetValue1 (.Value (Utilities|Map|Find _arena_index_slots _array_element))))
      (:1
        (LocalVariables|SetKey2 _array_element)
        (LocalVariables|SetValue2 (.Value (Utilities|Map|Find _arena_index_slots _array_element))))
      (:2
        (LocalVariables|SetKey3 _array_element)
        (LocalVariables|SetValue3 (.Value (Utilities|Map|Find _arena_index_slots _array_element))))
      (:3
        (LocalVariables|SetKey4 _array_element)
        (LocalVariables|SetValue4 (.Value (Utilities|Map|Find _arena_index_slots _array_element))))))
  (return (LocalVariables|GetKey1) (LocalVariables|GetValue1) (LocalVariables|GetKey2) (LocalVariables|GetValue2) (LocalVariables|GetKey3) (LocalVariables|GetValue3) (LocalVariables|GetKey4) (LocalVariables|GetValue4)))

(fn FulfillPlayersIndexes
  (params (Target :type Hexagon%20Cell%20World%20Object%20Reference))
  (bind (_array_element _array_index) (Utilities|Array|ForEachLoopwithBreak (Variables|/Game/Blueprints/ProceduralGeneration/HexagonCellWorld.HexagonCellWorld_C|GetPlayersAssignToBattle Target))
    (:LoopBody
      (bind _array_element_2 (Utilities|Array|ForEachLoopwithBreak (Variables|/Game/Blueprints/ReplicatedActors/ServerOnlyNetworkManager.ServerOnlyNetworkManager_C|GetPlayersInfo (Variables|GeneralNetworkManager_C|GetServerOnlyNetworkManager (Variables|/Game/Blueprints/NPC/BaseCharacter_DG.BaseCharacter_DG_C|GetGeneralNetworkManager (Variables|/Game/Blueprints/GameSettings/GameInst_DG.GameInst_DG_C|GetPlayer%20Character%20DG (Variables|Default|GetGameInstance))))) :!label _label)
        (:LoopBody
          (if (Utilities|Enum|Equal(Enum) _array_element (.PlayerName (Utilities|Struct|BreakPlayersNetInfo _array_element_2)))
            (goto _label Break)))
        (:Completed
          (switch int _array_index
            (:0
              (bind _output_get (LocalVariables|Seta (.PlayerIndex (Utilities|Struct|BreakPlayersNetInfo _array_element_2)))))
            (:1
              (bind _output_get_2 (LocalVariables|Setb (.PlayerIndex (Utilities|Struct|BreakPlayersNetInfo _array_element_2)))))
            (:2
              (bind _output_get_3 (LocalVariables|Setc (.PlayerIndex (Utilities|Struct|BreakPlayersNetInfo _array_element_2)))))
            (:3
              (bind _output_get_4 (LocalVariables|Setd (.PlayerIndex (Utilities|Struct|BreakPlayersNetInfo _array_element_2)))))))))
    (:Completed
      (return _output_get _output_get_2 _output_get_3 _output_get_4))))

(fn FulfillPlayerReadytoBattleArray
  (params (a1 :type Byte) (b1 :type Byte) (b2 :type Byte) (a12 :type Integer))
  (bind (_a _b) (CallFunction|DecodeThreeBytetoTwoInt a1 b1 b2))
  (bind (_a_2 _b_2 _c _d) (CallFunction|DecodeOneInttoFourInt a12))
  (Utilities|FlowControl|Sequence
    (:then_0
      (if (!= _a_2 9)
        (LocalVariables|SetPlayerIndexTemp _a_2)
        (for _array_element (Variables|/Game/Blueprints/ReplicatedActors/ServerOnlyNetworkManager.ServerOnlyNetworkManager_C|GetPlayersInfo (Variables|GeneralNetworkManager_C|GetServerOnlyNetworkManager (Variables|/Game/Blueprints/NPC/BaseCharacter_DG.BaseCharacter_DG_C|GetGeneralNetworkManager (Variables|/Game/Blueprints/GameSettings/GameInst_DG.GameInst_DG_C|GetPlayer%20Character%20DG (Variables|Default|GetGameInstance))))) :!label _label
          (if (== (LocalVariables|GetPlayerIndexTemp) (.PlayerIndex (Utilities|Struct|BreakPlayersNetInfo _array_element)))
            (Utilities|Array|AddUnique (Variables|/Game/Blueprints/ProceduralGeneration/HexagonCellWorld.HexagonCellWorld_C|GetPlayersAssignToBattle (.Hexagon (CallFunction|FindHex (Variables|Default|GetGameInstance) _a _b))) (.PlayerName (Utilities|Struct|BreakPlayersNetInfo _array_element)))))))
    (:then_1
      (if (!= _b_2 9)
        (LocalVariables|SetPlayerIndexTemp _b_2)
        (goto _label)))
    (:then_2
      (if (!= _c 9)
        (LocalVariables|SetPlayerIndexTemp _c)
        (goto _label)))
    (:then_3
      (if (!= _d 9)
        (LocalVariables|SetPlayerIndexTemp _d)
        (goto _label)))))

(fn CounterforLoadingIsland
  (bind _gameinstance (Variables|Default|GetGameInstance))
  (bind _island_index_slots (Variables|/Game/Blueprints/GameSettings/GameInst_DG.GameInst_DG_C|GetIsland%20Index%20Slots _gameinstance))
  (bind _keys (Utilities|Map|Keys _island_index_slots))
  (if (not (== (Utilities|Array|Length _keys) (Variables|Default|GetCounterForLoadingIslands)))
    (return (Utilities|Array|Get(acopy) _keys (Variables|Default|GetCounterForLoadingIslands)) (.Value (Utilities|Map|Find _island_index_slots (Utilities|Array|Get(acopy) _keys (Variables|Default|GetCounterForLoadingIslands)))))))

(event Custom|NewPlayerConnection
  (params (PlayerController :type Player%20Controller%20DG%20Object%20Reference) (Player%20Nickname :type String))
  (bind _randomplayernickname (Variables|Default|GetRandomPlayerNickname))
  ;[1 1 1] Устанавливаем базовую информацию о игроках на сервере
  ;;[1 1 1] Инкрементируем текущее число игроков
  (Math|Integer|IncrementInt (Variables|Default|GetNum%20Net%20Players)
    (:%20%20
      ;;[1 1 1] Играем ли мы через стим?
      (if (Class|AdvancedSessionsLibrary|HasOnlineSubsystem "STEAM")
        (Variables|Default|SetPlayer%20Nickname Player%20Nickname)
        (else
          (bind _output_get (Variables|Default|SetPlayer%20Nickname (.OutItem (Utilities|Array|Random _randomplayernickname))))
          (Utilities|Array|RemoveItem _randomplayernickname _output_get)))
      (bind _asplayer_character_dg (Utilities|Casting|CastToPlayerCharacter_DG (Pawn|GetControlledPawn PlayerController)))
      (Variables|/Game/Blueprints/PlayerCharacter/PlayerCharacter_DG.PlayerCharacter_DG_C|SetPlayerInfo _asplayer_character_dg (Utilities|Struct|MakePlayersNetInfo (Variables|Default|GetPlayer%20Nickname) PlayerController _asplayer_character_dg (Variables|Default|GetNum%20Net%20Players)))
      (Utilities|Array|AddUnique (Variables|/Game/Blueprints/ReplicatedActors/ServerOnlyNetworkManager.ServerOnlyNetworkManager_C|GetPlayersInfo (Variables|Default|GetServerOnlyNetworkManager)) (Utilities|Struct|MakePlayersNetInfo (Variables|Default|GetPlayer%20Nickname) PlayerController _asplayer_character_dg (Variables|Default|GetNum%20Net%20Players)))
      (Utilities|Array|Add (Variables|Default|GetPlayersRadyForNextTurn) false))))

(event Custom|WorldTurnSystemInitialization
  (bind _gameinstance (Variables|Default|GetGameInstance))
  (bind _player_controller_dg (Variables|/Game/Blueprints/GameSettings/GameInst_DG.GameInst_DG_C|GetPlayer%20Controller%20DG _gameinstance))
  (bind _uniquenetid (Class|AdvancedSessionsLibrary|GetUniqueNetID _player_controller_dg))
  (if (== (Variables|Default|GetOwnerPlayerCharacter) (Variables|/Game/Blueprints/GameSettings/GameInst_DG.GameInst_DG_C|GetPlayer%20Character%20DG _gameinstance))
    ;[0 1 0] Инициализация WorldTurnSystem
    (Utilities|IsValidWaiting-ExternalBool (Class|AdvancedSessionsLibrary|IsValidUniqueNetID _uniquenetid)
      (:Is%20Valid
        (CallFunction|WorldTurnSystemInitialization-Server _player_controller_dg (Class|AdvancedIdentityLibrary|GetPlayerNickname _uniquenetid))))))

(event Custom|WorldTurnSystemInitialization%20-%20Server
  (params (PlayerController :type Player%20Controller%20DG%20Object%20Reference) (Player%20Nickname :type String))
  (bind _gameinstance (Variables|Default|GetGameInstance))
  ;[1 0 0] Инициализация WorldTurnSystem - Сервер
  (Utilities|IsValidWaiting (Variables|/Game/Blueprints/GameSettings/GameInst_DG.GameInst_DG_C|GetWorldTurnSystem _gameinstance)
    (:Is%20Valid
      (CallFunction|NewPlayerConnection (Variables|/Game/Blueprints/NPC/BaseCharacter_DG.BaseCharacter_DG_C|GetGeneralNetworkManager (Variables|/Game/Blueprints/GameSettings/GameInst_DG.GameInst_DG_C|GetPlayer%20Character%20DG _gameinstance)) PlayerController Player%20Nickname))))

(event Custom|CallServerToSetArenaSlotData
  ;[1 0 0] Передача данных заполненности слотов арены. Серверная часть
  (bind (_island_index_key1 _island_index_value1 _island_index_key2 _island_index_value2 _island_index_key3 _island_index_value3 _island_index_key4 _island_index_value4) (CallFunction|TransferArenaSlotMaptoValues))
  (CallFunction|SetArenaSlotData (.islandindex _island_index_key1) (.ordinarindex _island_index_key1) _island_index_value1 (.islandindex _island_index_key2) (.ordinarindex _island_index_key2) _island_index_value2 (.islandindex _island_index_key3) (.ordinarindex _island_index_key3) _island_index_value3 (.islandindex _island_index_key4) (.ordinarindex _island_index_key4) _island_index_value4))

(event Custom|SetArenaSlotData
  (params (IslandIndexIslandIndex1 :type Integer) (IslandIndexOrdinarIndex1 :type Integer) (IslandIndexValue1 :type Integer) (IslandIndexIslandIndex2 :type Integer) (IslandIndexOrdinarIndex2 :type Integer) (IslandIndexValue2 :type Integer) (IslandIndexIslandIndex3 :type Integer) (IslandIndexOrdinarIndex3 :type Integer) (IslandIndexValue3 :type Integer) (IslandIndexIslandIndex4 :type Integer) (IslandIndexOrdinarIndex4 :type Integer) (IslandIndexValue4 :type Integer))
  (bind _gameinstance (Variables|Default|GetGameInstance))
  (bind _arena_index_slots (Variables|/Game/Blueprints/GameSettings/GameInst_DG.GameInst_DG_C|GetArena%20Index%20Slots _gameinstance))
  (bind _arenaslot (Variables|/Game/Blueprints/GameSettings/GameInst_DG.GameInst_DG_C|GetArenaSlot _gameinstance))
  ;[0 0 1] Передача данных заполненности слотов арены. Мультикаст
  (if (== IslandIndexIslandIndex1 999)
    _
    (else
      (Utilities|Map|Add _arena_index_slots (Utilities|Struct|MakeArenaKey IslandIndexIslandIndex1 IslandIndexOrdinarIndex1) IslandIndexValue1)
      (Utilities|Array|SetArrayElem _arenaslot IslandIndexValue1 true)))
  (if (== IslandIndexIslandIndex2 999)
    _
    (else
      (Utilities|Map|Add _arena_index_slots (Utilities|Struct|MakeArenaKey IslandIndexIslandIndex2 IslandIndexOrdinarIndex2) IslandIndexValue2)
      (Utilities|Array|SetArrayElem _arenaslot IslandIndexValue2 true)))
  (if (== IslandIndexIslandIndex3 999)
    _
    (else
      (Utilities|Map|Add _arena_index_slots (Utilities|Struct|MakeArenaKey IslandIndexIslandIndex3 IslandIndexOrdinarIndex3) IslandIndexValue3)
      (Utilities|Array|SetArrayElem _arenaslot IslandIndexValue3 true)))
  (if (== IslandIndexIslandIndex4 999)
    _
    (else
      (Utilities|Map|Add _arena_index_slots (Utilities|Struct|MakeArenaKey IslandIndexIslandIndex4 IslandIndexOrdinarIndex4) IslandIndexValue4)
      (Utilities|Array|SetArrayElem _arenaslot IslandIndexValue4 true)))
  (Variables|/Game/Blueprints/GameSettings/GameInst_DG.GameInst_DG_C|SetArenasLoaded (Variables|Default|GetGameInstance) true)
  (CallFunction|LoadArenas))

(event Custom|CallServerToSetSaveData
  (bind (_indexofcurrentislandinarray _savename _worlddatasaved_ _worldgenerationnetworkdata) (|CurrentSaveData_2_3))
  ;[1 0 0] Передача общих данных сохранения. Серверная часть
  (CallFunction|SetSaveDatafromServer _indexofcurrentislandinarray _savename _worlddatasaved_ _worldgenerationnetworkdata))

(event Custom|SetSaveDataFromServer
  (params (IndexOfCurrentIslandInArray :type Integer) (SaveName :type String) (WorldDataSaved? :type Boolean) (WorldGenerationNetworkData :type World%20Generation%20Network%20Data%20Save%20Structure))
  (bind _gameinstance (Variables|Default|GetGameInstance))
  (bind _activesavegame_worldstorage (Variables|/Game/Blueprints/GameSettings/GameInst_DG.GameInst_DG_C|GetActiveSaveGame_WorldStorage _gameinstance))
  ;[0 0 1] Передача общих данных сохранения. Owning Client
  (Variables|/Game/Blueprints/GameSettings/WorldStorage.WorldStorage_C|SetIndexOfCurrentIslandInArray _activesavegame_worldstorage IndexOfCurrentIslandInArray)
  (Variables|/Game/Blueprints/GameSettings/WorldStorage.WorldStorage_C|SetSaveName _activesavegame_worldstorage SaveName)
  (Variables|/Game/Blueprints/GameSettings/WorldStorage.WorldStorage_C|SetWorldDataSaved? _activesavegame_worldstorage WorldDataSaved?)
  (bind _output_get (Variables|/Game/Blueprints/GameSettings/WorldStorage.WorldStorage_C|SetWorldGenerationNetworkData _activesavegame_worldstorage WorldGenerationNetworkData))
  (CallFunction|CallServertoSetWorldGenerationHexagonData)
  (Development|PrintString (Utilities|String|EnumtoString (Utilities|Struct|BreakWorldGenerationNetworkDataSave _output_get))))

(event Custom|CallServerToSetWorldGenerationHexagonData
  (params (IndexWorldGenerationHexagonData :type Byte))
  (bind _worldgenerationhexagondata (|CurrentSaveData_3_2))
  ;[1 0 0] Передача данных сохранения карты мира. Серверная часть
  (CallFunction|SetWorldGenerationHexagonData (Utilities|Array|Get(acopy) _worldgenerationhexagondata (Math|Conversions|ToInteger(Byte) IndexWorldGenerationHexagonData)) (Utilities|Array|Length _worldgenerationhexagondata)))

(event Custom|SetWorldGenerationHexagonData
  (params (NewItem :type World%20Generation%20Hexagon%20Data%20Save%20Structure%20%28by%20ref%29) (Lenght :type Integer))
  ;[0 0 1] Передача данных сохранения карты мира. Owning Client
  (bind _returnvalue (Utilities|Array|Add (Variables|/Game/Blueprints/GameSettings/WorldStorage.WorldStorage_C|GetWorldGenerationHexagonData (Variables|/Game/Blueprints/GameSettings/GameInst_DG.GameInst_DG_C|GetActiveSaveGame_WorldStorage (Variables|Default|GetGameInstance))) NewItem))
  (Variables|Default|SetWorldGenerationHexagonDataFill? (== _returnvalue (- Lenght 1)))
  (if (Variables|Default|GetWorldGenerationHexagonDataFill?)
    (CallFunction|CallServertoSetWorldClusterData)
    (else
      (CallFunction|CallServertoSetWorldGenerationHexagonData (Math|Conversions|ToByte(Integer) (+ _returnvalue 1))))))

(event Custom|CallServerToSetIslandSlotData
  ;[1 0 0] Передача данных заполненности слотов островов. Серверная часть
  (bind (_island_index_key1 _island_index_value1 _island_index_key2 _island_index_value2 _island_index_key3 _island_index_value3 _island_index_key4 _island_index_value4) (CallFunction|TransferIslandSlotMaptoValues))
  (CallFunction|SetIslandSlotData _island_index_key1 _island_index_value1 _island_index_key2 _island_index_value2 _island_index_key3 _island_index_value3 _island_index_key4 _island_index_value4))

(event Custom|SetWorldClusterData
  (params (NewItem :type Ocean%20Cluster%20Save%20Structure%20%28by%20ref%29) (Lenght :type Integer))
  ;[0 0 1] Пеоедача данных сохранения секторов. Owning Client
  (bind _returnvalue (Utilities|Array|Add (Variables|/Game/Blueprints/GameSettings/WorldStorage.WorldStorage_C|GetWorldClusterData (Variables|/Game/Blueprints/GameSettings/GameInst_DG.GameInst_DG_C|GetActiveSaveGame_WorldStorage (Variables|Default|GetGameInstance))) NewItem))
  (Variables|Default|SetClusterDataFill? (== _returnvalue (- Lenght 1)))
  (if (Variables|Default|GetClusterDataFill?)
    (CallFunction|CallServertoSetIslandSlotData)
    (else
      (CallFunction|CallServertoSetWorldClusterData (Math|Conversions|ToByte(Integer) (+ _returnvalue 1))))))

(event Custom|SetIslandSlotData
  (params (IslandIndexKey1 :type Integer) (IslandIndexSlot1 :type Integer) (IslandIndexKey2 :type Integer) (IslandIndexSlot2 :type Integer) (IslandIndexKey3 :type Integer) (IslandIndexSlot3 :type Integer) (IslandIndexKey4 :type Integer) (IslandIndexSlot4 :type Integer))
  (bind _gameinstance (Variables|Default|GetGameInstance))
  (bind _islandslot (Variables|/Game/Blueprints/GameSettings/GameInst_DG.GameInst_DG_C|GetIslandSlot _gameinstance))
  (bind _island_index_slots (Variables|/Game/Blueprints/GameSettings/GameInst_DG.GameInst_DG_C|GetIsland%20Index%20Slots _gameinstance))
  ;[0 0 1] Передача данных заполненности слотов островов - Owning Client
  (if (== IslandIndexKey1 999)
    _
    (else
      (Utilities|Map|Add _island_index_slots IslandIndexKey1 IslandIndexSlot1)
      (Utilities|Array|SetArrayElem _islandslot IslandIndexSlot1 true)))
  (if (== IslandIndexKey2 999)
    _
    (else
      (Utilities|Map|Add _island_index_slots IslandIndexKey2 IslandIndexSlot2)
      (Utilities|Array|SetArrayElem _islandslot IslandIndexSlot2 true)))
  (if (== IslandIndexKey3 999)
    _
    (else
      (Utilities|Map|Add _island_index_slots IslandIndexKey3 IslandIndexSlot3)
      (Utilities|Array|SetArrayElem _islandslot IslandIndexSlot3 true)))
  (if (== IslandIndexKey4 999)
    _
    (else
      (Utilities|Map|Add _island_index_slots IslandIndexKey4 IslandIndexSlot4)
      (Utilities|Array|SetArrayElem _islandslot IslandIndexSlot4 true)))
  (Variables|/Game/Blueprints/GameSettings/GameInst_DG.GameInst_DG_C|SetIslandsLoaded (Variables|Default|GetGameInstance) true)
  (CallFunction|LoadWorld))

(event Custom|LoadIslands
  (params (SlotOfIsland :type Integer) (IndexOfIsland :type Integer))
  (bind _gameinstance (Variables|Default|GetGameInstance))
  ;[0 0 1] Загрузка островов
  (Default|CreateIsland (Variables|/Game/Blueprints/NPC/BaseCharacter_DG.BaseCharacter_DG_C|GetLocationNetworkManager (Variables|/Game/Blueprints/GameSettings/GameInst_DG.GameInst_DG_C|GetPlayer%20Character%20DG (Variables|Default|GetGameInstance))) SlotOfIsland IndexOfIsland)
  (for _array_element (Variables|/Game/Blueprints/ReplicatedActors/ServerOnlyNetworkManager.ServerOnlyNetworkManager_C|GetPlayersInfo (Variables|GeneralNetworkManager_C|GetServerOnlyNetworkManager (Variables|/Game/Blueprints/NPC/BaseCharacter_DG.BaseCharacter_DG_C|GetGeneralNetworkManager (Variables|/Game/Blueprints/GameSettings/GameInst_DG.GameInst_DG_C|GetPlayer%20Character%20DG _gameinstance))))
    (if (== (Variables|/Game/Blueprints/PlayerCharacter/PlayerCharacter_DG.PlayerCharacter_DG_C|GetCurrentIsland (.PlayerCharacter (Utilities|Struct|BreakPlayersNetInfo _array_element))) IndexOfIsland)
      (Variables|/Game/Blueprints/GameSettings/GameInst_DG.GameInst_DG_C|SetCurrentPlayerCharacter _gameinstance (.PlayerCharacter (Utilities|Struct|BreakPlayersNetInfo _array_element)))
      (Default|EnterIsland (Variables|/Game/Blueprints/NPC/BaseCharacter_DG.BaseCharacter_DG_C|GetLocationNetworkManager (.PlayerCharacter (Utilities|Struct|BreakPlayersNetInfo _array_element))) IndexOfIsland))))

(event Custom|LoadWorld
  (bind _gameinstance (Variables|Default|GetGameInstance))
  (bind _gameinstance_2 (Variables|Default|GetGameInstance))
  (bind _island_index_slots (Variables|/Game/Blueprints/GameSettings/GameInst_DG.GameInst_DG_C|GetIsland%20Index%20Slots _gameinstance_2))
  ;[0 0 1] Загрузка мира
  (Default|LoadWorld _gameinstance)
  (Variables|/Game/Blueprints/GameSettings/GameInst_DG.GameInst_DG_C|SetInGame? _gameinstance true)
  (bind _keys (Utilities|Map|Keys _island_index_slots))
  (for _array_element _keys
    (CallFunction|LoadIslands (.Value (Utilities|Map|Find _island_index_slots _array_element)) _array_element))
  (CallFunction|CallServertoSetArenaSlotData))

(event Custom|LoadArenas
  (bind _gameinstance (Variables|Default|GetGameInstance))
  (bind _arena_index_slots (Variables|/Game/Blueprints/GameSettings/GameInst_DG.GameInst_DG_C|GetArena%20Index%20Slots _gameinstance))
  ;[0 0 1] Загрузка арены
  (bind _keys (Utilities|Map|Keys _arena_index_slots))
  (for _array_element _keys
    (bind _array_element_2 (Utilities|Array|ForEachLoopwithBreak (Variables|/Game/Blueprints/ReplicatedActors/ServerOnlyNetworkManager.ServerOnlyNetworkManager_C|GetPlayersInfo (Variables|GeneralNetworkManager_C|GetServerOnlyNetworkManager (Variables|/Game/Blueprints/NPC/BaseCharacter_DG.BaseCharacter_DG_C|GetGeneralNetworkManager (Variables|/Game/Blueprints/GameSettings/GameInst_DG.GameInst_DG_C|GetPlayer%20Character%20DG (Variables|Default|GetGameInstance))))) :!label _label)
      (:LoopBody
        (if (== (Variables|/Game/Blueprints/PlayerCharacter/PlayerCharacter_DG.PlayerCharacter_DG_C|GetCurrentArenaHex (.PlayerCharacter (Utilities|Struct|BreakPlayersNetInfo _array_element_2))) (.OrdinarIndex (Utilities|Struct|BreakArenaKey _array_element)))
          (goto _label Break)))
      (:Completed
        (Default|CreateArena-LocationManage (Variables|/Game/Blueprints/NPC/BaseCharacter_DG.BaseCharacter_DG_C|GetLocationNetworkManager (.PlayerCharacter (Utilities|Struct|BreakPlayersNetInfo _array_element_2))) (.Value (Utilities|Map|Find _arena_index_slots _array_element)) (.IslandIndex (Utilities|Struct|BreakArenaKey _array_element)) (.OrdinarIndex (Utilities|Struct|BreakArenaKey _array_element)))
        (for _array_element_3 (Variables|/Game/Blueprints/ReplicatedActors/ServerOnlyNetworkManager.ServerOnlyNetworkManager_C|GetPlayersInfo (Variables|GeneralNetworkManager_C|GetServerOnlyNetworkManager (Variables|/Game/Blueprints/NPC/BaseCharacter_DG.BaseCharacter_DG_C|GetGeneralNetworkManager (Variables|/Game/Blueprints/GameSettings/GameInst_DG.GameInst_DG_C|GetPlayer%20Character%20DG (Variables|Default|GetGameInstance)))))
          (if (== (Variables|/Game/Blueprints/PlayerCharacter/PlayerCharacter_DG.PlayerCharacter_DG_C|GetCurrentArenaHex (.PlayerCharacter (Utilities|Struct|BreakPlayersNetInfo _array_element_3))) (.OrdinarIndex (Utilities|Struct|BreakArenaKey _array_element)))
            (Default|EnterArena-LocationManage (Variables|/Game/Blueprints/NPC/BaseCharacter_DG.BaseCharacter_DG_C|GetLocationNetworkManager (.PlayerCharacter (Utilities|Struct|BreakPlayersNetInfo _array_element_3))) (.IslandIndex (Utilities|Struct|BreakArenaKey _array_element)) (.OrdinarIndex (Utilities|Struct|BreakArenaKey _array_element))))))))
  (CallFunction|CallServerLoadHexParameters)
  (CallFunction|EnableAllInput-Multicast))

(event Custom|CallServerLoadHexParameters
  ;[1 0 0] Передача параметров измененных гексов
  (for _array_element (Variables|/Game/Blueprints/GameSettings/GameInst_DG.GameInst_DG_C|GetHexagonNeedToBeSaved_World (Variables|Default|GetGameInstance))
    (bind (_player1 _player2 _player3 _player4) (CallFunction|FulfillPlayersIndexes _array_element))
    (CallFunction|LoadHexParameters (.a1 (CallFunction|EncodeTwoInttoThreeByte (Variables|/Game/Blueprints/ProceduralGeneration/HexagonCellWorld.HexagonCellWorld_C|GetIndexOfThisIslandInArray _array_element) (Variables|/Game/Blueprints/ProceduralGeneration/HexagonCellWorld.HexagonCellWorld_C|GetOrdinarIndex _array_element))) (.b1 (CallFunction|EncodeTwoInttoThreeByte (Variables|/Game/Blueprints/ProceduralGeneration/HexagonCellWorld.HexagonCellWorld_C|GetIndexOfThisIslandInArray _array_element) (Variables|/Game/Blueprints/ProceduralGeneration/HexagonCellWorld.HexagonCellWorld_C|GetOrdinarIndex _array_element))) (.b2 (CallFunction|EncodeTwoInttoThreeByte (Variables|/Game/Blueprints/ProceduralGeneration/HexagonCellWorld.HexagonCellWorld_C|GetIndexOfThisIslandInArray _array_element) (Variables|/Game/Blueprints/ProceduralGeneration/HexagonCellWorld.HexagonCellWorld_C|GetOrdinarIndex _array_element))) (CallFunction|EncodeFourInttoOneInt _player1 _player2 _player3 _player4))))

(event Custom|SetIslandsOnWorldMapFromServer
  (params (IslandOnWorldMap :type Islands%20on%20World%20Map%20Save%20Structure) (Lenght :type Integer))
  ;[0 0 1] Передача сохранений островов по циклу. Owning Client
  (bind _returnvalue (Utilities|Array|Add (Variables|/Game/Blueprints/GameSettings/WorldStorage.WorldStorage_C|GetIslandsOnWorldMap (Variables|/Game/Blueprints/GameSettings/GameInst_DG.GameInst_DG_C|GetActiveSaveGame_WorldStorage (Variables|Default|GetGameInstance))) IslandOnWorldMap))
  (Variables|Default|SetIslandsOnWorldMapFill? (== _returnvalue (- Lenght 1)))
  (if (Variables|Default|GetIslandsOnWorldMapFill?)
    (CallFunction|CallServertoSetSaveData)
    (else
      (CallFunction|CallServertoSetIslandonWorldMap (Math|Conversions|ToByte(Integer) (+ _returnvalue 1))))))

(event Custom|LoadHexParameters
  (params (IndexOfThisIslandInArray :type Byte) (OrdinarIndex1 :type Byte) (OrdinarIndex2 :type Byte) (PlayersAssignToBattle :type Integer))
  ;[0 0 1] Передача параметров измененных гексов
  (CallFunction|FulfillPlayerReadytoBattleArray IndexOfThisIslandInArray OrdinarIndex1 OrdinarIndex2 PlayersAssignToBattle))

(event Custom|Disable%20All%20Input%20-%20Server
  ;[1 0 0] Переключение инпутов - Сервер
  (CallFunction|DisableAllInput))

(event Custom|Enable%20All%20Input%20-%20Multicast
  ;[1 0 0] Переключение инпутов - Сервер
  (CallFunction|EnableAllInput))

(event Custom|CallServerToSetWorldClusterData
  (params (InByte :type Byte))
  (bind _worldclusterdata (|CurrentSaveData_2_2_2))
  ;[1 0 0] Передача данных сохранения секторов. Серверная часть
  (CallFunction|SetWorldClusterData (Utilities|Array|Get(acopy) _worldclusterdata (Math|Conversions|ToInteger(Byte) InByte)) (Utilities|Array|Length _worldclusterdata)))

(event Custom|Call%20Position%20Adjustment
  ;[0 0 1] Вызов корректировки положения всех игроков с сервером
  (Default|PositionAdjustmentClient (Variables|/Game/Blueprints/GameSettings/GameInst_DG.GameInst_DG_C|GetPlayer%20Character%20DG (Variables|Default|GetGameInstance)))
  (Development|PrintString "Корректировка положения игроков произведена..."))

(event Custom|CallLoadSaveData
  ;[0 1 0] Инициализация загрузки данных
  (CallFunction|CallServertoSetIslandonWorldMap)
  (CallFunction|DisableAllInput-Server))

(event Custom|CallServerToSetIslandOnWorldMap
  (params (Index_IslandOnWorldMap :type Byte))
  (bind _islandsonworldmap (|CurrentSaveData_4))
  ;[1 0 0] Передача сохранений островов по циклу. Серверная часть
  (CallFunction|SetIslandsonWorldMapfromServer (Utilities|Array|Get(acopy) _islandsonworldmap (Math|Conversions|ToInteger(Byte) Index_IslandOnWorldMap)) (Utilities|Array|Length _islandsonworldmap)))

(event Custom|EnableAllInput
  ;[0 0 1] Переключение инпутов
  (bind _asplayer_controller_dg (Utilities|Casting|CastToPlayerController_DG (Game|GetPlayerController 0)))
  (Input|SetInputModeGameandUI _asplayer_controller_dg 0 "DoNotLock" true))

(event Custom|DisableAllInput
  ;[0 0 1] Переключение инпутов
  (bind _asplayer_controller_dg (Utilities|Casting|CastToPlayerController_DG (Game|GetPlayerController 0)))
  (Input|SetInputModeUIOnly _asplayer_controller_dg 0 "DoNotLock"))