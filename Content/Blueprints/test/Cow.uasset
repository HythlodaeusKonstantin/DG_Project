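; Cow is a test actor that slides along negative Y and takes on the material of any Cow112 it overlaps.
; Tick applies a fixed, unswept world offset each frame, so its speed depends on frame rate.
; On overlap, it casts the other actor to Cow112, copies that actor's CurMat onto its StaticMesh and plays a 2D sound.
; BeginPlay caches its own starting material in CurMat.
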(event EventBeginPlay
  (Variables|Default|SetCurMat (Rendering|Material|GetMaterial (Variables|Default|GetStaticMesh) 0)))

(event Collision|EventActorBeginOverlap
  (params (OtherActor :type Actor%20Object%20Reference))
  (bind _ascow_112 (Utilities|Casting|CastToCow112 OtherActor))
  (Rendering|Material|SetMaterial (Variables|Default|GetStaticMesh) 0 (Variables|/Game/Blueprints/test/Cow112.Cow112_C|GetCurMat _ascow_112))
  (Audio|PlaySound2D "/Game/Blueprints/test/y2mate-_mp3cut_net_.y2mate-_mp3cut_net_" 1.0 1.0 0.0 0 0))

(event EventTick
  (params (DeltaSeconds :type Float%20%28single-precision%29))
  (Transformation|AddActorWorldOffset "0,-15.000000, 0"))

(fn ConstructionScript)