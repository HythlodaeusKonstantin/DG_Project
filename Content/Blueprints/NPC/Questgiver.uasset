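; Questgiver NPC Blueprint that builds a randomly gendered villager from modular skeletal meshes.
; The construction script flips a 50/50 coin for Gender, then assigns matching body, hair, tunic, pants and shoe meshes, adding a beard for males and clearing it for females.
; Because the roll happens at construction, appearance can change whenever the script reruns.
; The event graph has no active logic, so no quest behavior is implemented here.
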(event EventBeginPlay
  (|CallParentFunction) ; This node is disabled and will not be called.\nDrag off pins to build functionality.
)

(event Collision|EventActorBeginOverlap
  (params (OtherActor :type Actor%20Object%20Reference)))

(event EventTick
  (params (DeltaSeconds :type Float%20%28single-precision%29)))

(fn ConstructionScript
  (|CallParentFunction)
  (Utilities|RandomCase 0.5
    (:true
      (Variables|Default|SetGender true))
    (:false
      (Variables|Default|SetGender false)))
  (if (Variables|Default|GetGender)
    (Class|SkinnedMeshComponent|SetSkeletalMesh (Variables|Default|GetBaseSkeletalMesh) "/Game/Meshes/Character/Male/Character_Male.Character_Male" true)
    (Class|SkinnedMeshComponent|SetSkeletalMesh (Variables|Default|GetHair) "/Game/Meshes/Character/Male/Hair/Male_Hair1.Male_Hair1" true)
    (Class|SkinnedMeshComponent|SetSkeletalMesh (Variables|Default|GetBeard) "/Game/Meshes/Character/Male/Hair/Beard1.Beard1" true)
    (Class|SkinnedMeshComponent|SetSkeletalMesh (Variables|Default|GetClothesBody) "/Game/Meshes/Character/Male/Clothes/Tunic_Male.Tunic_Male" true)
    (Class|SkinnedMeshComponent|SetSkeletalMesh (Variables|Default|GetClothesPants) "/Game/Meshes/Character/Male/Clothes/Pants_Male.Pants_Male" true)
    (Class|SkinnedMeshComponent|SetSkeletalMesh (Variables|Default|GetClothesShoes) "/Game/Meshes/Character/Male/Clothes/Shoes_Male.Shoes_Male" true)
    (else
      (Class|SkinnedMeshComponent|SetSkeletalMesh (Variables|Default|GetBaseSkeletalMesh) "/Game/Meshes/Character/Female/Character_Female.Character_Female" true)
      (Class|SkinnedMeshComponent|SetSkeletalMesh (Variables|Default|GetHair) "/Game/Meshes/Character/Female/Hair/Female_Hair1.Female_Hair1" true)
      (Class|SkinnedMeshComponent|SetSkeletalMesh (Variables|Default|GetBeard) 0 true)
      (Class|SkinnedMeshComponent|SetSkeletalMesh (Variables|Default|GetClothesBody) "/Game/Meshes/Character/Female/Clothes/Tunic_Female.Tunic_Female" true)
      (Class|SkinnedMeshComponent|SetSkeletalMesh (Variables|Default|GetClothesPants) "/Game/Meshes/Character/Female/Clothes/Pants_Female.Pants_Female" true)
      (Class|SkinnedMeshComponent|SetSkeletalMesh (Variables|Default|GetClothesShoes) "/Game/Meshes/Character/Female/Clothes/Shoes_Female.Shoes_Female" true))))