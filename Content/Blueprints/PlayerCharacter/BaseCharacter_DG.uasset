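; Player character Blueprint that moves across hex grids on the world map, island and battle arena.
; Clicks trigger a greedy best-first search using a distance-keyed map as priority queue, where equal distances overwrite each other.
; Paths are walked cell by cell through server and multicast events driving MovementComponent.
; World and island steps each cost an action point; arena steps are free, but its search rejects height differences above one.
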(event Custom|OnClick
  (params (TargetHexCell :type Hexagon%20Cell%20World%20Object%20Reference) (ClickedHexCell :type Hexagon%20Cell%20World%20Object%20Reference))
  ;[1 1 1 0.25] Логика выстраивания пути и перемещения персонажа по гексам на карте мира\острова
  ;;[0 1 0] Эвент по клику на гекс, стартовые проверки
  (if (not (Variables|MovementParent|GetMakeActiveStep))
    (Variables|MovementParent|SetMakeActiveStep true)
    (Variables|MovementParent|SetTargetHexagonCell TargetHexCell)
    (Variables|MovementParent|SetClickedHexCell ClickedHexCell)
    (if (Variables|MovementParent|GetOnWorldMap?)
      (Variables|MovementParent|SetHexagon%20Cells%20ALL%20-%20FindPath (Variables|/Game/Blueprints/ProceduralGeneration/ProceduralWorldGeneration.ProceduralWorldGeneration_C|GetHexagonCells-ALL (Variables|/Game/Blueprints/GameSettings/GameInst_DG.GameInst_DG_C|GetWorldGenerationNetwork (Variables|Default|GetGameInst))))
      (CallFunction|MovebyPath (Variables|MovementParent|GetTargetHexagonCell))
      (else
        (Variables|MovementParent|SetHexagon%20Cells%20ALL%20-%20FindPath (Variables|/Game/Blueprints/ProceduralGeneration/ProceduralHexagonalNetwork.ProceduralHexagonalNetwork_C|GetHexagonCells-ALL (Variables|/Game/Blueprints/GameSettings/GameInst_DG.GameInst_DG_C|GetIslandGenerationNetwork (Variables|Default|GetGameInst))))
        (CallFunction|MovebyPath (Variables|MovementParent|GetTargetHexagonCell))))))

(event Custom|MoveToLocation_Server
  (params (TargetLocation :type Vector) (Key :type Integer%20%28by%20ref%29))
  ;[1 1 1 0.25] Логика выстраивания пути и перемещения персонажа по гексам на карте мира\острова
  ;;[1 0 0] Вызываем мультикаст эвент с сервера и передаем данные для перемещения
  (Utilities|MinusOneActionPoint
    (:ActionPoints
      (CallFunction|MovetoLocationMulticast TargetLocation Key))
    (:NoActionPoints
      (CallFunction|SetMakeActiveStep-False))))

(event Custom|StopMoving%20-%20Client
  ;[1 1 1 0.25] Логика выстраивания пути и перемещения персонажа по гексам на карте мира\острова
)

(event Custom|SetMakeActiveStep%20-%20False
  ;[1 1 1 0.25] Логика выстраивания пути и перемещения персонажа по гексам на карте мира\острова
  ;;[0 0 1] Устанавливаем MakeActiveStep на false
  (Variables|MovementParent|SetMakeActiveStep false)
  (CallFunction|StopMoving-Client))

(event Custom|MoveByPathArena
  (params (goalCell :type Hexagon%20Cell%20Arena%20Object%20Reference))
  ;[0 1 0] Передвижение персонажа по выстроенному пути
  (bind _foundpath (CallFunction|FindPathArena (Variables|MovementParent|GetcurrentCharacterLocationArena) goalCell))
  (bind _output_get (Variables|MovementParent|SetFound%20Path%20Arena _foundpath))
  (if (== (Utilities|Array|Length _output_get) 0)
    (Variables|MovementParent|SetMakeActiveStep false)
    (CallFunction|StopMovingArena)
    (Development|PrintString "ПУСТО")
    (else
      (Utilities|Array|Reverse _output_get)
      (Utilities|Array|RemoveItem _output_get (Utilities|Array|Get(acopy) _output_get))
      (CallFunction|MovetoLocationServerArena (Transformation|GetActorLocation (Utilities|Array|Get(acopy) _output_get)) (Variables|/Game/Blueprints/ProceduralGeneration/HexagonCellArena.HexagonCellArena_C|GetOrdinarIndex (Utilities|Array|Get(acopy) _output_get))))))

(event Custom|moveByPath
  (params (targetCell :type Hexagon%20Cell%20World%20Object%20Reference))
  ;[1 1 1 0.25] Логика выстраивания пути и перемещения персонажа по гексам на карте мира\острова
  ;;[0 1 0] Передвижение персонажа по выстроенному пути
  (bind _foundpath (CallFunction|FindPath (Variables|MovementParent|GetcurrentCharacterLocation) targetCell (Variables|MovementParent|GetHexagon%20Cells%20ALL%20-%20FindPath)))
  (bind _output_get (Variables|MovementParent|SetFound%20Path _foundpath))
  (if (== (Utilities|Array|Length _output_get) 0)
    (Variables|MovementParent|SetMakeActiveStep false)
    (CallFunction|StopMoving-Client)
    (Development|PrintString "ПУСТО")
    (else
      (Utilities|Array|Reverse _output_get)
      (Utilities|Array|RemoveItem _output_get (Utilities|Array|Get(acopy) _output_get))
      (CallFunction|MovetoLocationServer (Transformation|GetActorLocation (Utilities|Array|Get(acopy) _output_get)) (Variables|/Game/Blueprints/ProceduralGeneration/HexagonCellWorld.HexagonCellWorld_C|GetOrdinarIndex (Utilities|Array|Get(acopy) _output_get))))))

(event Custom|makeStepArena
  (bind _found_path_arena (Variables|MovementParent|GetFound%20Path%20Arena))
  (bind _returnvalue (Utilities|Array|Length _found_path_arena))
  (bind _output (Utilities|Array|Get(acopy) _found_path_arena))
  (bind _returnvalue_2 (== _returnvalue 0))
  ;[0 1 0] Передвижение на один гекс по выстроенному пути
  (if _returnvalue_2
    (Variables|MovementParent|SetMakeActiveStep false)
    (CallFunction|StopMovingArena)
    (else
      (Utilities|Array|RemoveItem _found_path_arena _output)
      (if _returnvalue_2
        (Variables|MovementParent|SetMakeActiveStep false)
        (CallFunction|StopMovingArena)
        (else
          (CallFunction|MovetoLocationServerArena (Transformation|GetActorLocation _output) (Variables|/Game/Blueprints/ProceduralGeneration/HexagonCellArena.HexagonCellArena_C|GetOrdinarIndex _output)))))))

(event Custom|StopMovingArena)

(event Custom|makeStep
  (bind _found_path (Variables|MovementParent|GetFound%20Path))
  (bind _returnvalue (Utilities|Array|Length _found_path))
  (bind _output (Utilities|Array|Get(acopy) _found_path))
  (bind _returnvalue_2 (== _returnvalue 0))
  ;[1 1 1 0.25] Логика выстраивания пути и перемещения персонажа по гексам на карте мира\острова
  ;;[0 1 0] Передвижение на один гекс по выстроенному пути
  (if _returnvalue_2
    (Variables|MovementParent|SetMakeActiveStep false)
    (CallFunction|StopMoving-Client)
    (else
      (Utilities|Array|RemoveItem _found_path _output)
      (if _returnvalue_2
        (Variables|MovementParent|SetMakeActiveStep false)
        (CallFunction|StopMoving-Client)
        (else
          (CallFunction|MovetoLocationServer (Transformation|GetActorLocation _output) (Variables|/Game/Blueprints/ProceduralGeneration/HexagonCellWorld.HexagonCellWorld_C|GetOrdinarIndex _output)))))))

(event Custom|MoveToLocation_ServerArena
  (params (TargetLocation :type Vector) (Key :type Integer%20%28by%20ref%29))
  ;[1 0 0] Вызываем мультикаст эвент с сервера и передаем данные для перемещения - Арена
  (CallFunction|MovetoLocationMulticastArena TargetLocation Key))

(event Custom|MoveToLocation_MulticastArena
  (params (TargetLocation :type Vector) (Key :type Integer%20%28by%20ref%29))
  (bind _gameinst (Variables|Default|GetGameInst))
  (bind _arenanetwork (Variables|/Game/Blueprints/GameSettings/GameInst_DG.GameInst_DG_C|GetArenaNetwork _gameinst))
  (bind _hexallmapordinarindex (Variables|/Game/Blueprints/ProceduralGeneration/ArenaNetwork.ArenaNetwork_C|GetHexAllMapOrdinarIndex _arenanetwork))
  (bind _value (Utilities|Map|Find _hexallmapordinarindex Key))
  ;[0 0 1] Мультикаст вызыв перемещения персонажа к указанным координатам - Арена
  (Default|MovetoLocation (Variables|Default|GetMovementComponent) TargetLocation (Variables|/Game/Blueprints/ProceduralGeneration/HexagonCellArena.HexagonCellArena_C|GetHexagonCellOwner _value))
  (Variables|MovementParent|SetcurrentCharacterLocationArena _value))

(event Custom|SetMakeActivaStep-FalseArena
  ;[0 0 1] Устанавливаем MakeActiveStep на false Арена
  (Variables|MovementParent|SetMakeActiveStep false)
  (CallFunction|StopMovingArena))

(event Custom|MoveToLocation_Multicast
  (params (TargetLocation :type Vector) (Key :type Integer%20%28by%20ref%29))
  (bind _gameinst (Variables|Default|GetGameInst))
  ;[1 1 1 0.25] Логика выстраивания пути и перемещения персонажа по гексам на карте мира\острова
  ;;[0 0 1] Мультикаст вызыв перемещения персонажа к указанным координатам
  (if (Variables|MovementParent|GetOnWorldMap?)
    (Variables|MovementParent|SetcurrentCharacterLocation (.Value (Utilities|Map|Find (Variables|/Game/Blueprints/ProceduralGeneration/ProceduralWorldGeneration.ProceduralWorldGeneration_C|GetHexAllMap_OrdinarIndex (Variables|/Game/Blueprints/GameSettings/GameInst_DG.GameInst_DG_C|GetWorldGenerationNetwork _gameinst)) Key)))
    (else
      (Variables|MovementParent|SetcurrentCharacterLocation (.Value (Utilities|Map|Find (Variables|/Game/Blueprints/ProceduralGeneration/ProceduralHexagonalNetwork.ProceduralHexagonalNetwork_C|GetHexAllMapInt (Variables|/Game/Blueprints/GameSettings/GameInst_DG.GameInst_DG_C|GetIslandGenerationNetwork _gameinst)) Key)))))
  (Default|MovetoLocation (Variables|Default|GetMovementComponent) TargetLocation (Variables|/Game/Blueprints/ProceduralGeneration/HexagonCellWorld.HexagonCellWorld_C|GetHexagonCellOwner (Variables|MovementParent|GetcurrentCharacterLocation))))

(event Custom|OnClick_BattleArena
  (params (TargetHexagonCell :type Hexagon%20Cell%20Arena%20Object%20Reference))
  ;[0 1 0] Эвент по клику на гекс, стартовые проверки - Арена
  (if (not (Variables|MovementParent|GetMakeActiveStep))
    (Variables|MovementParent|SetMakeActiveStep true)
    (bind _output_get (Variables|MovementParent|SetTarget%20Hexagon%20Cell%20Arena TargetHexagonCell))
    (CallFunction|MovebyPathArena _output_get)))

(event Custom|clientCallSetTransform
  (params (NewLocation :type Vector))
  ;[1 1 1 0.25] Логика выстраивания пути и перемещения персонажа по гексам на карте мира\острова
  ;;[0 1 0] Вызов перемещения у клиента
  (CallFunction|ServerSetTransform NewLocation))

(event Custom|ServerSetTransform
  (params (NewLocation :type Vector))
  ;[1 1 1 0.25] Логика выстраивания пути и перемещения персонажа по гексам на карте мира\острова
  ;;[1 0 0] Перемещение на сервере
  (CallFunction|MulticastSetTransform NewLocation))

(event Custom|MulticastSetTransform
  (params (NewLocation :type Vector))
  ;[1 1 1 0.25] Логика выстраивания пути и перемещения персонажа по гексам на карте мира\острова
  ;;[0 0 1] Перемещение у всех клиентов
  (Transformation|SetActorLocation NewLocation false false))

(event EventBeginPlay
  ;[0 0 0] Инициализация
  (bind _asgame_inst_dg (Utilities|Casting|CastToGameInst_DG (Game|GetGameInstance)))
  (Variables|Default|SetGameInst _asgame_inst_dg))

(fn ConstructionScript)

(fn FindPath
  (params (startCell :type Hexagon%20Cell%20World%20Object%20Reference) (goalCell :type Hexagon%20Cell%20World%20Object%20Reference) (hexAllArray :type Array%20of%20Hexagon%20Cell%20World%20Object%20References))
  ;[1 1 1] Подготовка и помещение первой вершины в очередь с приоритетом
  (CallFunction|RefreshCells hexAllArray)
  (LocalVariables|SetnotFound? true)
  (LocalVariables|Setstart startCell)
  (LocalVariables|Setfinish goalCell)
  (Variables|/Game/Blueprints/ProceduralGeneration/HexagonCellWorld.HexagonCellWorld_C|SetpathfinderVisited (LocalVariables|Getstart) true)
  (Utilities|Map|Add (LocalVariables|GetfrontierQueue) (Transformation|GetDistanceTo (LocalVariables|Getstart) (LocalVariables|Getfinish)) (LocalVariables|Getstart))
  ;[1 1 1] Пока в очереди есть хотя бы одна вершина
  (while (> (Utilities|Map|Length (LocalVariables|GetfrontierQueue)) 0)
    ;[1 1 1] Берем из своеобразной очереди с приоритетом самую приоритетную вершину
    (bind _keys (Utilities|Map|Keys (LocalVariables|GetfrontierQueue)))
    (bind _output_get (LocalVariables|SetminCost (.MinValue (Math|Float|MinOfFloatArray _keys))))
    (LocalVariables|Setcurrent (.Value (Utilities|Map|Find (LocalVariables|GetfrontierQueue) _output_get)))
    (Utilities|Map|Remove (LocalVariables|GetfrontierQueue) (LocalVariables|GetminCost))
    ;[1 1 1] Дошли до финиша?
    (if (== (LocalVariables|Getcurrent) (LocalVariables|Getfinish))
      (Utilities|IsValid (Variables|/Game/Blueprints/ProceduralGeneration/HexagonCellWorld.HexagonCellWorld_C|GetcameFrom (LocalVariables|Getfinish))
        (:Is%20Valid
          (LocalVariables|Setcurrent (LocalVariables|Getfinish))
          ;[1 1 1] Пока не найден путь
          (while (LocalVariables|GetnotFound?)
            (Utilities|Array|Add (LocalVariables|Getpath) (LocalVariables|Getcurrent))
            (bind _output_get_2 (LocalVariables|Setcurrent (Variables|/Game/Blueprints/ProceduralGeneration/HexagonCellWorld.HexagonCellWorld_C|GetcameFrom (LocalVariables|Getcurrent))))
            ;[1 1 1] Нашли путь?
            (if (== (LocalVariables|Getstart) _output_get_2)
              (LocalVariables|SetnotFound? false)
              (Utilities|Array|Add (LocalVariables|Getpath) (LocalVariables|Getstart)))))
        (:Is%20Not%20Valid
          (Development|PrintString "Нет пути..." true true "(R=1.000000,G=0.000000,B=0.023098,A=1.000000)")))
      (return (LocalVariables|Getpath))
      (else
        ;[1 1 1] Для каждого соседа считаем рассточние до точки финиша (то есть приоритет) и затем заносим в очередь пару "расстояние-ячейка"
        (bind _array_element (Utilities|Array|ForEachLoopwithBreak (Variables|/Game/Blueprints/ProceduralGeneration/HexagonCellWorld.HexagonCellWorld_C|GetNeigborsHex (LocalVariables|Getcurrent)))
          (:LoopBody
            (bind _output_get_3 (LocalVariables|SetcurrentNeighbour _array_element))
            (if (not (Variables|/Game/Blueprints/ProceduralGeneration/HexagonCellWorld.HexagonCellWorld_C|GetpathfinderVisited _output_get_3))
              (if (Variables|/Game/Blueprints/ProceduralGeneration/HexagonCellWorld.HexagonCellWorld_C|GetCanPass? _output_get_3)
                (Utilities|Map|Add (LocalVariables|GetfrontierQueue) (Transformation|GetDistanceTo _output_get_3 (LocalVariables|Getfinish)) (LocalVariables|GetcurrentNeighbour))
                (Variables|/Game/Blueprints/ProceduralGeneration/HexagonCellWorld.HexagonCellWorld_C|SetpathfinderVisited (LocalVariables|GetcurrentNeighbour) true)
                (Variables|/Game/Blueprints/ProceduralGeneration/HexagonCellWorld.HexagonCellWorld_C|SetcameFrom (LocalVariables|GetcurrentNeighbour) (LocalVariables|Getcurrent)))))))))
  (Utilities|IsValid (Variables|/Game/Blueprints/ProceduralGeneration/HexagonCellWorld.HexagonCellWorld_C|GetcameFrom (LocalVariables|Getfinish))
    (:Is%20Valid
      (LocalVariables|Setcurrent (LocalVariables|Getfinish))
      (while (LocalVariables|GetnotFound?)
        (Utilities|Array|Add (LocalVariables|Getpath) (LocalVariables|Getcurrent))
        (bind _output_get_4 (LocalVariables|Setcurrent (Variables|/Game/Blueprints/ProceduralGeneration/HexagonCellWorld.HexagonCellWorld_C|GetcameFrom (LocalVariables|Getcurrent))))
        (if (== (LocalVariables|Getstart) _output_get_4)
          (LocalVariables|SetnotFound? false)
          (Utilities|Array|Add (LocalVariables|Getpath) (LocalVariables|Getstart)))))
    (:Is%20Not%20Valid
      (Development|PrintString "Нет пути..." true true "(R=1.000000,G=0.000000,B=0.023098,A=1.000000)")))
  (return (LocalVariables|Getpath)))

(fn FindPathArena
  (params (startCell :type Hexagon%20Cell%20Arena%20Object%20Reference) (goalCell :type Hexagon%20Cell%20Arena%20Object%20Reference))
  ;[1 1 1] Подготовка и помещение первой вершины в очередь с приоритетом
  (LocalVariables|SetnotFound? true)
  (LocalVariables|Setstart startCell)
  (LocalVariables|Setfinish goalCell)
  (Utilities|Array|Add (LocalVariables|GetvisitedCells) (LocalVariables|Getstart))
  (Utilities|Map|Add (LocalVariables|GetfrontierQueue) (Transformation|GetDistanceTo (LocalVariables|Getstart) (LocalVariables|Getfinish)) (LocalVariables|Getstart))
  ;[1 1 1] Пока в очереди есть хотя бы одна вершина
  (while (> (Utilities|Map|Length (LocalVariables|GetfrontierQueue)) 0)
    ;[1 1 1] Берем из своеобразной очереди с приоритетом самую приоритетную вершину
    (bind _keys (Utilities|Map|Keys (LocalVariables|GetfrontierQueue)))
    (bind _output_get (LocalVariables|SetminCost (.MinValue (Math|Float|MinOfFloatArray _keys))))
    (LocalVariables|Setcurrent (.Value (Utilities|Map|Find (LocalVariables|GetfrontierQueue) _output_get)))
    (Utilities|Map|Remove (LocalVariables|GetfrontierQueue) (LocalVariables|GetminCost))
    ;[1 1 1] Дошли до финиша?
    (if (== (LocalVariables|Getcurrent) (LocalVariables|Getfinish))
      (Utilities|IsValid (.Value (Utilities|Map|Find (LocalVariables|GetcameFrom) (LocalVariables|Getfinish)))
        (:Is%20Valid
          (LocalVariables|Setcurrent (LocalVariables|Getfinish))
          ;[1 1 1] Пока не найден путь
          (while (LocalVariables|GetnotFound?)
            (Utilities|Array|Add (LocalVariables|Getpath) (LocalVariables|Getcurrent))
            (bind _output_get_2 (LocalVariables|Setcurrent (.Value (Utilities|Map|Find (LocalVariables|GetcameFrom) (LocalVariables|Getcurrent)))))
            ;[1 1 1] Нашли путь?
            (if (== _output_get_2 (LocalVariables|Getstart))
              (LocalVariables|SetnotFound? false)
              (Utilities|Array|Add (LocalVariables|Getpath) (LocalVariables|Getstart)))))
        (:Is%20Not%20Valid
          (Development|PrintString "Нет пути..." true true "(R=1.000000,G=0.000000,B=0.023098,A=1.000000)")))
      (return (LocalVariables|Getpath))
      (else
        ;[1 1 1] Для каждого соседа считаем рассточние до точки финиша (то есть приоритет) и затем заносим в очередь пару "расстояние-ячейка"
        (bind _array_element (Utilities|Array|ForEachLoopwithBreak (Variables|/Game/Blueprints/ProceduralGeneration/HexagonCellArena.HexagonCellArena_C|GetNeigborsHex (LocalVariables|Getcurrent)))
          (:LoopBody
            (bind _output_get_3 (LocalVariables|SetcurrentNeighbour _array_element))
            (if (not (Utilities|Array|ContainsItem (LocalVariables|GetvisitedCells) _output_get_3))
              (if (Variables|/Game/Blueprints/ProceduralGeneration/HexagonCellArena.HexagonCellArena_C|GetCanPass? _output_get_3)
                (if (> (Math|Integer|Absolute(Integer) (- (Math|Conversions|ToInteger(Byte) (Variables|/Game/Blueprints/ProceduralGeneration/HexagonCellArena.HexagonCellArena_C|GetHexHeight (LocalVariables|GetcurrentNeighbour))) (Math|Conversions|ToInteger(Byte) (Variables|/Game/Blueprints/ProceduralGeneration/HexagonCellArena.HexagonCellArena_C|GetHexHeight (LocalVariables|Getcurrent))))) 1)
                  (Development|PrintString "Hello")
                  (else
                    (Utilities|Map|Add (LocalVariables|GetfrontierQueue) (Transformation|GetDistanceTo _output_get_3 (LocalVariables|Getfinish)) (LocalVariables|GetcurrentNeighbour))
                    (Utilities|Array|Add (LocalVariables|GetvisitedCells) (LocalVariables|GetcurrentNeighbour))
                    (Utilities|Map|Add (LocalVariables|GetcameFrom) (LocalVariables|GetcurrentNeighbour) (LocalVariables|Getcurrent)))))))))))
  (Utilities|IsValid (.Value (Utilities|Map|Find (LocalVariables|GetcameFrom) (LocalVariables|Getfinish)))
    (:Is%20Valid
      (LocalVariables|Setcurrent (LocalVariables|Getfinish))
      (while (LocalVariables|GetnotFound?)
        (Utilities|Array|Add (LocalVariables|Getpath) (LocalVariables|Getcurrent))
        (bind _output_get_4 (LocalVariables|Setcurrent (.Value (Utilities|Map|Find (LocalVariables|GetcameFrom) (LocalVariables|Getcurrent)))))
        (if (== _output_get_4 (LocalVariables|Getstart))
          (LocalVariables|SetnotFound? false)
          (Utilities|Array|Add (LocalVariables|Getpath) (LocalVariables|Getstart)))))
    (:Is%20Not%20Valid
      (Development|PrintString "Нет пути..." true true "(R=1.000000,G=0.000000,B=0.023098,A=1.000000)")))
  (return (LocalVariables|Getpath)))

(fn RefreshCells
  (params (hexAllArray :type Array%20of%20Hexagon%20Cell%20World%20Object%20References))
  (for _array_element hexAllArray
    (Variables|/Game/Blueprints/ProceduralGeneration/HexagonCellWorld.HexagonCellWorld_C|SetpathfinderVisited _array_element false)
    (Variables|/Game/Blueprints/ProceduralGeneration/HexagonCellWorld.HexagonCellWorld_C|SetcameFrom _array_element 0)))