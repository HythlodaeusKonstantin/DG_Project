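; Combat component that applies healing and typed damage to a Health value, with armor mitigation per damage type.
; EventChangeHealth adds a truncated amount to Health, scaling heals by HealDiff and reducing other changes by the percentage from ArmorCulculations.
; ArmorCulculations selects the matching fire, ice, poison, light, darkness or physical defense and sums a geometrically decaying series over it, giving diminishing returns per armor point.
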(event Custom|EventChangeHealth
  (params (HealthEvent :type Integer) (DamageType :type DamageType%20Enum :default "NewEnumerator0"))
  ;[1 1 1] Логика изменения здоровья (урон или хил, вкючая тип урона) и вычисление скейлящегося вычитания урона от брони
  (if (Utilities|Enum|Equal(Enum) DamageType "NewEnumerator7")
    (Variables|Defence|SetHealth (+ (Math|Float|Truncate (* HealthEvent (Variables|Defence|GetHealDiff))) (Variables|Defence|GetHealth)))
    (else
      (bind _defarmor_ (CallFunction|ArmorCulculations DamageType))
      (Variables|Defence|SetHealth (+ (Math|Float|Truncate (- (Math|Conversions|ToFloat(Integer) HealthEvent) (* HealthEvent (/ _defarmor_ 1e+02)))) (Variables|Defence|GetHealth))))))

(event EventBeginPlay)

(event EventTick
  (params (DeltaSeconds :type Float%20%28single-precision%29)))

(fn ArmorCulculations
  (params (DamageType :type DamageType%20Enum :default "NewEnumerator0"))
  (switch Utilities|FlowControl|Switch|SwitchonDamageType DamageType
    (:NewEnumerator0
      (Variables|Defence|SetArmor (Variables|Defence|GetDefFire)))
    (:NewEnumerator1
      (Variables|Defence|SetArmor (Variables|Defence|GetDefIce)))
    (:NewEnumerator2
      (Variables|Defence|SetArmor (Variables|Defence|GetDefPoison)))
    (:NewEnumerator3
      (Variables|Defence|SetArmor (Variables|Defence|GetDefLight)))
    (:NewEnumerator4
      (Variables|Defence|SetArmor (Variables|Defence|GetDefDarkness)))
    (:NewEnumerator5
      (Variables|Defence|SetArmor (Variables|Defence|GetDefPhysic))))
  (for _index (range 0 (Variables|Defence|GetArmor))
    (bind _output_get (LocalVariables|SetTempArmorIndex (* (LocalVariables|GetTempArmorIndex) 0.952)))
    (LocalVariables|SetLocalDefArmor (+ _output_get (LocalVariables|GetLocalDefArmor))))
  (return (LocalVariables|GetLocalDefArmor)))