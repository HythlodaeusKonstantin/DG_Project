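; Placeable hex-cell point of interest that acts as a two-way portal for the player character, on either the world map or the arena grid.
; Portal picks the world or arena hexagon pair via InWorld and requires the player within one hex of the currently active end.
; FlipFlopCustom toggles the stored FlipFlop state, alternating the destination, then the player character's Everyone calls update its transform and current cell.
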(event EventBeginPlay
  (bind _asgame_inst_dg (Utilities|Casting|CastToGameInst_DG (Game|GetGameInstance)))
  (Variables|Default|SetGame%20Inst%20DG _asgame_inst_dg))

(fn ConstructionScript)

(fn Portal
  (bind _game_inst_dg (Variables|Default|GetGame%20Inst%20DG))
  (bind _hexagonout_arena (Variables|Portal|GetHexagonOut_Arena))
  (bind _game_inst_dg_2 (Variables|Default|GetGame%20Inst%20DG))
  (bind _hexagonin_world (Variables|Portal|GetHexagonIn_World))
  (bind _hexagonout_world (Variables|Portal|GetHexagonOut_World))
  (bind _game_inst_dg_3 (Variables|Default|GetGame%20Inst%20DG))
  (bind _hexagonin_arena (Variables|Portal|GetHexagonIn_Arena))
  (bind _player_character_dg (Variables|/Game/Blueprints/GameSettings/GameInst_DG.GameInst_DG_C|GetPlayer%20Character%20DG _game_inst_dg))
  (bind _player_character_dg_2 (Variables|/Game/Blueprints/GameSettings/GameInst_DG.GameInst_DG_C|GetPlayer%20Character%20DG _game_inst_dg_2))
  (bind _player_character_dg_3 (Variables|/Game/Blueprints/GameSettings/GameInst_DG.GameInst_DG_C|GetPlayer%20Character%20DG _game_inst_dg_3))
  (bind _currentcharacterlocationworld (Variables|/Game/Blueprints/NPC/BaseCharacter_DG.BaseCharacter_DG_C|GetcurrentCharacterLocationWorld _player_character_dg_2))
  (bind _currentcharacterlocationarena (Variables|/Game/Blueprints/NPC/BaseCharacter_DG.BaseCharacter_DG_C|GetcurrentCharacterLocationArena _player_character_dg_2))
  (if (Variables|Portal|GetInWorld)
    (if (Variables|Portal|GetFlipFlop)
      (if (<= (CallFunction|HexagonDistance _currentcharacterlocationworld (Variables|Portal|GetHexagonOut_World) true) 1)
        (Utilities|FlipFlopCustom :!label _label
          (:A
            (Default|EveryoneCallSetTranform _player_character_dg_3 (Transformation|GetActorLocation _hexagonin_world))
            (Default|EveryoneSetHexagonCell _player_character_dg_3 _hexagonin_world))
          (:B
            (Default|EveryoneCallSetTranform _player_character_dg_3 (Transformation|GetActorLocation _hexagonout_world))
            (Default|EveryoneSetHexagonCell _player_character_dg_3 _hexagonout_world))))
      (elif (<= (CallFunction|HexagonDistance _currentcharacterlocationworld (Variables|Portal|GetHexagonIn_World) true) 1)
        (goto _label)))
    (elif (Variables|Portal|GetFlipFlop)
      (if (<= (CallFunction|HexagonDistance _currentcharacterlocationarena (Variables|Portal|GetHexagonOut_Arena) false) 1)
        (Utilities|FlipFlopCustom :!label _label_2
          (:A
            (Default|EveryoneCallSetTranform _player_character_dg (Transformation|GetWorldLocation (Variables|/Game/Blueprints/ProceduralGeneration/HexagonCellArena.HexagonCellArena_C|GetHexagonPointLocation _hexagonin_arena)))
            (Default|EveryoneSetHexagonCell _player_character_dg 0 _hexagonin_arena))
          (:B
            (Default|EveryoneCallSetTranform _player_character_dg (Transformation|GetWorldLocation (Variables|/Game/Blueprints/ProceduralGeneration/HexagonCellArena.HexagonCellArena_C|GetHexagonPointLocation _hexagonout_arena)))
            (Default|EveryoneSetHexagonCell _player_character_dg 0 _hexagonout_arena))))
      (elif (<= (CallFunction|HexagonDistance _currentcharacterlocationarena (Variables|Portal|GetHexagonIn_Arena) false) 1)
        (goto _label_2)))))