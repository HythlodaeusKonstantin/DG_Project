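; Player controller for a hexagon-based game with a world map and islands, handling world startup and click-to-move.
; StartGame generates or loads a world via GameInst_DG; multiplayer loading spawns ReplicatedStorage on the server, while clients create an empty save object.
; A separate RPC pair copies the server's save data to the owning client, then loads it.
; Hex clicks enter islands or move the pawn through server-to-multicast events, marked unfinished.
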(event Custom|OnClick
  (params (HexagonCell :type Hexagon%20Cell%20Object%20Reference))
  ;[0.1336 0.1188 1] Логика перемещения по гексам (ДОРАБОТАТЬ)
  ;;[0 1 0] Клиентская часть
  (Variables|Default|SetCurrent%20Hexagon%20Cell HexagonCell)
  (bind _asplayer_character_dg (Utilities|Casting|CastToPlayerCharacter_DG (Pawn|GetControlledPawn)))
  (if (Variables|/Game/Blueprints/PlayerCharacter/PlayerCharacter_DG.PlayerCharacter_DG_C|GetOnWorldMap? _asplayer_character_dg)
    (if (not (== (Variables|/Game/Blueprints/PlayerCharacter/PlayerCharacter_DG.PlayerCharacter_DG_C|GetCurrentWorldMapHex _asplayer_character_dg) (Variables|Default|GetCurrent%20Hexagon%20Cell)))
      (if (Variables|/Game/Blueprints/ProceduralGeneration/HexagonCell.HexagonCell_C|GetisIsland? (Variables|Default|GetCurrent%20Hexagon%20Cell))
        (bind _asplayer_character_dg_2 (Utilities|Casting|CastToPlayerCharacter_DG (Pawn|GetControlledPawn)))
        (Variables|/Game/Blueprints/PlayerCharacter/PlayerCharacter_DG.PlayerCharacter_DG_C|SetOnWorldMap? _asplayer_character_dg_2 false)
        (Default|Enterisland (Variables|Default|GetGameInst) (Variables|/Game/Blueprints/ProceduralGeneration/HexagonCell.HexagonCell_C|GetIndexOfThisIslandInArray (Variables|Default|GetCurrent%20Hexagon%20Cell)))
        (else
          (CallFunction|MovetoLocationServer (Transformation|GetActorLocation (Variables|Default|GetCurrent%20Hexagon%20Cell)) (Variables|Default|GetCurrent%20Hexagon%20Cell) (Variables|/Game/Blueprints/ProceduralGeneration/HexagonCell.HexagonCell_C|GetIndex (Variables|Default|GetCurrent%20Hexagon%20Cell))))))
    (elif (not (== (Variables|/Game/Blueprints/PlayerCharacter/PlayerCharacter_DG.PlayerCharacter_DG_C|GetCurrentIslandHex _asplayer_character_dg) (Variables|Default|GetCurrent%20Hexagon%20Cell)))
      (if (Variables|/Game/Blueprints/ProceduralGeneration/HexagonCell.HexagonCell_C|GetCanPass? (Variables|Default|GetCurrent%20Hexagon%20Cell))
        (CallFunction|MovetoLocationServer (Transformation|GetActorLocation (Variables|Default|GetCurrent%20Hexagon%20Cell)) 0 (Variables|/Game/Blueprints/ProceduralGeneration/HexagonCell.HexagonCell_C|GetIndex (Variables|Default|GetCurrent%20Hexagon%20Cell)))))))

(event Custom|StartGame
  (bind _gameinst (Variables|Default|GetGameInst))
  (bind _gameinst_2 (Variables|Default|GetGameInst))
  ;[1 1 1] Генерация нового мира
  (Utilities|FlowControl|Delay 0.2)
  (if (Variables|/Game/Blueprints/GameSettings/GameInst_DG.GameInst_DG_C|GetLoadingGame? (Variables|Default|GetGameInst))
    (if (Variables|/Game/Blueprints/GameSettings/GameInst_DG.GameInst_DG_C|GetMultiplayer? (Variables|Default|GetGameInst))
      (if (Networking|IsServer)
        (Game|SpawnActorfromClass "/Game/Blueprints/GameSettings/ReplicatedStorage.ReplicatedStorage_C" (Math|Transform|MakeTransform "0, 0, 0") "Undefined" 0 0)
        (else
          (bind _returnvalue (SaveGame|CreateSaveGameObject "/Game/Blueprints/GameSettings/WorldStorage.WorldStorage_C"))
          (Variables|/Game/Blueprints/GameSettings/GameInst_DG.GameInst_DG_C|SetActiveSaveGame_WorldStorage (Variables|Default|GetGameInst) _returnvalue)))
      (else
        ;[1 1 1] Загрузка мира
        (Default|LoadWorld _gameinst_2)
        (Variables|/Game/Blueprints/GameSettings/GameInst_DG.GameInst_DG_C|SetInGame? _gameinst_2 true)))
    (else
      (Default|GenerateWorld _gameinst)
      (Variables|/Game/Blueprints/GameSettings/GameInst_DG.GameInst_DG_C|SetInGame? _gameinst true))))

(event Custom|MoveToLocation_Server
  (params (TargetLocation :type Vector) (Target :type Hexagon%20Cell%20Object%20Reference) (Key :type Vector%20%28by%20ref%29))
  ;[0.1336 0.1188 1] Логика перемещения по гексам (ДОРАБОТАТЬ)
  ;;[1 0 0] Серверная часть
  (CallFunction|MovetoLocationMulticast TargetLocation Key))

(event Custom|RunOwningCall_TranferSaveData
  (params (World%20Storage%20Save%20Data :type World%20Storage%20Save%20Data%20Structure))
  (bind (_worldgenerationhexagondata _worldgenerationnetworkdata _worlddatasaved_ _islandsonworldmap _indexofcurrentislandinarray _savename) (Utilities|Struct|BreakWorldStorageSaveData World%20Storage%20Save%20Data))
  (bind _gameinst (Variables|Default|GetGameInst))
  (bind _gameinst_2 (Variables|Default|GetGameInst))
  (bind _activesavegame_worldstorage (Variables|/Game/Blueprints/GameSettings/GameInst_DG.GameInst_DG_C|GetActiveSaveGame_WorldStorage _gameinst))
  (Utilities|FlowControl|Sequence
    (:then_0
      (Variables|/Game/Blueprints/GameSettings/WorldStorage.WorldStorage_C|SetIndexOfCurrentIslandInArray _activesavegame_worldstorage _indexofcurrentislandinarray)
      (Variables|/Game/Blueprints/GameSettings/WorldStorage.WorldStorage_C|SetIslandsOnWorldMap _activesavegame_worldstorage _islandsonworldmap)
      (Variables|/Game/Blueprints/GameSettings/WorldStorage.WorldStorage_C|SetSaveName _activesavegame_worldstorage _savename)
      (Variables|/Game/Blueprints/GameSettings/WorldStorage.WorldStorage_C|SetWorldDataSaved? _activesavegame_worldstorage _worlddatasaved_)
      (Variables|/Game/Blueprints/GameSettings/WorldStorage.WorldStorage_C|SetWorldGenerationHexagonData _activesavegame_worldstorage _worldgenerationhexagondata)
      (Variables|/Game/Blueprints/GameSettings/WorldStorage.WorldStorage_C|SetWorldGenerationNetworkData _activesavegame_worldstorage _worldgenerationnetworkdata))
    (:then_1
      (Default|LoadWorld _gameinst_2)
      (Variables|/Game/Blueprints/GameSettings/GameInst_DG.GameInst_DG_C|SetInGame? _gameinst_2 true))))

(event Custom|ServerCall_TransferSaveData
  (bind _gameinst (Variables|Default|GetGameInst))
  (bind _activesavegame_worldstorage (Variables|/Game/Blueprints/GameSettings/GameInst_DG.GameInst_DG_C|GetActiveSaveGame_WorldStorage _gameinst))
  (CallFunction|RunOwningCallTranferSaveData (Utilities|Struct|MakeWorldStorageSaveData (Variables|/Game/Blueprints/GameSettings/WorldStorage.WorldStorage_C|GetWorldGenerationHexagonData _activesavegame_worldstorage) (Variables|/Game/Blueprints/GameSettings/WorldStorage.WorldStorage_C|GetWorldGenerationNetworkData _activesavegame_worldstorage) (Variables|/Game/Blueprints/GameSettings/WorldStorage.WorldStorage_C|GetWorldDataSaved? _activesavegame_worldstorage) (Variables|/Game/Blueprints/GameSettings/WorldStorage.WorldStorage_C|GetIslandsOnWorldMap _activesavegame_worldstorage) (Variables|/Game/Blueprints/GameSettings/WorldStorage.WorldStorage_C|GetIndexOfCurrentIslandInArray _activesavegame_worldstorage) (Variables|/Game/Blueprints/GameSettings/WorldStorage.WorldStorage_C|GetSaveName _activesavegame_worldstorage))))

(event Custom|MoveToLocation_Multicast
  (params (TargetLocation :type Vector) (Key :type Vector%20%28by%20ref%29))
  (bind _gameinst (Variables|Default|GetGameInst))
  (bind _islandgenerationnetwork (Variables|/Game/Blueprints/GameSettings/GameInst_DG.GameInst_DG_C|GetIslandGenerationNetwork _gameinst))
  (bind _worldmap (Variables|/Game/Blueprints/GameSettings/GameInst_DG.GameInst_DG_C|GetWorldMap _gameinst))
  (bind _hexallmap (Variables|/Game/Blueprints/ProceduralGeneration/ProceduralWorldGeneration.ProceduralWorldGeneration_C|GetHexAllMap _worldmap))
  (bind _hexallmap_2 (Variables|/Game/Blueprints/ProceduralGeneration/ProceduralHexagonalNetwork.ProceduralHexagonalNetwork_C|GetHexAllMap _islandgenerationnetwork))
  (bind _value (Utilities|Map|Find _hexallmap_2 Key))
  (bind _value_2 (Utilities|Map|Find _hexallmap Key))
  (bind _asplayer_character_dg (Utilities|Casting|CastToPlayerCharacter_DG (Pawn|GetControlledPawn)))
  (Default|MovetoLocation (Variables|/Game/Blueprints/PlayerCharacter/PlayerCharacter_DG.PlayerCharacter_DG_C|GetMovementComponent _asplayer_character_dg) TargetLocation)
  (if (Variables|/Game/Blueprints/PlayerCharacter/PlayerCharacter_DG.PlayerCharacter_DG_C|GetOnWorldMap? (Variables|Default|GetPlayer%20Character%20DG))
    (Variables|/Game/Blueprints/PlayerCharacter/PlayerCharacter_DG.PlayerCharacter_DG_C|SetCurrentIslandHex _asplayer_character_dg _value_2)
    (Variables|/Game/Blueprints/PlayerCharacter/PlayerCharacter_DG.PlayerCharacter_DG_C|SetCurrentIslandHexIndex _asplayer_character_dg (Variables|/Game/Blueprints/ProceduralGeneration/HexagonCell.HexagonCell_C|GetIndex _value_2))
    (else
      (Variables|/Game/Blueprints/PlayerCharacter/PlayerCharacter_DG.PlayerCharacter_DG_C|SetCurrentIslandHex _asplayer_character_dg _value)
      (Variables|/Game/Blueprints/PlayerCharacter/PlayerCharacter_DG.PlayerCharacter_DG_C|SetCurrentIslandHexIndex _asplayer_character_dg (Variables|/Game/Blueprints/ProceduralGeneration/HexagonCell.HexagonCell_C|GetIndex _value)))))

(event Custom|clientCallSetTransform
  (params (NewLocation :type Vector))
  ;[0 1 0] Вызов перемещения у клиента
  (CallFunction|ServerSetTransform NewLocation))

(event Custom|ServerSetTransform
  (params (NewLocation :type Vector))
  ;[1 0 0] Перемещение на сервере
  (CallFunction|MulticastSetTransform NewLocation))

(event Custom|MulticastSetTransform
  (params (NewLocation :type Vector))
  ;[0 0 1] Перемещение у всех клиентов
  (Transformation|SetActorLocation (Pawn|GetControlledPawn self) NewLocation false false))

(event EventBeginPlay
  ;[0.1667 0.1667 0.1667] Инициализация
  (bind _asgame_inst_dg (Utilities|Casting|CastToGameInst_DG (Game|GetGameInstance)))
  (Variables|Default|SetGameInst _asgame_inst_dg)
  (Variables|SaveDataTransfer|SetInizialisationDone false))

(fn ConstructionScript)