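; Forest prop, apparently for the world map, that varies the child components under its Scene component to break up repetition.
; The construction script uses unseeded randomness to give about 75% of children a random yaw and small uniform scale, hiding the rest.
; On BeginPlay it applies the Material variable to the first slot of those children that are static meshes.
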(event EventBeginPlay
  (for _array_element (Components|GetChildrenComponents (Variables|Default|GetScene) false)
    (bind _asstatic_mesh_component (Utilities|Casting|CastToStaticMeshComponent _array_element))
    (Rendering|Material|SetMaterial _asstatic_mesh_component 0 (Variables|Default|GetMaterial))))

(fn ConstructionScript
  (for _array_element (Components|GetChildrenComponents (Variables|Default|GetScene) false)
    (Utilities|RandomCase 0.75
      (:true
        (Transformation|SetWorldRotation _array_element (Math|Rotator|MakeRotator 0.0 0.0 (Math|Random|RandomFloatinRange 0.0 3.6e+02)) false false)
        (Transformation|SetWorldScale3D _array_element (Math|Conversions|ToVector(Float) (Math|Random|RandomFloatinRange 0.2 0.3))))
      (:false
        (Rendering|SetVisibility _array_element false false)))))