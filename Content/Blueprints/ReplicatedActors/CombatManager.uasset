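; CombatManager is a player-owned actor that relays turn-based combat start and end-turn events over the network, registering itself with its owning character on BeginPlay.
; Server events forward to multicasts that act on the current combat turn system.
; Battle start fills the combat UI queue with players and enemies, giving players initiative, and retries on a timer until the turn system is valid.
; Ending a turn notifies the turn system.
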(event Custom|endTurn%20-%20Server
  (CallFunction|EndTurn-Multicast))

(event Custom|endTurn%20-%20Multicast
  (Default|CallTurnEnded (Variables|Default|GetCurrentCombatTurnSystem))
  (Development|PrintString "Конец хода"))

(event Custom|StartBattle%20-%20Server
  (CallFunction|StartBattle-Multicast))

(event Custom|StartBattle%20-%20Multicast
  (bind _currentcombatturnsystem (Variables|Default|GetCurrentCombatTurnSystem))
  (Utilities|IsValid _currentcombatturnsystem
    (:Is%20Valid
      (Default|FillQueue (Variables|/Game/Blueprints/UserInterface/InGameUI/InGameUI.InGameUI_C|GetCombatTurnBasedUI (Variables|/Game/Blueprints/GameSettings/GameInst_DG.GameInst_DG_C|GetInGameUI (Variables|Default|GetGameInstance))) (Variables|/Game/Blueprints/TurnBased/CombatTurnSystem.CombatTurnSystem_C|GetPlayers%20in%20Combat _currentcombatturnsystem) (Variables|/Game/Blueprints/TurnBased/CombatTurnSystem.CombatTurnSystem_C|GetEnemy%20in%20Combat _currentcombatturnsystem) _currentcombatturnsystem true))
    (:Is%20Not%20Valid
      (Utilities|Time|SetTimerbyEvent (delegate Custom|StartBattle%20-%20Multicast) 0.5))))

(event EventBeginPlay
  (bind _asplayer_character_dg (Utilities|Casting|CastToPlayerCharacter_DG (Components|GetOwner)))
  (Variables|/Game/Blueprints/NPC/BaseCharacter_DG.BaseCharacter_DG_C|SetCombatManager _asplayer_character_dg self)
  (bind _asgame_inst_dg (Utilities|Casting|CastToGameInst_DG (Game|GetGameInstance)))
  (Variables|Default|SetGameInstance _asgame_inst_dg))

(fn ConstructionScript)