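; Fog of war and map manager that paints vision, explored areas and position markers into render targets, optionally server-only.
; A looping timer redraws moving fog components, accumulates explored area additively and composites the map through a material.
; SetNewOffset switches between world and island/battle targets, wiping the latter's exploration.
; It also updates map UI, post-process texture and parameter collection offsets, then redraws static components.
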(event Custom|DrawMovableObjects
  (Rendering|ClearRenderTarget2D (Variables|Default|GetMovementWorldMap))
  (Rendering|ClearRenderTarget2D (Variables|Default|GetPlayersPositionRenderTarget))
  (for _array_element (Variables|Default|GetFogOfWarComponent)
    (bind (_canvas _size _context) (Rendering|BeginDrawCanvastoRenderTarget (Variables|Default|GetMovementWorldMap)))
    (Canvas|DrawTexture _canvas "/Game/Materials/FogOfWar/UtilityRenderTarget_Tex.UtilityRenderTarget_Tex" (+ (Math|Vector2D|MakeVector2D (CallFunction|CalculateLocationonRenderTargetLowRes (.x (Variables|/Game/Blueprints/RenderTargetManager/FogOfWar/FogOfWarPlayerCharacterComponent.FogOfWarPlayerCharacterComponent_C|GetCurrentLocation _array_element)) (Variables|Default|GetOffsetX)) (CallFunction|CalculateLocationonRenderTargetLowRes (.y (Variables|/Game/Blueprints/RenderTargetManager/FogOfWar/FogOfWarPlayerCharacterComponent.FogOfWarPlayerCharacterComponent_C|GetCurrentLocation _array_element)) (Variables|Default|GetOffsetY))) "(X=-12.500000,Y=-12.500000)") "(X=25.000000,Y=25.000000)" "(X=0.000000,Y=0.000000)" "(X=1.000000,Y=1.000000)" "(R=1.000000,G=1.000000,B=1.000000,A=1.000000)" "BLEND_Additive" 0.0 "(X=0.500000,Y=0.500000)")
    (Rendering|EndDrawCanvastoRenderTarget _context)
    (bind (_canvas_2 _size_2 _context_2) (Rendering|BeginDrawCanvastoRenderTarget (Variables|Default|GetBeenthereRenderTarget)))
    (Canvas|DrawTexture _canvas_2 "/Game/Materials/FogOfWar/UtilityRenderTarget_Tex.UtilityRenderTarget_Tex" (+ (Math|Vector2D|MakeVector2D (CallFunction|CalculateLocationonRenderTargetLowRes (.x (Variables|/Game/Blueprints/RenderTargetManager/FogOfWar/FogOfWarPlayerCharacterComponent.FogOfWarPlayerCharacterComponent_C|GetCurrentLocation _array_element)) (Variables|Default|GetOffsetX)) (CallFunction|CalculateLocationonRenderTargetLowRes (.y (Variables|/Game/Blueprints/RenderTargetManager/FogOfWar/FogOfWarPlayerCharacterComponent.FogOfWarPlayerCharacterComponent_C|GetCurrentLocation _array_element)) (Variables|Default|GetOffsetY))) "(X=-12.500000,Y=-12.500000)") "(X=25.000000,Y=25.000000)" "(X=0.000000,Y=0.000000)" "(X=1.000000,Y=1.000000)" "(R=1.000000,G=1.000000,B=1.000000,A=1.000000)" "BLEND_Additive" 0.0 "(X=0.500000,Y=0.500000)")
    (Rendering|EndDrawCanvastoRenderTarget _context_2)
    (bind (_canvas_3 _size_3 _context_3) (Rendering|BeginDrawCanvastoRenderTarget (Variables|Default|GetPlayersPositionRenderTarget)))
    (Canvas|DrawTexture _canvas_3 "/Game/Materials/Map/PlayerPointOnMap.PlayerPointOnMap" (Math|Vector2D|MakeVector2D (CallFunction|CalculateLocationonRenderTargetHighRes (.x (Variables|/Game/Blueprints/RenderTargetManager/FogOfWar/FogOfWarPlayerCharacterComponent.FogOfWarPlayerCharacterComponent_C|GetCurrentLocation _array_element)) (Variables|Default|GetOffsetX)) (CallFunction|CalculateLocationonRenderTargetHighRes (.y (Variables|/Game/Blueprints/RenderTargetManager/FogOfWar/FogOfWarPlayerCharacterComponent.FogOfWarPlayerCharacterComponent_C|GetCurrentLocation _array_element)) (Variables|Default|GetOffsetY))) "(X=15.000000,Y=15.000000)" "(X=0.000000,Y=0.000000)" "(X=1.000000,Y=1.000000)" "(R=1.000000,G=0.000000,B=0.000000,A=1.000000)" "BLEND_Masked" 0.0 "(X=0.500000,Y=0.500000)")
    (Rendering|EndDrawCanvastoRenderTarget _context_3))
  (Rendering|ClearRenderTarget2D (Variables|Default|GetMap))
  (Rendering|DrawMaterialtoRenderTarget (Variables|Default|GetMap) (Variables|Default|GetDrawMapMaterial)))

(event Custom|DrawStaticObjects
  (Rendering|ClearRenderTarget2D (Variables|Default|GetStaticWorldMap))
  (for _array_element (Variables|Default|GetFogOfWarStaticComponents)
    (bind (_canvas _size _context) (Rendering|BeginDrawCanvastoRenderTarget (Variables|Default|GetStaticWorldMap)))
    (Canvas|DrawTexture _canvas "/Game/Materials/FogOfWar/UtilityRenderTarget_Tex.UtilityRenderTarget_Tex" (+ (Math|Vector2D|MakeVector2D (CallFunction|CalculateLocationonRenderTargetLowRes (.x (Variables|/Game/Blueprints/RenderTargetManager/FogOfWar/FogOfWarStaticComponent.FogOfWarStaticComponent_C|GetCurrentLocation _array_element)) (Variables|Default|GetOffsetX)) (CallFunction|CalculateLocationonRenderTargetLowRes (.y (Variables|/Game/Blueprints/RenderTargetManager/FogOfWar/FogOfWarStaticComponent.FogOfWarStaticComponent_C|GetCurrentLocation _array_element)) (Variables|Default|GetOffsetY))) "(X=-12.500000,Y=-12.500000)") "(X=25.000000,Y=25.000000)" "(X=0.000000,Y=0.000000)" "(X=1.000000,Y=1.000000)" "(R=1.000000,G=1.000000,B=1.000000,A=1.000000)" "BLEND_Opaque" 0.0 "(X=0.500000,Y=0.500000)")
    (Rendering|EndDrawCanvastoRenderTarget _context)
    (bind (_canvas_2 _size_2 _context_2) (Rendering|BeginDrawCanvastoRenderTarget (Variables|Default|GetBeenthereRenderTarget)))
    (Canvas|DrawTexture _canvas_2 "/Game/Materials/FogOfWar/UtilityRenderTarget_Tex.UtilityRenderTarget_Tex" (+ (Math|Vector2D|MakeVector2D (CallFunction|CalculateLocationonRenderTargetLowRes (.x (Variables|/Game/Blueprints/RenderTargetManager/FogOfWar/FogOfWarStaticComponent.FogOfWarStaticComponent_C|GetCurrentLocation _array_element)) (Variables|Default|GetOffsetX)) (CallFunction|CalculateLocationonRenderTargetLowRes (.y (Variables|/Game/Blueprints/RenderTargetManager/FogOfWar/FogOfWarStaticComponent.FogOfWarStaticComponent_C|GetCurrentLocation _array_element)) (Variables|Default|GetOffsetY))) "(X=-12.500000,Y=-12.500000)") "(X=25.000000,Y=25.000000)" "(X=0.000000,Y=0.000000)" "(X=1.000000,Y=1.000000)" "(R=1.000000,G=1.000000,B=1.000000,A=1.000000)" "BLEND_Additive" 0.0 "(X=0.500000,Y=0.500000)")
    (Rendering|EndDrawCanvastoRenderTarget _context_2)))

(event EventBeginPlay
  (bind _asgame_inst_dg (Utilities|Casting|CastToGameInst_DG (Game|GetGameInstance)))
  (Variables|Default|SetGame%20Inst%20DG _asgame_inst_dg)
  (if (Variables|Default|GetFogOfWarOnlyForServer)
    (if (Networking|IsServer)
      (Rendering|ClearRenderTarget2D (Variables|Default|GetBeenthereRenderTarget) :!label _label)
      (Rendering|ClearRenderTarget2D (Variables|Default|GetStaticWorldMap))
      (Utilities|Time|SetTimerbyEvent (delegate Custom|DrawMovableObjects) 0.1 true))
    (else
      (goto _label))))

(fn ConstructionScript)

(fn CalculateLocationonRenderTargetLowRes
  (params (AxisLocation :type Float%20%28single-precision%29) (AxisOffset :type Float%20%28single-precision%29))
  (return (* (- 1.0 (/ (+ (- AxisLocation AxisOffset) 4.5e+03) 9e+03)) 64.0)))

(fn SetNewOffset
  (params (OffsetX :type Float%20%28single-precision%29) (OffsetY :type Float%20%28single-precision%29) (WhereTo :type CurrentWorld%20Enum :default "NewEnumerator0"))
  (bind _game_inst_dg (Variables|Default|GetGame%20Inst%20DG))
  (bind _collectionparameter (Variables|Default|GetCollectionParameter))
  (bind _weathermanager (Variables|/Game/Blueprints/GameSettings/GameInst_DG.GameInst_DG_C|GetWeatherManager _game_inst_dg))
  (bind _posprocessmaterial (Variables|/Game/Blueprints/Weather/WeatherManager.WeatherManager_C|GetPosprocessMaterial _weathermanager))
  (switch Utilities|FlowControl|Switch|SwitchonCurrentWorld WhereTo
    (:NewEnumerator0
      (Rendering|Material|SetTextureParameterValue _posprocessmaterial "BeenthereRenderTarget" "/Game/Materials/FogOfWar/FogOfWarBeenThere_WorldMap.FogOfWarBeenThere_WorldMap")
      (Variables|Default|SetBeenthereRenderTarget (Variables|Default|GetBeenthereWorldMap))
      (Variables|Default|SetDrawMapMaterial "/Game/Materials/Map/DrawMapWorld.DrawMapWorld")
      (Variables|Default|SetMap (Variables|Default|GetMap_World))
      (Class|Image|SetBrushfromMaterial (Variables|/Game/Blueprints/UserInterface/MapUI/MapUI.MapUI_C|GetMap (Variables|/Game/Blueprints/UserInterface/InGameUI/InGameUI.InGameUI_C|GetMapUI (Variables|/Game/Blueprints/GameSettings/GameInst_DG.GameInst_DG_C|GetInGameUI (Variables|Default|GetGame%20Inst%20DG)))) "/Game/Materials/Map/Map_WorldM.Map_WorldM"))
    (:NewEnumerator1
      (Rendering|Material|SetTextureParameterValue _posprocessmaterial "BeenthereRenderTarget" "/Game/Materials/FogOfWar/FogOfWarBeenThere_Event.FogOfWarBeenThere_Event" :!label _label)
      (bind _output_get (Variables|Default|SetBeenthereRenderTarget (Variables|Default|GetBeenthereWorldEvent)))
      (Rendering|ClearRenderTarget2D _output_get)
      (Variables|Default|SetDrawMapMaterial "/Game/Materials/Map/DrawMapEvent.DrawMapEvent")
      (Variables|Default|SetMap (Variables|Default|GetMap_Event))
      (Class|Image|SetBrushfromMaterial (Variables|/Game/Blueprints/UserInterface/MapUI/MapUI.MapUI_C|GetMap (Variables|/Game/Blueprints/UserInterface/InGameUI/InGameUI.InGameUI_C|GetMapUI (Variables|/Game/Blueprints/GameSettings/GameInst_DG.GameInst_DG_C|GetInGameUI (Variables|Default|GetGame%20Inst%20DG)))) "/Game/Materials/Map/Map_EventM.Map_EventM"))
    (:NewEnumerator2
      (goto _label)))
  (Variables|Default|SetOffsetX OffsetX)
  (Variables|Default|SetOffsetY OffsetY)
  (Rendering|Material|SetScalarParameterValue _collectionparameter (Utilities|Name|MakeLiteralName "OffsetX") OffsetX :!class /Script/Engine.KismetMaterialLibrary)
  (Rendering|Material|SetScalarParameterValue _collectionparameter (Utilities|Name|MakeLiteralName "OffsetY") OffsetY :!class /Script/Engine.KismetMaterialLibrary)
  (CallFunction|DrawStaticObjects))

(fn CalculateLocationonRenderTargetHighRes
  (params (AxisLocation :type Float%20%28single-precision%29) (AxisOffset :type Float%20%28single-precision%29))
  (return (* (- 1.0 (/ (+ (- AxisLocation AxisOffset) 4.5e+03) 9e+03)) 1024.0)))