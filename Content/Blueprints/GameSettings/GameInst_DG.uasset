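; Game instance that owns the WorldStorage save object and switches play between a procedural world map and hexagonal islands.
; Init deletes the save slot before its exists check, so the load branch normally gives way to creating a fresh save.
; Each switch saves the current view, destroys its hexes and network actor, then spawns and generates the other, skipping teardown on first world generation.
; It also wraps JoinSession for the first player controller.
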(event Custom|JoinSession
  (params (SessionResult :type Blueprint%20Session%20Result%20Structure))
  (|JoinSession (Game|GetPlayerController 0) SessionResult))

(event Custom|GenerateIsland
  (params (IsIsland? :type Boolean) (IslandStruct :type Island%20Structure) (IndexOfThisIslandInArray :type Integer))
  ;[1 1 1] Переход на остров
  (if IsIsland?
    ;;[1 1 1] №1: Сохраняем информацию о карте мира и очищаем уровень
    (Utilities|FlowControl|Sequence
      (:then_0
        (bind _output_get (Variables|Default|SetIsland%20Struct IslandStruct))
        (Variables|TempShit|SetIndex%20Of%20This%20Island%20in%20Array IndexOfThisIslandInArray)
        (Variables|TempShit|SetIslandSize (.islandSize (Utilities|Struct|BreakIsland _output_get)))
        (for _array_element (.islandComposition (Utilities|Struct|BreakIsland _output_get))
          (Variables|/Game/Blueprints/ProceduralGeneration/HexagonCell.HexagonCell_C|SetCurentGenerate _array_element true))
        (Default|SaveData (Variables|Default|GetWorldMap))
        (for _array_element_2 (Variables|/Game/Blueprints/ProceduralGeneration/ProceduralWorldGeneration.ProceduralWorldGeneration_C|GetHexagonCells-ALL (Variables|Default|GetWorldMap))
          (Actor|DestroyActor _array_element_2))
        (Actor|DestroyActor (Variables|Default|GetWorldMap)))
      (:then_1
        ;;[1 1 1] №2: Спавним актора-нетворк острова и генерируем остров
        (bind _returnvalue (Game|SpawnActorfromClass "/Game/Blueprints/ProceduralGeneration/ProceduralHexagonalNetwork.ProceduralHexagonalNetwork_C" (Math|Transform|MakeTransform "0, 0, 0") "Undefined" 0 0))
        (bind _output_get_2 (Variables|Default|SetIslandGenerationNetwork _returnvalue))
        (Default|Generate _output_get_2 (Variables|TempShit|GetIndex%20Of%20This%20Island%20in%20Array) (Variables|TempShit|GetIslandSize))))))

(event Custom|GenerateWorld
  (bind _islandgenerationnetwork (Variables|Default|GetIslandGenerationNetwork))
  ;[1 1 1] Создание карты мира/Переход на карту мира
  ;;[1 1 1] В первый раз не надо сохранять данные острова, поэтому есть DoOnce
  (if (Variables|Default|GetdoOnce)
    (Utilities|FlowControl|Sequence
      (:then_0
        ;;[1 1 1] №1: Сохраняем данные острова, удаляем все его гексы и нетворк
        (Default|SaveData (Variables|Default|GetIslandGenerationNetwork))
        (for _array_element (Variables|/Game/Blueprints/ProceduralGeneration/ProceduralHexagonalNetwork.ProceduralHexagonalNetwork_C|GetHexagonCells-ALL _islandgenerationnetwork)
          (Actor|DestroyActor _array_element))
        (Actor|DestroyActor _islandgenerationnetwork))
      (:then_1
        ;;[1 1 1] №2: Спавним актора-нетворк генерации карты мира и генерируем карту мира
        (bind _returnvalue (Game|SpawnActorfromClass "/Game/Blueprints/ProceduralGeneration/ProceduralWorldGeneration.ProceduralWorldGeneration_C" (Math|Transform|MakeTransform "0, 0, 0") "Undefined" 0 0 :!label _label))
        (bind _output_get (Variables|Default|SetWorldGenerationNetwork _returnvalue))
        (Default|Generate _output_get)))
    (else
      (Variables|Default|SetdoOnce true)
      (goto _label))))

(event EventInit
  (Utilities|FlowControl|Sequence
    (:then_0
      ;[1 1 1] Создание сохранения или загрузка
      (SaveGame|DeleteGameinSlot (Variables|Default|GetWorldStorageName))
      (bind _returnvalue (SaveGame|DoesSaveGameExist (Variables|Default|GetWorldStorageName)))
      (if _returnvalue
        (bind _returnvalue_2 (SaveGame|LoadGamefromSlot (Variables|Default|GetWorldStorageName)))
        (bind _asworld_storage (Utilities|Casting|CastToWorldStorage _returnvalue_2))
        (Variables|Default|SetWorldStorage _asworld_storage)
        (else
          (bind _returnvalue_3 (SaveGame|CreateSaveGameObject "/Game/Blueprints/GameSettings/WorldStorage.WorldStorage_C"))
          (Variables|Default|SetWorldStorage _returnvalue_3)
          (Development|PrintString "Слот создан" true true "(R=0.000000,G=0.660000,B=1.000000,A=1.000000)" 1e+01))))))