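; Actor component that makes a PlaceableOnHexagonCell actor highlight under the cursor as an interactable object.
; On BeginPlay it finds the owner's static or skeletal mesh and box collision by the "Interactable" tag, then records whether the owner has a current location.
; Box cursor-over events toggle the mesh's custom depth render for outlining.
; The click handler is bound but empty.
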(event Custom|OnBeginCursorOver
  (params (TouchedComponent :type Primitive%20Component%20Object%20Reference))
  (CallFunction|OutlineActor true))

(event Custom|OnEndCursorOver
  (params (TouchedComponent :type Primitive%20Component%20Object%20Reference))
  (CallFunction|OutlineActor false))

(event Custom|OnClicked
  (params (TouchedComponent :type Primitive%20Component%20Object%20Reference) (ButtonPressed :type Key%20Structure :default "None")))

(event EventBeginPlay
  (bind _asplaceable_on_hexagon_cell (Utilities|Casting|CastToPlaceableOnHexagonCell (Components|GetOwner)))
  (Variables|Default|SetOwner _asplaceable_on_hexagon_cell)
  (bind _asgame_inst_dg (Utilities|Casting|CastToGameInst_DG (Game|GetGameInstance)))
  (Variables|Default|SetGame%20Inst%20DG _asgame_inst_dg)
  (Variables|Default|SetStaticMesh (Utilities|Array|Get(acopy) (Actor|GetComponentsbyTag (Variables|Default|GetOwner) "/Script/Engine.StaticMeshComponent" "Interactable")))
  (Variables|Default|SetSkeletalMesh (Utilities|Array|Get(acopy) (Actor|GetComponentsbyTag (Variables|Default|GetOwner) "/Script/Engine.SkeletalMeshComponent" "Interactable")))
  (bind _output_get (Variables|Default|SetBoxCollision (Utilities|Array|Get(acopy) (Actor|GetComponentsbyTag (Variables|Default|GetOwner) "/Script/Engine.BoxComponent" "Interactable"))))
  (EventDispatchers|AssignOnBeginCursorOver _output_get (delegate Custom|OnBeginCursorOver))
  (EventDispatchers|AssignOnEndCursorOver _output_get (delegate Custom|OnEndCursorOver))
  (EventDispatchers|AssignOnClicked _output_get (delegate Custom|OnClicked))
  (Utilities|FlowControl|Sequence
    (:then_0
      (Utilities|IsValid (Variables|Default|GetStaticMesh)
        (:Is%20Valid
          (Variables|Default|SetMesh (Variables|Default|GetStaticMesh)))
        (:Is%20Not%20Valid
          (Utilities|IsValid (Variables|Default|GetSkeletalMesh)
            (:Is%20Valid
              (Variables|Default|SetMesh (Variables|Default|GetSkeletalMesh)))))))
    (:then_1
      (Utilities|IsValid (Variables|/Game/Blueprints/PointOfInterest/PlaceableOnHexagonCell.PlaceableOnHexagonCell_C|GetCurrentLocation (Variables|Default|GetOwner))
        (:Is%20Valid
          (Variables|Default|SetPlacedInWorld true))
        (:Is%20Not%20Valid
          (Variables|Default|SetPlacedInWorld false))))))

(fn OutlineActor
  (params (Active :type Boolean))
  (Rendering|SetRenderCustomDepth (Variables|Default|GetMesh) Active))