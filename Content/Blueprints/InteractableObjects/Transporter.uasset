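; Clickable transporter that moves the player character between paired In and Out hexagons, on either the world map or an arena.
; OnClick picks the world or arena pair via InWorld, then requires the character within one hex of the end selected by FlipFlop.
; A custom flip-flop macro toggles that stored bool and sends transform and cell updates through the character's Everyone-prefixed calls.
; Out-of-range clicks only print a debug string.
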(event EventBeginPlay
  (|CallParentFunction) ; This node is disabled and will not be called.\nDrag off pins to build functionality.
)

(event Collision|EventActorBeginOverlap
  (params (OtherActor :type Actor%20Object%20Reference))
  (|CallParentFunction OtherActor) ; This node is disabled and will not be called.\nDrag off pins to build functionality.
)

(event EventTick
  (params (DeltaSeconds :type Float%20%28single-precision%29))
  (|CallParentFunction DeltaSeconds) ; This node is disabled and will not be called.\nDrag off pins to build functionality.
)

(fn ConstructionScript
  (|CallParentFunction))

(fn OnClick
  (bind _game_inst_dg (Variables|Default|GetGame%20Inst%20DG))
  (bind _hexagonout_arena (Variables|Default|GetHexagonOut_Arena))
  (bind _game_inst_dg_2 (Variables|Default|GetGame%20Inst%20DG))
  (bind _hexagonin_world (Variables|Default|GetHexagonIn_World))
  (bind _hexagonout_world (Variables|Default|GetHexagonOut_World))
  (bind _game_inst_dg_3 (Variables|Default|GetGame%20Inst%20DG))
  (bind _hexagonin_arena (Variables|Default|GetHexagonIn_Arena))
  (bind _player_character_dg (Variables|/Game/Blueprints/GameSettings/GameInst_DG.GameInst_DG_C|GetPlayer%20Character%20DG _game_inst_dg))
  (bind _player_character_dg_2 (Variables|/Game/Blueprints/GameSettings/GameInst_DG.GameInst_DG_C|GetPlayer%20Character%20DG _game_inst_dg_2))
  (bind _player_character_dg_3 (Variables|/Game/Blueprints/GameSettings/GameInst_DG.GameInst_DG_C|GetPlayer%20Character%20DG _game_inst_dg_3))
  (bind _currentcharacterlocation (Variables|/Game/Blueprints/NPC/BaseCharacter_DG.BaseCharacter_DG_C|GetcurrentCharacterLocation _player_character_dg_2))
  (bind _currentcharacterlocationarena (Variables|/Game/Blueprints/NPC/BaseCharacter_DG.BaseCharacter_DG_C|GetcurrentCharacterLocationArena _player_character_dg_2))
  (|CallParentFunction)
  (if (Variables|Default|GetInWorld)
    (if (Variables|Default|GetFlipFlop)
      (if (<= (CallFunction|HexagonDistance _currentcharacterlocation (Variables|Default|GetHexagonOut_World) true) 1)
        (Utilities|FlipFlopCustom :!label _label
          (:A
            (Default|EveryoneCallSetTranform _player_character_dg_3 (Transformation|GetActorLocation _hexagonin_world))
            (Default|EveryoneSetHexagonCell _player_character_dg_3 _hexagonin_world))
          (:B
            (Default|EveryoneCallSetTranform _player_character_dg_3 (Transformation|GetActorLocation _hexagonout_world))
            (Default|EveryoneSetHexagonCell _player_character_dg_3 _hexagonout_world)))
        (else
          (Development|PrintString "Hello" :!label _label_2)))
      (elif (<= (CallFunction|HexagonDistance _currentcharacterlocation (Variables|Default|GetHexagonIn_World) true) 1)
        (goto _label)
        (else
          (goto _label_2))))
    (else
      (if (Variables|Default|GetFlipFlop)
        (if (<= (CallFunction|HexagonDistance _currentcharacterlocationarena (Variables|Default|GetHexagonOut_Arena) false) 1)
          _
          (else
            (goto _label_2)))
        (elif (<= (CallFunction|HexagonDistance _currentcharacterlocationarena (Variables|Default|GetHexagonIn_Arena) false) 1)
          _
          (else
            (goto _label_2))))
      (Utilities|FlipFlopCustom
        (:A
          (Default|EveryoneCallSetTranform _player_character_dg (Transformation|GetWorldLocation (Variables|/Game/Blueprints/ProceduralGeneration/HexagonCellArena.HexagonCellArena_C|GetHexagonPointLocation _hexagonin_arena)))
          (Default|EveryoneSetHexagonCell _player_character_dg 0 _hexagonin_arena))
        (:B
          (Default|EveryoneCallSetTranform _player_character_dg (Transformation|GetWorldLocation (Variables|/Game/Blueprints/ProceduralGeneration/HexagonCellArena.HexagonCellArena_C|GetHexagonPointLocation _hexagonout_arena)))
          (Default|EveryoneSetHexagonCell _player_character_dg 0 _hexagonout_arena))))))