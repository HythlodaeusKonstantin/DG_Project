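; Player-owned network relay for the pre-combat preparation widget, registering itself on its PlayerCharacter_DG owner.
; Ready clicks and battle joins go through server events to multicasts, with joins also marking the hex for world saving.
; Hexes travel as island and hex indices resolved on each machine, so ready and refresh updates apply only where that hex is being prepared.
; EnterBattleArena hands that hex to the character and clears it.
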(event EventBeginPlay
  (bind _asplayer_character_dg (Utilities|Casting|CastToPlayerCharacter_DG (Components|GetOwner)))
  (Variables|/Game/Blueprints/NPC/BaseCharacter_DG.BaseCharacter_DG_C|SetWidgetNetworkManager _asplayer_character_dg self)
  (Variables|Default|SetOwnerPlayerCharacter _asplayer_character_dg)
  (bind _asgame_inst_dg (Utilities|Casting|CastToGameInst_DG (Game|GetGameInstance)))
  (Variables|Default|SetGameInstance _asgame_inst_dg))

(fn ConstructionScript)

(event Custom|Add%20Player%20to%20Battle%20-%20Server
  (params (Island%20OrdinarIndex :type Integer) (Hex%20OrdinarIndex :type Integer))
  (bind _gameinstance (Variables|Default|GetGameInstance))
  ;[1 0 0] Добавляем игрока в список готовящихся к бою в виджет
  (Utilities|Array|AddUnique (Variables|/Game/Blueprints/GameSettings/GameInst_DG.GameInst_DG_C|GetHexagonNeedToBeSaved_World _gameinstance) (.Value (Utilities|Map|Find (Variables|/Game/Blueprints/ProceduralGeneration/ProceduralHexagonalNetwork.ProceduralHexagonalNetwork_C|GetHexAllMapInt (.Value (Utilities|Map|Find (Variables|/Game/Blueprints/GameSettings/GameInst_DG.GameInst_DG_C|GetIslandGenerationNetworks _gameinstance) Island%20OrdinarIndex))) Hex%20OrdinarIndex)))
  (CallFunction|AddPlayertoBattle-Multicast Island%20OrdinarIndex Hex%20OrdinarIndex))

(event Custom|Add%20Player%20to%20Battle%20-%20Multicast
  (params (Island%20OrdinarIndex :type Integer) (Hex%20OrdinarIndex :type Integer))
  (bind _gameinstance (Variables|Default|GetGameInstance))
  (bind _gameinstance_2 (Variables|Default|GetGameInstance))
  (bind _islandgenerationnetworks (Variables|/Game/Blueprints/GameSettings/GameInst_DG.GameInst_DG_C|GetIslandGenerationNetworks _gameinstance_2))
  (bind _precombatpreparationshex (Variables|/Game/Blueprints/GameSettings/GameInst_DG.GameInst_DG_C|GetPreCombatPreparationsHex _gameinstance))
  (bind _ingameui (Variables|/Game/Blueprints/GameSettings/GameInst_DG.GameInst_DG_C|GetInGameUI _gameinstance_2))
  (bind _value (Utilities|Map|Find _islandgenerationnetworks Island%20OrdinarIndex))
  (bind _precombatui (Variables|/Game/Blueprints/UserInterface/InGameUI/InGameUI.InGameUI_C|GetPreCombatUI _ingameui))
  (bind _hexallmapint (Variables|/Game/Blueprints/ProceduralGeneration/ProceduralHexagonalNetwork.ProceduralHexagonalNetwork_C|GetHexAllMapInt _value))
  (bind _value_2 (Utilities|Map|Find _hexallmapint Hex%20OrdinarIndex))
  ;[0 0 1] Добавляем игрока в список готовящихся к бою в виджет
  (Default|AddPlayertoBattle _precombatui _value_2 (Variables|/Game/Blueprints/PlayerCharacter/PlayerCharacter_DG.PlayerCharacter_DG_C|GetPlayerInfo (Variables|Default|GetOwnerPlayerCharacter)))
  (Utilities|IsValid _precombatpreparationshex
    (:Is%20Valid
      (if (== _precombatpreparationshex _value_2)
        (Default|RefreshPlayerReadytoComtatUI _precombatui _value_2)))))

(event Custom|PlayerClickedOnReadyButton_PreCombat%20-%20Multicast
  (params (PlayerClicked :type String) (IslandOrdinarIndex :type Integer%20%28by%20ref%29) (HexOrdinarIndex :type Integer%20%28by%20ref%29))
  (bind _gameinstance (Variables|Default|GetGameInstance))
  (bind _precombatpreparationshex (Variables|/Game/Blueprints/GameSettings/GameInst_DG.GameInst_DG_C|GetPreCombatPreparationsHex _gameinstance))
  ;[0 0 1] Игрок нажал на кнопку "Готов"
  (Utilities|IsValid _precombatpreparationshex
    (:Is%20Valid
      (if (== _precombatpreparationshex (.Value (Utilities|Map|Find (Variables|/Game/Blueprints/ProceduralGeneration/ProceduralHexagonalNetwork.ProceduralHexagonalNetwork_C|GetHexAllMapInt (.Value (Utilities|Map|Find (Variables|/Game/Blueprints/GameSettings/GameInst_DG.GameInst_DG_C|GetIslandGenerationNetworks (Variables|Default|GetGameInstance)) IslandOrdinarIndex))) HexOrdinarIndex)))
        (Default|ReadyButtonClicked (Variables|/Game/Blueprints/UserInterface/InGameUI/InGameUI.InGameUI_C|GetPreCombatUI (Variables|/Game/Blueprints/GameSettings/GameInst_DG.GameInst_DG_C|GetInGameUI _gameinstance)) PlayerClicked)))))

(event Custom|PlayerClickedOnReadyButton_PreCombat%20-%20Client
  (bind _gameinstance (Variables|Default|GetGameInstance))
  (bind _precombatpreparationshex (Variables|/Game/Blueprints/GameSettings/GameInst_DG.GameInst_DG_C|GetPreCombatPreparationsHex _gameinstance))
  ;[0 1 0] Игрок нажал на кнопку "Готов"
  (CallFunction|PlayerClickedonReadyButtonPreCombat-Server (.playername (Variables|/Game/Blueprints/PlayerCharacter/PlayerCharacter_DG.PlayerCharacter_DG_C|GetPlayerInfo (Variables|Default|GetOwnerPlayerCharacter))) (Variables|/Game/Blueprints/ProceduralGeneration/HexagonCellWorld.HexagonCellWorld_C|GetIndexOfThisIslandInArray _precombatpreparationshex) (Variables|/Game/Blueprints/ProceduralGeneration/HexagonCellWorld.HexagonCellWorld_C|GetOrdinarIndex _precombatpreparationshex)))

(event Custom|PlayerClickedOnReadyButton_PreCombat%20-%20Server
  (params (PlayerClicked :type String) (IslandOrdinarIndex :type Integer%20%28by%20ref%29) (HexOrdinarIndex :type Integer%20%28by%20ref%29))
  ;[1 0 0] Игрок нажал на кнопку "Готов"
  (CallFunction|PlayerClickedonReadyButtonPreCombat-Multicast PlayerClicked IslandOrdinarIndex HexOrdinarIndex))

(event Custom|Enter%20Battle%20Arena
  ;[0 1 0] Эвент перехода на баттл арену
  (Default|EnterBattleArenaClient-toPlayerCharacter (Variables|Default|GetOwnerPlayerCharacter) (Variables|/Game/Blueprints/ProceduralGeneration/HexagonCellWorld.HexagonCellWorld_C|GetIndexOfThisIslandInArray (Variables|/Game/Blueprints/GameSettings/GameInst_DG.GameInst_DG_C|GetPreCombatPreparationsHex (Variables|Default|GetGameInstance))) (Variables|/Game/Blueprints/ProceduralGeneration/HexagonCellWorld.HexagonCellWorld_C|GetOrdinarIndex (Variables|/Game/Blueprints/GameSettings/GameInst_DG.GameInst_DG_C|GetPreCombatPreparationsHex (Variables|Default|GetGameInstance))))
  (Variables|/Game/Blueprints/GameSettings/GameInst_DG.GameInst_DG_C|SetPreCombatPreparationsHex (Variables|Default|GetGameInstance) 0))